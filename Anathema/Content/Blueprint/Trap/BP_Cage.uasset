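; One-shot cage trap that topples a candle to start a timed fire that damages living actors.
; Overlapping Box enables physics and torque on a destructible and the candle, hiding the candle and a mesh.
; After a short delay, Niagara fire and HitBox run for a few seconds, then switch off along with lights and decal.
; HitBox damages overlapping actors on entry through their BP_AC_LivingActor component.
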(event `self.Box.OnComponentBeginOverlap`
  (params (OverlappedComponent :type "PrimitiveComponent Object Reference") (OtherActor :type "Actor Object Reference") (OtherComp :type "PrimitiveComponent Object Reference") (OtherBodyIndex :type Integer) (bFromSweep :type Boolean) (SweepResult :type "HitResult Structure (by ref)"))
  (bind _destructible1 (`self.Destructible1`))
  (`/Engine/EditorBlueprintResources/StandardMacros.DoOnce` false
    (:`Completed`
      (`|ExecutionSequence`
        (:`then_0`
          (`PrimitiveComponent.SetSimulatePhysics` _destructible1 true)
          (`PrimitiveComponent.SetSimulatePhysics` (`self.Candle`) true)
          (`PrimitiveComponent.SetEnableGravity` _destructible1 true)
          (`PrimitiveComponent.AddTorqueInDegrees` _destructible1 (* (`self.GetActorForwardVector`) (-10000.0 -10000.0 -10000.0)) "None" true)
          (`PrimitiveComponent.AddTorqueInDegrees` (`self.Candle`) (* (`self.GetActorForwardVector`) (-10000.0 -10000.0 -10000.0)) "None" true))
        (:`then_1`
          (`SceneComponent.SetHiddenInGame` (`self.StaticMesh4`) true false)
          (`SceneComponent.SetHiddenInGame` (`self.Candle`) true false)
          (`KismetSystemLibrary.Delay` 0.9)
          (`|ExecutionSequence`
            (:`then_0`
              (`NiagaraComponent.SetAsset` (`self.Fire`) "/Game/VFX/Fire/NS_Fire_System.NS_Fire_System" true)
              (`SceneComponent.SetVisibility` (`self.Fire`) true false)
              (`KismetSystemLibrary.Delay` 5.0)
              (`SceneComponent.SetVisibility` (`self.Fire`) false false))
            (:`then_1`
              (`PrimitiveComponent.SetCollisionEnabled` (`self.HitBox`) "QueryOnly")
              (`KismetSystemLibrary.Delay` 5.0)
              (`PrimitiveComponent.SetCollisionEnabled` (`self.HitBox`) "NoCollision")
              (`SceneComponent.SetHiddenInGame` (`self.PointLight2`) true false)
              (`SceneComponent.SetHiddenInGame` (`self.PointLight3`) true false)
              (`SceneComponent.SetHiddenInGame` (`self.PointLight1`) true false)
              (`SceneComponent.SetHiddenInGame` (`self.PointLight`) true false)
              (`SceneComponent.SetHiddenInGame` (`self.Decal`) true false))))))))

(event `self.HitBox.OnComponentBeginOverlap`
  (params (OverlappedComponent :type "PrimitiveComponent Object Reference") (OtherActor :type "Actor Object Reference") (OtherComp :type "PrimitiveComponent Object Reference") (OtherBodyIndex :type Integer) (bFromSweep :type Boolean) (SweepResult :type "HitResult Structure (by ref)"))
  (bind _returnvalue (`self.GetComponentByClass` OtherActor "/Game/Blueprint/Component/Actor/BP_AC_LivingActor.BP_AC_LivingActor_C"))
  (`/Engine/EditorBlueprintResources/StandardMacros.IsValid` _returnvalue
    (:`Is Valid`
      (`/Game/Blueprint/Component/Actor/BP_AC_LivingActor.TakeDamage` _returnvalue 100.0 self))))

(fn `UserConstructionScript`)