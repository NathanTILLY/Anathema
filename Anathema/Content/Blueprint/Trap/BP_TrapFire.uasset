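; BP_TrapFire is a trap Blueprint that briefly swings two grilles open when OpenTrap is called.
; A DoOnce limits it to one activation, then a Sequence starts two timelines that lerp each grille's pitch.
; Both grilles lose collision while open, and parallel five-second delays reverse the timelines from the end and restore collision.
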(event `self.OpenTrap`
  (`/Engine/EditorBlueprintResources/StandardMacros.DoOnce` false
    (:`Completed`
      (`|ExecutionSequence`
        (:`then_0`
          (bind (_direction _trap) (`Timeline|Open trap Up` :!label _label)
            (:`Update`
              (`SceneComponent.K2_SetRelativeRotation` (`self.Grille2`) (`KismetMathLibrary.MakeRotator` 0.0 (`KismetMathLibrary.Lerp` (`self.Close`) (`self.Open`) _trap)) false false))))
        (:`then_1`
          (`KismetSystemLibrary.Delay` 5.0)
          (goto _label :!via `ReverseFromEnd`))
        (:`then_2`
          (bind (_direction_2 _op) (`Timeline|OpenTr` :!label _label_2)
            (:`Update`
              (`SceneComponent.K2_SetRelativeRotation` (`self.Grille1`) (`KismetMathLibrary.MakeRotator` 0.0 (`KismetMathLibrary.Lerp` (`self.A`) (`self.B`) _op)) false false))))
        (:`then_3`
          (`KismetSystemLibrary.Delay` 5.0)
          (goto _label_2 :!via `ReverseFromEnd`))
        (:`then_4`
          (`PrimitiveComponent.SetCollisionEnabled` (`self.Grille1`) "NoCollision")
          (`PrimitiveComponent.SetCollisionEnabled` (`self.Grille2`) "NoCollision")
          (`KismetSystemLibrary.Delay` 5.0)
          (`PrimitiveComponent.SetCollisionEnabled` (`self.Grille1`) "QueryAndPhysics")
          (`PrimitiveComponent.SetCollisionEnabled` (`self.Grille2`) "QueryAndPhysics"))))))

(fn `UserConstructionScript`)