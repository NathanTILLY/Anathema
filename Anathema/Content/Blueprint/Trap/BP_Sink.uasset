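; BP_Sink is an interactable trap trigger that opens the up and down traps linked to its SinkValue.
; On Interact, it scans all BP_TrapUp actors, then all BP_TrapDown actors, passing the Player to OpenTrapUp or OpenTrap where TrapValue equals SinkValue.
; Each loop breaks at the first non-matching trap, so matching traps later in that array stay untriggered.
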(event `/Game/Blueprint/Trap/BPI_Interact.Interact`
  (params (Player :type "Character Object Reference"))
  (`|ExecutionSequence`
    (:`then_0`
      (bind _outactors (`GameplayStatics.GetAllActorsOfClass` "/Game/Blueprint/Trap/BP_TrapUp.BP_TrapUp_C"))
      (for _array_element _outactors
        (if (== (`/Game/Blueprint/Trap/BP_TrapUp.TrapValue` _array_element) (`self.SinkValue`))
          (`/Game/Blueprint/Trap/BP_TrapUp.OpenTrapUp` _array_element Player)
          (else
            (break)))))
    (:`then_1`
      (bind _outactors_2 (`GameplayStatics.GetAllActorsOfClass` "/Game/Blueprint/Trap/BP_TrapDown.BP_TrapDown_C"))
      (for _array_element_2 _outactors_2
        (if (== (`/Game/Blueprint/Trap/BP_TrapDown.TrapValue` _array_element_2) (`self.SinkValue`))
          (`/Game/Blueprint/Trap/BP_TrapDown.OpenTrap` _array_element_2 Player)
          (else
            (break)))))))

(fn `UserConstructionScript`)