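; BP_TrapDown is a trap with two hinged grilles that swing open and a hit box that damages living actors.
; OpenTrap plays two timelines that interpolate each grille's pitch, then reverses both after a fixed delay to close them.
; Independently of the grilles' state, any overlap with HitBox deals heavy damage through the actor's BP_AC_LivingActor component, naming the trap as attacker.
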(event `OpenTrap`
  (params (Player :type "Actor Object Reference"))
  (`|ExecutionSequence`
    (:`then_0`
      (bind (_direction _trap) (`Timeline|Open trap` :!label _label)
        (:`Update`
          (`SceneComponent.K2_SetRelativeRotation` (`self.Grille2`) (`KismetMathLibrary.MakeRotator` 0.0 (`KismetMathLibrary.Lerp` (`self.Close`) (`self.Open`) _trap)) false false))))
    (:`then_1`
      (`KismetSystemLibrary.Delay` 5.0)
      (goto _label :!via `Reverse`))
    (:`then_2`
      (bind (_direction_2 _op) (`Timeline|OpenTr` :!label _label_2)
        (:`Update`
          (`SceneComponent.K2_SetRelativeRotation` (`self.Grille1`) (`KismetMathLibrary.MakeRotator` 0.0 (`KismetMathLibrary.Lerp` (`self.A`) (`self.B`) _op)) false false))))
    (:`then_3`
      (`KismetSystemLibrary.Delay` 5.0)
      (goto _label_2 :!via `Reverse`))))

(event `self.HitBox.OnComponentBeginOverlap`
  (params (OverlappedComponent :type "PrimitiveComponent Object Reference") (OtherActor :type "Actor Object Reference") (OtherComp :type "PrimitiveComponent Object Reference") (OtherBodyIndex :type Integer) (bFromSweep :type Boolean) (SweepResult :type "HitResult Structure (by ref)"))
  (bind _returnvalue (`self.GetComponentByClass` OtherActor "/Game/Blueprint/Component/Actor/BP_AC_LivingActor.BP_AC_LivingActor_C"))
  (`/Engine/EditorBlueprintResources/StandardMacros.IsValid` _returnvalue
    (:`Is Valid`
      (`/Game/Blueprint/Component/Actor/BP_AC_LivingActor.TakeDamage` _returnvalue 100.0 self))))

(fn `UserConstructionScript`)