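; Battering ram that advances along a spline while the player stays inside its trigger sphere, then breaks open a linked door.
; Entering starts audio, wheel animation and a Path timeline scaled by Time that moves and orients Core along the spline; leaving pauses them.
; When the timeline finishes, it plays the ram animation once, then after a delay plays the impact sound, opens REFBpDoor and destroys the audio.
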(event `self.Sphere.OnComponentBeginOverlap`
  (params (OverlappedComponent :type "PrimitiveComponent Object Reference") (OtherActor :type "Actor Object Reference") (OtherComp :type "PrimitiveComponent Object Reference") (OtherBodyIndex :type Integer) (bFromSweep :type Boolean) (SweepResult :type "HitResult Structure (by ref)"))
  (cast `/Game/Blueprint/Player/BP_Player` OtherActor)
  (`|ExecutionSequence`
    (:`then_0`
      (`AudioComponent.Play` (`self.Audio`) 0.0))
    (:`then_1`
      (`TimelineComponent.SetPlayRate` (`self.Path`) (/ 1.0 (`self.Time`)))
      (`SkeletalMeshComponent.SetPlayRate` (`self.Wheel`) 1.0)
      (bind (_direction _alpha) (`Timeline|Path` :!label _label)
        (:`Update`
          (bind _returnvalue (`KismetMathLibrary.Lerp` 0.0 (`SplineComponent.GetSplineLength` (`self.Spline`)) _alpha))
          (bind (_returnvalue_roll _returnvalue_pitch _returnvalue_yaw) (`KismetMathLibrary.BreakRotator` (`KismetMathLibrary.ComposeRotators` (`SplineComponent.GetRotationAtDistanceAlongSpline` (`self.Spline`) _returnvalue "Local") (struct :`Yaw` -90.0))))
          (`SceneComponent.K2_SetRelativeTransform` (`self.Core`) (`KismetMathLibrary.MakeTransform` (`SplineComponent.GetLocationAtDistanceAlongSpline` (`self.Spline`) _returnvalue "Local") (`KismetMathLibrary.MakeRotator` (* _returnvalue_pitch -1.0) 0.0 _returnvalue_yaw)) false false))
        (:`Finished`
          (`/Engine/EditorBlueprintResources/StandardMacros.DoOnce` false
            (:`Completed`
              (`SkeletalMeshComponent.Stop` (`self.Wheel`))
              (`SkeletalMeshComponent.PlayAnimation` (`self.Core`) "/Game/Meshes/BatteringRam/BatteringRam_Anim.BatteringRam_Anim" false)
              (`KismetSystemLibrary.Delay` 1.33)
              (`|ExecutionSequence`
                (:`then_0`
                  (`GameplayStatics.PlaySoundAtLocation` "/Game/Audio/Sound2_0/BelierDoor_Cue.BelierDoor_Cue" (0.0 0.0 0.0) (struct) 1.0 1.0 0.0 null null null))
                (:`then_1`
                  (`/Game/Blueprint/Door/BP_Door.open` (`self.REFBp_Door`))
                  (`ActorComponent.K2_DestroyComponent` (`self.Audio`)))))))))))

(event `self.Sphere.OnComponentEndOverlap`
  (params (OverlappedComponent :type "PrimitiveComponent Object Reference") (OtherActor :type "Actor Object Reference") (OtherComp :type "PrimitiveComponent Object Reference") (OtherBodyIndex :type Integer))
  (cast `/Game/Blueprint/Player/BP_Player` OtherActor)
  (`AudioComponent.FadeOut` (`self.Audio`) 0.1 0.0 "Linear")
  (`SkeletalMeshComponent.SetPlayRate` (`self.Wheel`) 0.0)
  (goto _label :!via `Stop`))

(event `self.ReceiveBeginPlay`
  (bind _wheel (`self.Wheel`))
  (`SkeletalMeshComponent.PlayAnimation` _wheel "/Game/Meshes/BatteringRam/Wheel_Anim.Wheel_Anim" true)
  (`SkeletalMeshComponent.SetPlayRate` _wheel 0.0)
  (`AudioComponent.Stop` (`self.Audio`)))

(fn `UserConstructionScript`)