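; Gameplay GameState that writes the current level's state to a named save slot.
; SaveGame loads or creates a BP_SaveLevel, then passes it the player, enemies, consumable weapons, traps, interactables, ballista states, levers and objectives.
; Each world category is cleared and rebuilt from a GetAllActorsOfClass sweep, with serialization delegated to BP_SaveLevel.
; SaveDataToSaveSlot stamps the current level name before writing to disk.
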(event `self.ReceiveBeginPlay`
  (set `self.Player` (cast `/Game/Blueprint/Player/BP_Player` (`GameplayStatics.GetPlayerCharacter` 0) :!pure true))
  (cast `/Game/Blueprint/Player/BP_FPS_NewPlayer` (`self.AuthorityGameMode`)))

(fn `Save Data to Save Slot`
  (params (SaveData :type "/Game/Blueprint/Save/BP_SaveLevel Object Reference") (SlotName :type String))
  ;[1 1 1] Save all the data to the save slot
  (bind _returnvalue (`GameplayStatics.GetCurrentLevelName` true))
  (set `/Game/Blueprint/Save/BP_SaveLevel.LevelName` _returnvalue SaveData)
  (`GameplayStatics.SaveGameToSlot` (`local.SaveData`) (`local.SlotName`)))

(fn `SaveGame`
  (params (SlotName :type String))
  (locals (LocSavedGame :type "/Game/Blueprint/Save/BP_SaveLevel Object Reference") (LocSaveName :type String))
  (bind _output_get (set `local.LocSaveName` SlotName))
  (bind _returnvalue (`GameplayStatics.DoesSaveGameExist` _output_get))
  (if _returnvalue
    (bind _returnvalue_2 (`GameplayStatics.LoadGameFromSlot` (`local.LocSaveName`)))
    (set `local.LocSavedGame` (cast `/Game/Blueprint/Save/BP_SaveLevel` _returnvalue_2 :!pure true))
    (else
      (bind _returnvalue_3 (`GameplayStatics.CreateSaveGameObject` "/Game/Blueprint/Save/BP_SaveLevel.BP_SaveLevel_C"))
      (set `local.LocSavedGame` _returnvalue_3)))
  ;[1 1 1] Save Player Data
  (bind _returnvalue_4 (`GameplayStatics.GetActorOfClass` "/Game/Blueprint/Player/BP_Player.BP_Player_C"))
  (`/Game/Blueprint/Save/BP_SaveLevel.SavePlayerData` (`local.LocSavedGame`) _returnvalue_4)
  ;[1 1 1] Save Enemy Data
  (`KismetArrayLibrary.Array_Clear` (`/Game/Blueprint/Save/BP_SaveLevel.EnemyList` (`local.LocSavedGame`)))
  (bind _outactors (`GameplayStatics.GetAllActorsOfClass` "/Game/Blueprint/Enemies/Grivetons/BP_GrivetonParent.BP_GrivetonParent_C"))
  (for _array_element _outactors
    (`/Game/Blueprint/Save/BP_SaveLevel.SaveEnemiesData` (`local.LocSavedGame`) _array_element))
  ;[1 1 1] Save ConsumableWeaponData
  (`KismetArrayLibrary.Array_Clear` (`/Game/Blueprint/Save/BP_SaveLevel.ConsumableWeaponList` (`local.LocSavedGame`)))
  (bind _outactors_2 (`GameplayStatics.GetAllActorsOfClass` "/Game/Blueprint/Weapons/Consumable/BP_ConsumableWeaponParent.BP_ConsumableWeaponParent_C"))
  (for _array_element_2 _outactors_2
    (`/Game/Blueprint/Save/BP_SaveLevel.SaveConsumableWeaponData` (`local.LocSavedGame`) _array_element_2))
  ;[1 1 1] Save Trap Data
  (`KismetArrayLibrary.Array_Clear` (`/Game/Blueprint/Save/BP_SaveLevel.TrapUsedList` (`local.LocSavedGame`)))
  (bind _outactors_3 (`GameplayStatics.GetAllActorsOfClass` "/Game/Blueprint/Trap/BP_TrapParent.BP_TrapParent_C"))
  (for _array_element_3 _outactors_3
    (`/Game/Blueprint/Save/BP_SaveLevel.SaveTrapData` (`local.LocSavedGame`) _array_element_3))
  ;[1 1 1] Save Interactable Data
  (`KismetArrayLibrary.Array_Clear` (`/Game/Blueprint/Save/BP_SaveLevel.InteractableList` (`local.LocSavedGame`)))
  (bind _outactors_4 (`GameplayStatics.GetAllActorsOfClass` "/Game/Blueprint/Objets/BP_ParentInteractable.BP_ParentInteractable_C"))
  (for _array_element_4 _outactors_4
    (`/Game/Blueprint/Save/BP_SaveLevel.SaveInteractable` (`local.LocSavedGame`) _array_element_4))
  ;[1 1 1] Save Ballista State
  (`KismetArrayLibrary.Array_Clear` (`/Game/Blueprint/Save/BP_SaveLevel.BallistaState` (`local.LocSavedGame`)))
  (bind _outactors_5 (`GameplayStatics.GetAllActorsOfClass` "/Game/Blueprint/Objets/BP_Ballista.BP_Ballista_C"))
  (for _array_element_5 _outactors_5
    (`/Game/Blueprint/Save/BP_SaveLevel.SaveBallista` (`local.LocSavedGame`) (`/Game/Blueprint/Objets/BP_Ballista.CurrentState` _array_element_5)))
  ;[1 1 1] Save Levers State
  (`KismetArrayLibrary.Array_Clear` (`/Game/Blueprint/Save/BP_SaveLevel.LeverList` (`local.LocSavedGame`)))
  (bind _outactors_6 (`GameplayStatics.GetAllActorsOfClass` "/Game/Blueprint/Objets/BP_Lever.BP_Lever_C"))
  (for _array_element_6 _outactors_6
    (`/Game/Blueprint/Save/BP_SaveLevel.SaveLever` (`local.LocSavedGame`) _array_element_6))
  ;[1 1 1] Save Objectives State
  (`BlueprintMapLibrary.Map_Clear` (`/Game/Blueprint/Save/BP_SaveLevel.ObjectivesSentencesMap` (`local.LocSavedGame`)))
  (bind _outactors_7 (`GameplayStatics.GetAllActorsOfClass` "/Game/Blueprint/Objectives/BP_ObjectivesIndication.BP_ObjectivesIndication_C"))
  (for _array_element_7 _outactors_7
    (`/Game/Blueprint/Save/BP_SaveLevel.SaveObjectives` (`local.LocSavedGame`) _array_element_7))
  (`self.Save Data to Save Slot` (`local.LocSavedGame`) (`local.LocSaveName`)))

(fn `UserConstructionScript`)