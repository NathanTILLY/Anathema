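; BP_CameraMode is a player pawn, apparently for a camera mode, that provides movement and look controls.
; Its Bind event casts the controller to BP_PlayerController and binds to that controller's forward, right, look-up and look-right input dispatchers.
; The handlers add movement input along the actor's forward and right vectors and feed look axes into controller yaw and pitch.
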(event `Bind`
  (bind _asbp_player_controller (cast `/Game/Blueprint/Player/BP_PlayerController` (`self.GetController`) :!pure true))
  (add `/Game/Blueprint/Player/BP_PlayerController.OnMoveForwardPressed` _asbp_player_controller (`|CreateDelegate` :!event `Forward`))
  (add `/Game/Blueprint/Player/BP_PlayerController.OnMoveRightPressed` _asbp_player_controller (`|CreateDelegate` :!event `Right`))
  (add `/Game/Blueprint/Player/BP_PlayerController.OnLookUpPressed` _asbp_player_controller (`|CreateDelegate` :!event `LookUp`))
  (add `/Game/Blueprint/Player/BP_PlayerController.OnLookRightPressed` _asbp_player_controller (`|CreateDelegate` :!event `LookRight`)))

(event `Forward`
  (params (AxisValue :type "Float (double-precision)"))
  (`self.AddMovementInput` (`self.GetActorForwardVector`) AxisValue))

(event `Right`
  (params (AxisValue :type "Float (double-precision)"))
  (`self.AddMovementInput` (`self.GetActorRightVector`) AxisValue))

(event `LookRight`
  (params (AxisValue :type "Float (double-precision)"))
  (`self.AddControllerYawInput` AxisValue))

(event `LookUp`
  (params (AxisValue :type "Float (double-precision)"))
  (`self.AddControllerPitchInput` AxisValue))

(fn `UserConstructionScript`)