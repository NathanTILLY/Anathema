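; Comitatus shield weapon Blueprint that provides a check for whether a hit actor counts as its owner.
; IsMyOwner treats the hit actor as the owner if it is MyOwner, the shield itself, or any actor of exactly the owner's class.
; The class comparison makes other instances of the owner's class count as the owner too.
; The construction script only runs the parent's.
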(fn `IsMyOwner?`
  (params (ActorHit :type "Actor Object Reference"))
  (returns (`Owner?` :type Boolean))
  (if (and (!= ActorHit (`self.MyOwner`)) (!= ActorHit self) (!= (`GameplayStatics.GetObjectClass` ActorHit) (`GameplayStatics.GetObjectClass` (`self.MyOwner`))))
    (return false)
    (else
      (return true))))

(fn `UserConstructionScript`
  (`parent.UserConstructionScript`))