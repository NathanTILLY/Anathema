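; Sword and shield weapon for an enemy, extending a parent weapon Blueprint.
; IsMyOwner treats the weapon itself, any actor of its holder's class and any BP_EnemyParent child as owners, so enemy allies count as friendly.
; EffectOnHit adds a Niagara component at the hit Box's world transform, while SetHitStopValue is left empty.
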(fn `EffectOnHit`
  (params (ActorHit :type "Actor Object Reference"))
  (`AddComponent|NODE_AddNiagaraComponent-1` :`bManualAttachment` true :`RelativeTransform` (`SceneComponent.K2_GetComponentToWorld` (`self.Box`))))

(fn `IsMyOwner?`
  (params (ActorHit :type "Actor Object Reference"))
  (returns (`Owner?` :type Boolean))
  ;[1 1 1] Check if the actor hit is the weapon itself, the actor holding the weapon or an enemy, if none of them then it's not an owner
  (if (and (!= ActorHit self) (!= (`GameplayStatics.GetObjectClass` ActorHit) (`GameplayStatics.GetObjectClass` (`self.MyOwner`))) (not (`KismetMathLibrary.ClassIsChildOf` (`GameplayStatics.GetObjectClass` ActorHit) "/Game/Blueprint/Enemies/BP_EnemyParent.BP_EnemyParent_C")))
    (return false)
    (else
      (return true))))

(fn `SetHitStopValue`
  (params (CurrentHitStop :type "Float (double-precision)") (RemoveHitStop :type Boolean)))

(fn `UserConstructionScript`
  (`parent.UserConstructionScript`))