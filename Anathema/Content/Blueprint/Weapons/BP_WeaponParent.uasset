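; Base weapon actor that attaches to its owner's sword socket and provides light, heavy and special attacks, with stub hooks for blocking or special behavior.
; Hitbox overlaps skip the owner, its class and already-hit actors, then damage and push living-actor components, reducing damage after each hit.
; Hits trigger camera shake, Niagara effects and damage-scaled hit-stop through the owner's time dilation.
; An optional projectile spawns from the player's arms carrying current damage.
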(event `self.Hitbox.OnComponentBeginOverlap`
  (params (OverlappedComponent :type "PrimitiveComponent Object Reference") (OtherActor :type "Actor Object Reference") (OtherComp :type "PrimitiveComponent Object Reference") (OtherBodyIndex :type Integer) (bFromSweep :type Boolean) (SweepResult :type "HitResult Structure (by ref)"))
  (`self.ActorHitLogic` OtherActor))

(event `/Game/Blueprint/Interface/BPI_WeaponAttack.PickUp`
  (params (Owner :type "Actor Object Reference") (OwnerSkeletal :type "SkeletalMeshComponent Object Reference"))
  ;[1 1 1] Attach the weapon to the actor and set MyOwner variable
  (`|ExecutionSequence`
    (:`then_0`
      (`/Engine/EditorBlueprintResources/StandardMacros.DoOnce` false
        (:`Completed`
          (`self.K2_AttachToComponent` OwnerSkeletal "SwordSocket" "SnapToTarget" "SnapToTarget" "SnapToTarget"))))
    (:`then_1`
      (set `self.MyOwner` Owner)
      (`self.SetActorHiddenInGame` self false))))

(event `StopAnimation`
  (bind _myowner (`self.MyOwner`))
  ;[1 1 1] Effects when hitting a damageable actor
  (set `Actor.CustomTimeDilation` 0.0 _myowner)
  (`KismetSystemLibrary.Delay` (`self.CurrentStopTimer`))
  (set `Actor.CustomTimeDilation` 1.0 _myowner))

(fn `ActorHitLogic`
  (params (ActorHit :type "Actor Object Reference"))
  ;[1 1 1] All the logic when an actor is hit
  (bind _owner_ (`self.IsMyOwner?` ActorHit))
  (if (not _owner_)
    (bind _alreadyhit_ (`self.HasAlreadyBeenHit?` ActorHit))
    (if (not _alreadyhit_)
      (`self.DealDamage` ActorHit)
      (`self.EffectOnHit` ActorHit)
      (`self.StopAnimation`))))

(fn `DealDamage`
  (params (ActorHit :type "Actor Object Reference"))
  (locals (LocLivingComponent :type "/Game/Blueprint/Component/Actor/BP_AC_LivingActor Object Reference"))
  (bind _loclivingcomponent (`local.LocLivingComponent`))
  ;[1 1 1] Deal damage to the target
  (bind _output_get (set `local.LocLivingComponent` (`self.GetComponentByClass` ActorHit "/Game/Blueprint/Component/Actor/BP_AC_LivingActor.BP_AC_LivingActor_C")))
  (`/Engine/EditorBlueprintResources/StandardMacros.IsValid` _output_get
    (:`Is Valid`
      (`/Game/Blueprint/Component/Actor/BP_AC_LivingActor.TakeDamage` _loclivingcomponent (`self.CurrentDamage`) (`self.MyOwner`))
      (bind (_returnvalue _canpush_) (`self.PushVector` ActorHit))
      (if _canpush_
        (`/Game/Blueprint/Component/Actor/BP_AC_LivingActor.Pushed` _loclivingcomponent _returnvalue))
      (bind _output_get_2 (set `self.CurrentDamage` (* (`self.CurrentDamage`) 0.66)))
      (`self.SetAnimationStopValue` _output_get_2)
      (`KismetArrayLibrary.Array_AddUnique` (`self.AlreadyHitActor`) ActorHit))))

(fn `EffectOnHit`
  (params (ActorHit :type "Actor Object Reference"))
  ;[1 1 1] Effects when hitting something
  (`GameplayStatics.PlayWorldCameraShake` "/Game/Blueprint/CameraShake/BP_CameraShakeHitting.BP_CameraShakeHitting_C" (`self.K2_GetActorLocation` ActorHit) 0.0 500.0)
  (`AddComponent|NODE_AddNiagaraComponent-6` :`bManualAttachment` true :`RelativeTransform` (`SceneComponent.K2_GetComponentToWorld` (`self.Box`))))

(fn `HasAlreadyBeenHit?`
  (params (ActorHit :type "Actor Object Reference"))
  (returns (`AlreadyHit?` :type Boolean))
  (locals (LocActorHit :type "Actor Object Reference") (`LocAlreadyHit?` :type Boolean) (LocLivingComponent :type "/Game/Blueprint/Component/Actor/BP_AC_LivingActor Object Reference"))
  ;[1 1 1] Check if the actor hit has already been hit
  (set `local.LocAlreadyHit?` false)
  (set `local.LocActorHit` ActorHit)
  (for _array_element (`self.AlreadyHitActor`)
    (if (not (!= _array_element (`local.LocActorHit`)))
      (set `local.LocAlreadyHit?` true)))
  (if (`local.LocAlreadyHit?`)
    (return true)
    (else
      (return false))))

(fn `HeavyAttack`
  (returns (`CanAttack?` :type Boolean))
  (`self.CanAttack?`
    (:`True`
      (set `self.AttackState` "NewEnumerator2")
      (bind _output_get (set `self.CurrentDamage` (`self.HeavyAttackDamage`)))
      (`self.SetAnimationStopValue` _output_get)
      (set `self.IsAttacking?` true)
      (return false))))

(fn `HideWeapon`
  (params (`Hide?` :type Boolean))
  (if `Hide?`
    (`self.SetActorHiddenInGame` true)
    (else
      (`self.SetActorHiddenInGame` false))))

(fn `IsMyOwner?`
  (params (ActorHit :type "Actor Object Reference"))
  (returns (`Owner?` :type Boolean))
  ;[1 1 1] Check if the actor hit is not the one attacking
  (if (and (!= ActorHit (`self.MyOwner`)) (!= ActorHit self) (!= (`GameplayStatics.GetObjectClass` ActorHit) (`GameplayStatics.GetObjectClass` (`self.MyOwner`))) (`KismetSystemLibrary.IsValid` (`self.GetComponentByClass` ActorHit "/Game/Blueprint/Component/Actor/BP_AC_LivingActor.BP_AC_LivingActor_C")))
    (return false)
    (else
      (return true))))

(fn `LightAttack`
  (returns (`CanAttack?` :type Boolean))
  (`self.CanAttack?`
    (:`True`
      (set `self.AttackState` "NewEnumerator1")
      (bind _output_get (set `self.CurrentDamage` (`self.LightAttackDamage`)))
      (`self.SetAnimationStopValue` _output_get)
      (set `self.IsAttacking?` true)
      (return false))))

(fn `OnSpecialAttack`
  (returns (`CanAttack?` :type Boolean))
  (set `self.AttackState` "NewEnumerator3")
  (return false))

(fn `OnSpecialAttackReleased`
  (returns (`CanAttack?` :type Boolean))
  (return false))

(fn `OwnerTakeHit`
  (params (Attacker :type "Actor Object Reference") (Damage :type "Float (double-precision)"))
  (returns (`TakingDamage?` :type Boolean) (NewDamage :type "Float (double-precision)"))
  (return true Damage))

(fn `PushVector`
  (params (ActorHit :type "Actor Object Reference"))
  (returns (ReturnValue :type "Vector Structure") (`CanPush?` :type Boolean))
  (bind (_currentpushvector_x _currentpushvector_y _currentpushvector_z) (`KismetMathLibrary.BreakVector` (`self.CurrentPushVector`)))
  (bind (_returnvalue_x _returnvalue_y) (`KismetMathLibrary.BreakVector` (* (`KismetMathLibrary.Normal` (- (`self.K2_GetActorLocation` ActorHit) (`self.K2_GetActorLocation` (`self.MyOwner`)))) (`self.CurrentPushVector`))))
  (return (`KismetMathLibrary.MakeVector` _returnvalue_x _returnvalue_y _currentpushvector_z) (> _currentpushvector_z 5.0)))

(fn `SetAnimationStopValue`
  (params (DamageValue :type "Float (double-precision)"))
  ;[1 1 1] Set the stop timer between 0.00...1s and 0.16s (stop between 0 (or 1, not sure) and 10 frame)
  (set `self.CurrentStopTimer` (* 0.16 (- 1.0 (/ 0.16 (`KismetMathLibrary.FClamp` (* DamageValue 2.0) 0.16 10000.0)))))
  (return))

(fn `SetHitboxState`
  (params (`Active?` :type Boolean))
  (if `Active?`
    (`PrimitiveComponent.SetCollisionEnabled` (`self.Hitbox`) "QueryOnly")
    (else
      (`PrimitiveComponent.SetCollisionEnabled` (`self.Hitbox`) "NoCollision")
      (set `self.IsAttacking?` false)
      (set `self.AttackState` "NewEnumerator0")
      (`KismetArrayLibrary.Array_Clear` (`self.AlreadyHitActor`)))))

(fn `ThrowProjectile`
  (if (`KismetSystemLibrary.IsValidClass` (`self.Projectile`))
    (bind _asbp_player (cast `/Game/Blueprint/Player/BP_Player` (`self.MyOwner`)))
    (bind _sk_mannequin_arms (`/Game/Blueprint/Player/BP_Player.SK_Mannequin_Arms` _asbp_player))
    (bind _returnvalue (`|SpawnActorFromClass` (`self.Projectile`) (`KismetMathLibrary.MakeTransform` (+ (+ (`SceneComponent.K2_GetComponentLocation` _sk_mannequin_arms) (0.0 0.0 150.0)) (* (`SceneComponent.GetForwardVector` _sk_mannequin_arms) 50.0)) (`SceneComponent.K2_GetComponentRotation` _sk_mannequin_arms)) "Undefined" "OverrideRootScale" (`self.MyOwner`) null))
    (set `/Game/Blueprint/Weapons/Projectiles/BP_ProjectileParent.Damage` (`self.CurrentDamage`) _returnvalue)))

(fn `UserConstructionScript`)