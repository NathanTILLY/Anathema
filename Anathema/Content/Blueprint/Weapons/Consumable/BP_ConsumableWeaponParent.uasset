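; Parent Blueprint for consumable weapons that are picked up from the world and deal area damage with a limited number of uses.
; On pickup overlap, it hands itself to the actor's BP_AC_ConsumableWeapon component if the slot is empty, then hides and disables mesh collision.
; CreateHitbox spawns a timeline-scaled sphere that damages non-owner actors through BP_AC_LivingActor, and DeleteHitbox removes it.
; UsingWeapon decrements the remaining uses.
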(event `self.PickupHitbox.OnComponentBeginOverlap`
  (params (OverlappedComponent :type "PrimitiveComponent Object Reference") (OtherActor :type "Actor Object Reference") (OtherComp :type "PrimitiveComponent Object Reference") (OtherBodyIndex :type Integer) (bFromSweep :type Boolean) (SweepResult :type "HitResult Structure (by ref)"))
  (bind _returnvalue (`self.GetComponentByClass` OtherActor "/Game/Blueprint/Component/Actor/BP_AC_ConsumableWeapon.BP_AC_ConsumableWeapon_C"))
  ;[1 1 1] Collide with the player, get inside his inventory
  (`/Engine/EditorBlueprintResources/StandardMacros.IsValid` _returnvalue
    (:`Is Valid`
      (`/Engine/EditorBlueprintResources/StandardMacros.IsValid` (`/Game/Blueprint/Component/Actor/BP_AC_ConsumableWeapon.WeaponSlot` _returnvalue)
        (:`Is Not Valid`
          (`/Game/Blueprint/Component/Actor/BP_AC_ConsumableWeapon.PickUpWeapon` _returnvalue self)
          (`PrimitiveComponent.SetCollisionEnabled` (`self.Mesh`) "NoCollision")
          (`self.SetActorHiddenInGame` true))))))

(event `CreateHitbox`
  (bind _returnvalue (`AddComponent|NODE_AddSphereComponent-1` :`RelativeTransform` (`KismetMathLibrary.MakeTransform` (0.0 0.0 150.0))))
  (bind _output_get (set `self.Hitboxes` _returnvalue))
  (add `PrimitiveComponent.OnComponentBeginOverlap` _output_get (delegate `HitboxOverlap`))
  (bind (_direction _radius) (`Timeline|HitboxesRadius`)
    (:`Update`
      (`SphereComponent.SetSphereRadius` (`self.Hitboxes`) _radius true))))

(event `HitboxOverlap`
  (params (OverlappedComponent :type "PrimitiveComponent Object Reference") (OtherActor :type "Actor Object Reference") (OtherComp :type "PrimitiveComponent Object Reference") (OtherBodyIndex :type Integer) (bFromSweep :type Boolean) (SweepResult :type "HitResult Structure (by ref)"))
  (if (!= OtherActor (`self.GetOwner`))
    (`/Game/Blueprint/Component/Actor/BP_AC_LivingActor.TakeDamage` (`self.GetComponentByClass` OtherActor "/Game/Blueprint/Component/Actor/BP_AC_LivingActor.BP_AC_LivingActor_C") (`self.Damage`) (`self.GetOwner`) "NewEnumerator0")))

(event `DeleteHitbox`
  (`TimelineComponent.Stop` (`self.HitboxesRadius`))
  (`ActorComponent.K2_DestroyComponent` (`self.Hitboxes`)))

(fn `UserConstructionScript`)

(fn `UsingWeapon`
  (bind _result (`/Engine/EditorBlueprintResources/StandardMacros.DecrementInt` (`self.NumberOfUses`))
    (:`  `
      (set `self.NumberOfUses` _result))))