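; BP_Trident is a consumable weapon whose attack hitbox is a spawned BP_SpearProjectile instead of a melee volume.
; CreateHitbox spawns the projectile at the trident's location, aimed along the owning BP_Player's Scene rotation, and passes on the owner and the weapon's Damage.
; DeleteHitbox is empty, and AttackStart only calls the parent implementation.
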(event `self.CreateHitbox`
  (bind _returnvalue_location (`KismetMathLibrary.BreakTransform` (`self.GetTransform`)))
  (`|SpawnActorFromClass` "/Game/Blueprint/Weapons/Projectiles/BP_SpearProjectile.BP_SpearProjectile_C" (`KismetMathLibrary.MakeTransform` _returnvalue_location (`SceneComponent.K2_GetComponentRotation` (`/Game/Blueprint/Player/BP_Player.Scene` (cast `/Game/Blueprint/Player/BP_Player` (`self.GetOwner`) :!pure true)))) "AlwaysSpawn" "OverrideRootScale" (`self.GetOwner`) (`self.Damage`) null))

(event `self.DeleteHitbox`)

(fn `AttackStart`
  (`parent.AttackStart`))

(fn `UserConstructionScript`
  (`parent.UserConstructionScript`))