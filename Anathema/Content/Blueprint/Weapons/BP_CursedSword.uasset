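; Cursed sword weapon that spends the owner's souls on attacks and gives life-steal on hit.
; Light and heavy attacks, gated on the attack state, run the parent attack, then consume their cost from the owner's SoulHandler, ignoring the result.
; DealDamage heals the owner's LivingActor for a fraction of damage; a separate hit function also passes it negative damage.
; The special attack is an empty override returning false.
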(fn `ActorHit_0`
  (params (ActorHit :type "Actor Object Reference"))
  (returns (NewActorHit :type Boolean))
  (if true
    (`/Game/Blueprint/Component/Actor/BP_AC_LivingActor.TakeDamage` (`self.GetComponentByClass` (`self.MyOwner`) "/Game/Blueprint/Component/Actor/BP_AC_LivingActor.BP_AC_LivingActor_C") (* (`self.CurrentDamage`) -0.5) null)
    (return false)))

(fn `DealDamage`
  (params (ActorHit :type "Actor Object Reference"))
  (`parent.DealDamage` ActorHit)
  (`/Game/Blueprint/Component/Actor/BP_AC_LivingActor.Heal` (`self.GetComponentByClass` (`self.MyOwner`) "/Game/Blueprint/Component/Actor/BP_AC_LivingActor.BP_AC_LivingActor_C") (* (`self.CurrentDamage`) 0.33)))

(fn `HeavyAttack`
  (returns (`CanAttack?` :type Boolean))
  (if (`|EnumEquality` (`self.AttackState`) "NewEnumerator0")
    (`parent.HeavyAttack`)
    (bind _canusesoul_ (`/Game/Blueprint/Component/Actor/BP_AC_SoulHandler.ConsumeSoul` (`self.GetComponentByClass` (`self.MyOwner`) "/Game/Blueprint/Component/Actor/BP_AC_SoulHandler.BP_AC_SoulHandler_C") (`self.HeavyAttackCost`)))
    (if _canusesoul_
      (return false)
      (else
        (return false)))))

(fn `LightAttack`
  (returns (`CanAttack?` :type Boolean))
  (if (`|EnumEquality` (`self.AttackState`) "NewEnumerator0")
    (`parent.LightAttack`)
    (bind _canusesoul_ (`/Game/Blueprint/Component/Actor/BP_AC_SoulHandler.ConsumeSoul` (`self.GetComponentByClass` (`self.MyOwner`) "/Game/Blueprint/Component/Actor/BP_AC_SoulHandler.BP_AC_SoulHandler_C") (`self.LightAttackCost`)))
    (if _canusesoul_
      (return false)
      (else
        (return false)))))

(fn `OnSpecialAttack`
  (returns (`CanAttack?` :type Boolean))
  (return false))

(fn `UserConstructionScript`
  (`parent.UserConstructionScript`))