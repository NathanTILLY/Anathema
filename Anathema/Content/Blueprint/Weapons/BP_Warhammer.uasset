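; Warhammer weapon Blueprint that pairs the hammer with a spawned BP_Shield, attaching both to the owner's sockets on first pickup.
; The shield follows the weapon's hitbox and visibility and forwards its hits to shared hit logic.
; Holding special attack blocks frontal damage, tested by comparing a 2D cosine against BlockAngle/180.
; Heavy attacks set a push vector, light attacks clear it, and dealing damage breaks BP_Griveton_Waiting armor.
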(event `OnShieldHit`
  (params (ActorHit :type "Actor Object Reference"))
  ;[1 1 1] Attach Sword and shield to the owner
  (`self.ActorHitLogic` ActorHit))

(event `/Game/Blueprint/Interface/BPI_WeaponAttack.PickUp`
  (params (Owner :type "Actor Object Reference") (OwnerSkeletal :type "SkeletalMeshComponent Object Reference"))
  ;[1 1 1] Attach Sword and shield to the owner
  (`|ExecutionSequence`
    (:`then_0`
      (`/Engine/EditorBlueprintResources/StandardMacros.DoOnce` false
        (:`Completed`
          (`self.K2_AttachToComponent` OwnerSkeletal "SwordSocket" "SnapToTarget" "SnapToTarget" "SnapToTarget")
          (bind _returnvalue (`|SpawnActorFromClass` "/Game/Blueprint/Weapons/BP_Shield.BP_Shield_C" (`self.GetTransform`) "Undefined" "OverrideRootScale" null null))
          (bind _output_get (set `self.ShieldRef` _returnvalue))
          (`self.K2_AttachToComponent` _output_get OwnerSkeletal "ShieldSocket" "SnapToTarget" "SnapToTarget" "SnapToTarget" true)
          (add `/Game/Blueprint/Weapons/BP_Shield.OnHitSomething` (`self.ShieldRef`) (delegate `OnShieldHit`)))))
    (:`then_1`
      (set `self.MyOwner` Owner)
      (`self.SetActorHiddenInGame` self false)
      (`self.SetActorHiddenInGame` (`self.ShieldRef`) false))))

(fn `BlockingLogic`
  (params (Attacker :type "Actor Object Reference") (Damage :type "Float (double-precision)"))
  (returns (`TakingDamage?` :type Boolean) (NewDamage :type "Float (double-precision)"))
  (locals (StartingDamage :type "Float (double-precision)"))
  (bind _myowner (`self.MyOwner`))
  ;[1 1 1] Get the angle between the enemy and the player, if it exceed the BlockAngle, the player take damage
  (set `local.StartingDamage` Damage)
  (if (>= (`KismetMathLibrary.Vector_CosineAngle2D` (- (`self.K2_GetActorLocation` Attacker) (`self.K2_GetActorLocation` _myowner)) (`self.GetActorForwardVector` _myowner)) (/ (`self.BlockAngle`) 180.0))
    (set `self.BlockingHit?` true)
    (return false 0.0)
    (else
      (return true (`local.StartingDamage`)))))

(fn `DealDamage`
  (params (ActorHit :type "Actor Object Reference"))
  (`parent.DealDamage` ActorHit)
  (bind _asbp_griveton_waiting (cast `/Game/Blueprint/Enemies/GrivetonQuiAttend/BP_Griveton_Waiting` ActorHit))
  (`/Game/Blueprint/Enemies/BP_EnemyParent.ArmorBreak` _asbp_griveton_waiting))

(fn `HeavyAttack`
  (returns (`CanAttack?` :type Boolean))
  (`parent.HeavyAttack`)
  (set `self.CurrentPushVector` (2000.0 2000.0 100.0))
  (return false))

(fn `HideWeapon`
  (params (`Hide?` :type Boolean))
  (bind _shieldref (`self.ShieldRef`))
  (`parent.HideWeapon` `Hide?`)
  (if `Hide?`
    (`self.SetActorHiddenInGame` _shieldref true)
    (else
      (`self.SetActorHiddenInGame` _shieldref false))))

(fn `LightAttack`
  (returns (`CanAttack?` :type Boolean))
  (`parent.LightAttack`)
  (set `self.CurrentPushVector` (0.0 0.0 0.0))
  (return false))

(fn `OnSpecialAttack`
  (returns (`CanAttack?` :type Boolean))
  (set `self.IsBlocking?` true)
  (return false))

(fn `OnSpecialAttackReleased`
  (returns (`CanAttack?` :type Boolean))
  (set `self.IsBlocking?` false)
  (return false))

(fn `OwnerTakeHit`
  (params (Attacker :type "Actor Object Reference") (Damage :type "Float (double-precision)"))
  (returns (`TakingDamage?` :type Boolean) (NewDamage :type "Float (double-precision)"))
  ;[1 1 1] Modify the damage taken with the weapon
  (if (`self.IsBlocking?`)
    (bind (_takingdamage_ _newdamage) (`self.BlockingLogic` Attacker Damage))
    (return _takingdamage_ _newdamage)
    (else
      (return true Damage))))

(fn `SetHitboxState`
  (params (`Active?` :type Boolean))
  (bind _hitbox (`/Game/Blueprint/Weapons/BP_Shield.Hitbox` (`self.ShieldRef`)))
  (`parent.SetHitboxState` `Active?`)
  (if `Active?`
    (`PrimitiveComponent.SetCollisionEnabled` _hitbox "QueryOnly")
    (else
      (`PrimitiveComponent.SetCollisionEnabled` _hitbox "NoCollision"))))

(fn `UserConstructionScript`
  (`parent.UserConstructionScript`))