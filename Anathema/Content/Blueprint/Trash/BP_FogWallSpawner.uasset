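; BP_FogWallSpawner is a trigger actor that spawns BP_FogWalll actors when BP_Player overlaps its Box.
; The overlap runs a delayed loop that counts spawns up to AmountToSpawn and never resets the count.
; Each wall spawns a fixed distance along the spawner's forward vector with its rotation and scale, adjusting for collisions but always spawning, and a debug string prints.
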(event `self.ReceiveBeginPlay`)

(event `self.Box.OnComponentBeginOverlap`
  (params (OverlappedComponent :type "PrimitiveComponent Object Reference") (OtherActor :type "Actor Object Reference") (OtherComp :type "PrimitiveComponent Object Reference") (OtherBodyIndex :type Integer) (bFromSweep :type Boolean) (SweepResult :type "HitResult Structure (by ref)"))
  (cast `/Game/Blueprint/Player/BP_Player` OtherActor)
  (while (< (`self.AmountAlreadySpawned`) (`self.AmountToSpawn`))
    (`/Engine/EditorBlueprintResources/StandardMacros.IncrementFloat` (`self.AmountAlreadySpawned`)
      (:`  `
        (`KismetSystemLibrary.Delay` 0.2)
        (`|SpawnActorFromClass` "/Game/Blueprint/Trash/BP_FogWalll.BP_FogWalll_C" (`KismetMathLibrary.MakeTransform` (+ (* (`self.GetActorForwardVector` self) 300.0) (.location (`self.GetTransform` self))) (.rotation (`self.GetTransform` self)) (.scale (`self.GetTransform` self))) "AdjustIfPossibleButAlwaysSpawn" "OverrideRootScale" self null)
        (`KismetSystemLibrary.PrintString` "RATIO" true true (struct :`R` 1.0 :`B` 0.940684 :`A` 1.0))))))

(fn `UserConstructionScript`)