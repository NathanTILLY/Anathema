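; Blueprint math function library, apparently an unfinished attempt at finding the smallest circle containing an array of actors.
; The main function returns its circle without computing it, and MakeCircumcircle is empty.
; MakeDiameter builds a circle centered between two points using the MakeAverage helper.
; CircleContainsPoint only tests whether a point is nearly at the center, ignoring radius, and CircleContainsPoints returns false on every path.
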(fn `CircleContainsPoint`
  (params (Circle :type "/Game/Blueprint/Trash/F_Circle Structure") (Point :type "Vector Structure"))
  (returns (return :type Boolean))
  (return (`KismetMathLibrary.IsNearlyZero2D` (`KismetMathLibrary.MakeVector2D` (`KismetMathLibrary.Vector_Distance` (`.position_4_C34C7CAE422D36747C77E9922692DBD5` (break `/Game/Blueprint/Trash/F_Circle` Circle)) Point)))))

(fn `CircleContainsPoints`
  (params (Circle :type "/Game/Blueprint/Trash/F_Circle Structure") (Point :type "Array of Actor Object Reference") (__WorldContext :type "Object Object Reference"))
  (returns (return :type Boolean))
  (for _array_element Point
    (if (not (`self.CircleContainsPoint` (`local.Circle`) (`Actor.K2_GetActorLocation` _array_element)))
      (return false)))
  (return false))

(fn `MakeAverage`
  (params (floats :type "Array of Float (double-precision)"))
  (returns (average :type "Float (double-precision)"))
  (locals (tempTotal :type "Float (double-precision)"))
  (for _array_element floats
    (set `local.tempTotal` (+ (`local.tempTotal`) _array_element)))
  (return (/ (`local.tempTotal`) (`KismetMathLibrary.Conv_IntToDouble` (`KismetArrayLibrary.Array_Length` floats)))))

(fn `MakeCircumcircle`
  (params (NewParam :type "Vector Structure")))

(fn `MakeDiameter`
  (params (pointA :type "Vector Structure") (pointB :type "Vector Structure"))
  (returns (NewCircle :type "/Game/Blueprint/Trash/F_Circle Structure"))
  (locals (C :type "Vector Structure"))
  (set `local.C` (`KismetMathLibrary.MakeVector` (`self.MakeAverage` (`|MakeArray` (.x pointA) (.x pointB))) (`self.MakeAverage` (`|MakeArray` (.y pointA) (.y pointB))) (`self.MakeAverage` (`|MakeArray` (.z pointA) (.z pointB)))))
  (return (make `/Game/Blueprint/Trash/F_Circle` (`KismetMathLibrary.FMax` (`KismetMathLibrary.Vector_Distance` (`local.pointA`) (`local.C`)) (`KismetMathLibrary.Vector_Distance` (`local.pointA`) (`local.C`))) (`local.C`))))

(fn `ReturnSmallestCircleContainingArrayOfObject`
  (params (ArrayOfActors :type "Array of Actor Object Reference"))
  (returns (NewParam :type "/Game/Blueprint/Trash/F_Circle Structure"))
  (locals (ReturnedCircle :type "/Game/Blueprint/Trash/F_Circle Structure"))
  (`|ExecutionSequence`
    (:`then_5`
      (return (`local.ReturnedCircle`)))))