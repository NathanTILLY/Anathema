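; BP_CursedSwordProjectile is a damaging projectile, named for a cursed sword, that can pierce a limited number of targets.
; Its Box overlap event ignores the owner and looks for a BP_AC_LivingActor component on the other actor, passing it Damage with the owner as attacker.
; Each such hit decrements EnemyHitable, and the projectile destroys itself when that count reaches zero or below.
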(event `self.Box.OnComponentBeginOverlap`
  (params (OverlappedComponent :type "PrimitiveComponent Object Reference") (OtherActor :type "Actor Object Reference") (OtherComp :type "PrimitiveComponent Object Reference") (OtherBodyIndex :type Integer) (bFromSweep :type Boolean) (SweepResult :type "HitResult Structure (by ref)"))
  (if (!= OtherActor (`self.GetOwner`))
    (bind _output_get (set `self.ActorHitLivingComponent` (`self.GetComponentByClass` OtherActor "/Game/Blueprint/Component/Actor/BP_AC_LivingActor.BP_AC_LivingActor_C")))
    (`/Engine/EditorBlueprintResources/StandardMacros.IsValid` _output_get
      (:`Is Valid`
        (`/Game/Blueprint/Component/Actor/BP_AC_LivingActor.TakeDamage` _output_get (`self.Damage`) (`self.GetOwner`))
        (bind _result (`/Engine/EditorBlueprintResources/StandardMacros.DecrementInt` (`self.EnemyHitable`))
          (:`  `
            (if (<= _result 0)
              (`self.K2_DestroyActor`))))))))

(fn `UserConstructionScript`)