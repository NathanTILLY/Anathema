(fn `Get Owner as Character`
  (returns (AsCharacter :type "Character Object Reference") (Sucess :type Boolean))
  (bind (_ascharacter _bsuccess) (cast `Character` (`self.GetOwner`) :!pure true))
  (return _ascharacter _bsuccess))

(fn `Implement`
  (params (WeaponData :type "/Game/Blueprint/Trash/BP_WeaponParentDataAsset Object Reference"))
  (bind _output_get (set `self.WeaponData` WeaponData))
  (`self.SetStaticMesh` (`/Game/Blueprint/Trash/BP_WeaponParentDataAsset.WeaponMesh` _output_get)))

(fn `ImplementSword`
  (`self.Implement` (select `int` (`KismetMathLibrary.RandomInteger` 5) :`0` "/Game/Blueprint/Trash/NewDataAsset.NewDataAsset" :`1` "/Game/Blueprint/Trash/NewDataAsset1.NewDataAsset1" :`2` "/Game/Blueprint/Trash/NewDataAsset2.NewDataAsset2" :`3` "/Game/Blueprint/Trash/NewDataAsset3.NewDataAsset3" :`4` "/Game/Blueprint/Trash/NewDataAsset4.NewDataAsset4" :`5` "/Game/Blueprint/Trash/NewDataAsset5.NewDataAsset5" :!type "/Game/Blueprint/Trash/BP_WeaponParentDataAsset Object Reference")))

(fn `Push`)

(fn `WeaponHeavyAttack`)

(fn `WeaponLightAttack`
  (`/Game/Blueprint/Trash/BP_WeaponParentDataAsset.LightAttack` (`self.WeaponData`) self))