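; Fire light actor with an animated-shadow light function, meant to flicker only while the player is near.
; Construction creates a dynamic instance of a torch material, caches its noise parameters (Tiling and Animation swapped), assigns it to the light, and applies custom radius, intensity and color.
; Tick checks player overlap with the radius sphere to call play or stop.
; Both animation events are empty, and the random noise-size update is unwired.
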(event `self.ReceiveTick`
  (params (DeltaSeconds :type "Float (single-precision)"))
  (if (`PrimitiveComponent.IsOverlappingActor` (`self.FireLight_OnOffRaduis`) (`GameplayStatics.GetPlayerCharacter` 0))
    (`self.FireShadesAnimation_Play`)
    (else
      (`self.FireShadesAnimation_Stop`))))

(event `FireShadesAnimation_Play`)

(event `FireShadesAnimation_Stop`)

(fn `GetScalarParametersValues`
  (params (Target :type "MaterialInstanceDynamic Object Reference") (ScalarParameter1_Name :type Name) (ScalarParameter2_Name :type Name) (ScalarParameter3_Name :type Name) (ScalarParameter4_Name :type Name))
  (returns (ScalarParameter1_Value :type "Float (double-precision)") (ScalarParameter2_Value :type "Float (double-precision)") (ScalarParameter3_Value :type "Float (double-precision)") (ScalarParameter4_Value :type "Float (double-precision)"))
  (bind _returnvalue (`MaterialInstanceDynamic.K2_GetScalarParameterValue` Target ScalarParameter1_Name))
  (bind _returnvalue_2 (`MaterialInstanceDynamic.K2_GetScalarParameterValue` Target ScalarParameter2_Name))
  (bind _returnvalue_3 (`MaterialInstanceDynamic.K2_GetScalarParameterValue` Target ScalarParameter3_Name))
  (bind _returnvalue_4 (`MaterialInstanceDynamic.K2_GetScalarParameterValue` Target ScalarParameter4_Name))
  (return _returnvalue _returnvalue_2 _returnvalue_3 _returnvalue_4))

(fn `UserConstructionScript`
  ;[1 1 1] Create Instance of Material "Fire" Effect, gets and sets varaibles of all Scalar Parameters, and assign it to Light Function
  (bind _returnvalue (`KismetMaterialLibrary.CreateDynamicMaterialInstance` "/Game/VFX/MP_TorchEffect_TEMP.MP_TorchEffect_TEMP"))
  (bind _output_get (set `self.MI_LightFunction` _returnvalue))
  (bind (_scalarparameter1_value _scalarparameter2_value _scalarparameter3_value _scalarparameter4_value) (`self.GetScalarParametersValues` _output_get "Noise_Animation" "Noise_Intensity" "Noise_Size" "Noise_Tiling"))
  (set `self.Tiling_Value` _scalarparameter1_value)
  (set `self.Intensity_Value` _scalarparameter2_value)
  (set `self.Size_Value` _scalarparameter3_value)
  (set `self.Animation_Value` _scalarparameter4_value)
  (`LightComponent.SetLightFunctionMaterial` (`self.FireLight`) (`self.MI_LightFunction`))
  ;[1 1 1] Sets User Light Parameters
  (`SphereComponent.SetSphereRadius` (`self.FireLight_OnOffRaduis`) (`self.Custom_Light_OnOffRadius`) true)
  (`LightComponent.SetIntensity` (`self.FireLight`) (`self.Custom_Light_Intensity`))
  (`LightComponent.SetLightColor` (`self.FireLight`) (`self.Custom_Light_Color`) true))