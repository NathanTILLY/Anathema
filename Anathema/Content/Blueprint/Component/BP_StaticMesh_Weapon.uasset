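; Static mesh weapon component that drives a wielder's attacks, hit response and projectile throws, with stats and attack logic held in WeaponData.
; Selecting it shows the mesh and applies the weapon's anim class, and attack state gates light attacks until the hitbox is disabled.
; Hits apply damage and pushback through BP_AC_LivingActor, then trigger camera shake, sparks and hit-stop by freezing the owner's time dilation.
; Projectiles spawn in front of BP_Player's scene component.
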(event `StopAnimation`
  (bind _returnvalue (`self.GetOwner`))
  (set `Actor.CustomTimeDilation` 0.0 _returnvalue)
  (`KismetSystemLibrary.Delay` (`/Game/Data/Asset/BPDA_WeaponParent.CurrentHitStop` (`self.WeaponData`)))
  (set `Actor.CustomTimeDilation` 1.0 _returnvalue))

(fn `ActorHit`
  (params (ActorHit :type "Actor Object Reference"))
  (`self.CanDamageActor` ActorHit)
  (if (!= ActorHit (`self.GetOwner`))
    (`self.DealDamage` ActorHit)
    (`self.EffectOnHit`)))

(fn `CanDamageActor`
  (params (ActorHit :type "Actor Object Reference (by ref)"))
  (returns (`AlreadyHit?` :type Boolean))
  (locals (LocActorHit :type "Actor Object Reference") (`LocAlreadyHit?` :type Boolean))
  (bind _output_get (set `local.LocActorHit` ActorHit))
  (`/Engine/EditorBlueprintResources/StandardMacros.IsValid` (`Actor.GetComponentByClass` _output_get "/Game/Blueprint/Component/Actor/BP_AC_LivingActor.BP_AC_LivingActor_C")
    (:`Is Valid`
      (if (!= (`local.LocActorHit`) (`self.GetOwner`))
        (set `local.LocAlreadyHit?` false)
        (for _array_element (`self.AlreadyHitActor`)
          (if (not (!= _array_element (`local.LocActorHit`)))
            (set `local.LocAlreadyHit?` true)))
        (if (`local.LocAlreadyHit?`)
          (return true)
          (else
            (return false)))))))

(fn `DealDamage`
  (params (ActorHit :type "Actor Object Reference"))
  (locals (LocLivingComponent :type "/Game/Blueprint/Component/Actor/BP_AC_LivingActor Object Reference"))
  (bind _returnvalue (`self.GetOwner`))
  (set `local.LocLivingComponent` (`Actor.GetComponentByClass` ActorHit "/Game/Blueprint/Component/Actor/BP_AC_LivingActor.BP_AC_LivingActor_C"))
  (`/Game/Blueprint/Component/Actor/BP_AC_LivingActor.TakeDamage` (`local.LocLivingComponent`) (`/Game/Data/Asset/BPDA_WeaponParent.CurrentDamage` (`self.WeaponData`)) _returnvalue)
  (bind (_returnvalue_2 _canpush_) (`/Game/Data/Asset/BPDA_WeaponParent.PushVector` (`self.WeaponData`) ActorHit _returnvalue))
  (if _canpush_
    (`/Game/Blueprint/Component/Actor/BP_AC_LivingActor.Pushed` (`local.LocLivingComponent`) _returnvalue_2))
  (`/Game/Data/Asset/BPDA_WeaponParent.ReduceDamageAndHitStop` (`self.WeaponData`))
  (`KismetArrayLibrary.Array_AddUnique` (`self.AlreadyHitActor`) ActorHit))

(fn `EffectOnHit`
  (bind (_returnvalue_location _returnvalue_rotation _returnvalue_scale) (`KismetMathLibrary.BreakTransform` (`self.GetSocketTransform` "SparkSocket")))
  (`GameplayStatics.PlayWorldCameraShake` "/Game/Blueprint/CameraShake/BP_CameraShakeHitting.BP_CameraShakeHitting_C" (`Actor.K2_GetActorLocation` (`self.GetOwner`)) 0.0 500.0)
  (`NiagaraFunctionLibrary.SpawnSystemAtLocation` "/Game/VFX/Spark/NS_SparkSystem.NS_SparkSystem" _returnvalue_location _returnvalue_rotation _returnvalue_scale)
  (`self.StopAnimation`))

(fn `Implement`)

(fn `LightAttack`
  (`self.CanAttack`
    (:`true`
      (bind _output_get (set `self.AttackState` "NewEnumerator1"))
      (`/Game/Data/Asset/BPDA_WeaponParent.LightAttack` (`self.WeaponData`) _output_get))))

(fn `SelectWeapon`
  (params (OwnerSkeletal :type "SkeletalMeshComponent Object Reference"))
  (`SkeletalMeshComponent.SetAnimInstanceClass` OwnerSkeletal (`/Game/Data/Asset/BPDA_WeaponParent.WeaponAnim` (`self.WeaponData`)))
  (`self.SetHiddenInGame` self false true))

(fn `SetHitboxState`
  (params (`Active?` :type Boolean))
  (if `Active?`
    (`self.SetCollisionEnabled` (`self.Hitbox`) "QueryOnly")
    (`KismetSystemLibrary.PrintString` "Hitbox")
    (else
      (`self.SetCollisionEnabled` (`self.Hitbox`) "NoCollision")
      (set `self.Attacking?` false)
      (set `self.AttackState` "NewEnumerator0")
      (`KismetArrayLibrary.Array_Clear` (`self.AlreadyHitActor`)))))

(fn `ThrowProjectile`
  (if (`KismetSystemLibrary.IsValidClass` (`self.Projectile`))
    (bind _asbp_player (cast `/Game/Blueprint/Player/BP_Player` (`self.GetOwner`)))
    (bind _scene (`/Game/Blueprint/Player/BP_Player.Scene` _asbp_player))
    (`|SpawnActorFromClass` (`self.Projectile`) (`KismetMathLibrary.MakeTransform` (+ (+ (`self.K2_GetComponentLocation` _scene) (0.0 0.0 -10.0)) (* (`self.GetForwardVector` _scene) 50.0)) (`self.K2_GetComponentRotation` _scene)) "Undefined" "OverrideRootScale" (`self.GetOwner`) null)))

(fn `UnselectWeapon`
  (`self.SetHiddenInGame` self true true))