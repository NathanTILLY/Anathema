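; Actor component that tracks the player's soul resource, clamped between zero and a maximum.
; GainSoul adds soul unless the owning BP_Player's current weapon is the Cursed Sword.
; ConsumeSoul succeeds whenever any soul remains, even below the cost, and otherwise fires OnLastSoulUsed and returns false.
; Both gains and successful spends fire the OnsoulConsumed dispatcher to announce the change.
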(fn `ConsumeSoul`
  (params (SoulCost :type "Float (double-precision)"))
  (returns (`CanUseSoul?` :type Boolean))
  ;[1 1 1] Can't use soul if equal to zero or weapon is CursedSword
  (if (> (`self.CurrentSoul`) 0.0)
    (set `self.CurrentSoul` (`KismetMathLibrary.FClamp` (- (`self.CurrentSoul`) SoulCost) 0.0 (`self.MaxSoul`)))
    (`self.OnsoulConsumed` false)
    (return true)
    (else
      (`self.OnLastSoulUsed`)
      (return false))))

(fn `GainSoul`
  (params (AddedSoul :type "Float (double-precision)"))
  ;[1 1 1] Gain soul when enemy dies with weapon other than the Cursed Sword
  (if (not (== (`GameplayStatics.GetObjectClass` (`/Game/Blueprint/Player/BP_Player.CurrentWeapon` (cast `/Game/Blueprint/Player/BP_Player` (`self.GetOwner`) :!pure true))) "/Game/Blueprint/Component/BP_CursedSwordComponent.BP_CursedSwordComponent_C"))
    (set `self.CurrentSoul` (`KismetMathLibrary.FClamp` (+ AddedSoul (`self.CurrentSoul`)) 0.0 (`self.MaxSoul`)))
    (`self.OnsoulConsumed` false)))