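; BP_AC_TicketHandler is an actor component that lets its owner take a single ticket from the player.
; TakeTicket checks that the referenced player has tickets left and that this component holds none.
; It then decrements the player's count, records the ticket locally and sets the "Ticket" Blackboard key to true, exposing the state to AI logic.
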(fn `TakeTicket`
  (bind _tickets (`/Game/Blueprint/Player/BP_Player.Tickets` (`self.PlayerRef`)))
  (if (> _tickets 0)
    (if (== (`self.MyTicketIGot`) 0)
      (set `/Game/Blueprint/Player/BP_Player.Tickets` (- _tickets 1) (`self.PlayerRef`))
      (set `self.MyTicketIGot` (+ 0 1))
      (`BlackboardComponent.SetValueAsBool` (`AIBlueprintHelperLibrary.GetBlackboard` null) "Ticket" true))))