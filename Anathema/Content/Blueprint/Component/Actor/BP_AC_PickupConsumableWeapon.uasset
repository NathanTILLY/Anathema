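; Actor component that lets the player pick up and temporarily use a consumable weapon.
; Pickup attaches the weapon to the mesh's SwordSocket, stores it and binds the player's consumable weapon input.
; Use swaps in the weapon's anim class, hides the regular weapon, unbinds switching and attack, and reveals the consumable.
; After a fixed delay, AttackEnd hides it, switches to weapon slot zero and rebinds switching.
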(event `AttackDelay`
  (`KismetSystemLibrary.Delay` 4.0)
  (`self.AttackEnd`))

(fn `AttackEnd`
  (bind _player (`self.Player`))
  (`Actor.SetActorHiddenInGame` (`self.WeaponSlot`) true)
  (`/Game/Blueprint/Player/BP_Player.HideWeapon` _player)
  (`/Game/Blueprint/Player/BP_Player.SwitchWeapon` _player 0)
  (`/Game/Blueprint/Player/BP_Player.BindSwitchWeapon` _player))

(fn `PickUpWeapon`
  (params (Weapon :type "/Game/Blueprint/Weapons/Consumable/BP_ConsumableWeaponParent Object Reference"))
  (locals (LocWeapon :type "/Game/Blueprint/Weapons/Consumable/BP_ConsumableWeaponParent Object Reference"))
  (`Actor.K2_AttachToComponent` Weapon (`self.SkeletalMesh`) "SwordSocket" "SnapToTarget" "SnapToTarget" "SnapToTarget" true)
  (set `self.WeaponSlot` Weapon)
  (`/Game/Blueprint/Player/BP_Player.BindConsumableWeapon` (`self.Player`)))

(fn `SetupComponent`
  (params (SkeletalMesh :type "SkeletalMeshComponent Object Reference") (Player :type "/Game/Blueprint/Player/BP_Player Object Reference"))
  (set `self.SkeletalMesh` SkeletalMesh)
  (set `self.Player` Player))

(fn `UseWeapon`
  (bind _player (`self.Player`))
  (`SkeletalMeshComponent.SetAnimInstanceClass` (`self.SkeletalMesh`) (`/Game/Blueprint/Weapons/Consumable/BP_ConsumableWeaponParent.AnimInstance` (`self.WeaponSlot`)))
  (`/Game/Blueprint/Player/BP_Player.HideWeapon` _player)
  (`/Game/Blueprint/Player/BP_Player.UnbindSwitchWeapon` _player)
  (`/Game/Blueprint/Player/BP_Player.UnbindAttack` (`self.Player`))
  (`Actor.SetActorHiddenInGame` (`self.WeaponSlot`) false)
  (`self.AttackDelay`))