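; Actor component that manages the on-screen objective text for player 0 through a WBP_Objectives widget.
; SetPlayerObjectives removes any existing widget, stores the sentence and shows a new widget if it is not empty.
; LoadObjectives shows a saved sentence and restores the level objectives map, without updating CurrentObjectives.
; ClearObjectives calls FadeOut, removes the widget immediately and empties the current sentence.
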(fn `ClearObjectives`
  (bind _w_objectives (`self.W_Objectives`))
  (`/Game/Blueprint/UI/WBP_Objectives.FadeOut` _w_objectives)
  (`Widget.RemoveFromParent` _w_objectives)
  (set `self.CurrentObjectives` ""))

(fn `LoadObjectives`
  (params (ObjectivesSentence :type String) (SavedObjectivesMap :type "Map of String to Boolean"))
  (bind _returnvalue (`|CreateWidget` "/Game/Blueprint/UI/WBP_Objectives.WBP_Objectives_C" (`GameplayStatics.GetPlayerController` 0) ObjectivesSentence))
  (`UserWidget.AddToViewport` _returnvalue 0)
  (set `self.W_Objectives` _returnvalue)
  (set `self.LevelObjectivesMap` (`local.SavedObjectivesMap`)))

(fn `SetPlayerObjectives`
  (params (ObjectivesSentence :type String))
  (bind _w_objectives (`self.W_Objectives`))
  (`/Engine/EditorBlueprintResources/StandardMacros.IsValid` _w_objectives
    (:`Is Valid`
      (`Widget.RemoveFromParent` _w_objectives))
    (:`Is Not Valid`
      _))
  (bind _output_get (set `self.CurrentObjectives` (`local.ObjectivesSentence`)))
  (if (not (`KismetStringLibrary.IsEmpty` _output_get))
    (bind _returnvalue (`|CreateWidget` "/Game/Blueprint/UI/WBP_Objectives.WBP_Objectives_C" (`GameplayStatics.GetPlayerController` 0) _output_get))
    (bind _output_get_2 (set `self.W_Objectives` _returnvalue))
    (`UserWidget.AddToViewport` _output_get_2 0)))