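; BP_AC_LineTraceInteractable is an actor component that detects interactable actors in front of its owner's camera.
; It caches the owner's camera on BeginPlay and line-traces forward on the Visibility channel each Tick.
; Hitting a BPI_Interact actor shows a WBP_Interact widget and stores the actor as CurrentInteractableActor, gated by a DoOnce.
; A miss or non-interactable hit removes the widget, clears the actor and resets the gate.
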(event `self.ReceiveBeginPlay`
  (bind _returnvalue (`Actor.GetComponentByClass` (`self.GetOwner`) "/Script/Engine.CameraComponent"))
  (`/Engine/EditorBlueprintResources/StandardMacros.IsValid` _returnvalue
    (:`Is Valid`
      (set `self.OwnerCamera` _returnvalue)
      (`self.SetComponentTickEnabled` true))))

(event `self.ReceiveTick`
  (params (DeltaSeconds :type "Float (single-precision)"))
  (bind _ownercamera (`self.OwnerCamera`))
  (bind _returnvalue (`SceneComponent.K2_GetComponentLocation` _ownercamera))
  (bind (_outhit _returnvalue_2) (`KismetSystemLibrary.LineTraceSingle` _returnvalue (+ _returnvalue (* (`SceneComponent.GetForwardVector` _ownercamera) (`self.Distance`))) "TraceTypeQuery1"))
  (if _returnvalue_2
    (bind (_bblockinghit _binitialoverlap _time _distance _location _impactpoint _normal _impactnormal _physmat _hitactor) (`GameplayStatics.BreakHitResult` _outhit))
    (if (`KismetSystemLibrary.DoesImplementInterface` _hitactor "/Game/Blueprint/Interface/BPI_Interact.BPI_Interact_C")
      (`/Engine/EditorBlueprintResources/StandardMacros.DoOnce` false :!label _label
        (:`Completed`
          (bind _returnvalue_3 (`|CreateWidget` "/Game/Blueprint/UI/WBP_Interact.WBP_Interact_C"))
          (bind _output_get (set `self.W_Interact` _returnvalue_3))
          (`UserWidget.AddToViewport` _output_get 0)
          (set `self.CurrentInteractableActor` _hitactor)))
      (else
        (if (`KismetSystemLibrary.IsValid` (`self.W_Interact`)) :!label _label_2
          (`Widget.RemoveFromParent` (`self.W_Interact`))
          (set `self.W_Interact` null)
          (set `self.CurrentInteractableActor` null)
          (goto _label :!via `Reset`))))
    (else
      (goto _label_2))))