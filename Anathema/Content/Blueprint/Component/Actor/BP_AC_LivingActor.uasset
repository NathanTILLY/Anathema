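; BP_AC_LivingActor is an actor component that gives its owner health, damage, healing and knockback handling.
; TakeDamage first lets a valid OwnerWeapon veto or alter the hit, then reduces clamped HP and fires OnTakingDamage, plus OnDeath at zero.
; Heal restores clamped HP and fires OnHeal.
; Pushed launches a Character owner only while it is moving on the ground.
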(fn `Heal`
  (params (HealValue :type "Float (double-precision)"))
  ;[1 1 1] Heal Actor
  (set `self.CurrentHp` (`KismetMathLibrary.FClamp` (+ (`self.CurrentHp`) HealValue) 0.0 (`self.MaxHp`)))
  (`self.OnHeal`))

(fn `Pushed`
  (params (PushVector :type "Vector Structure"))
  (bind _ascharacter (cast `Character` (`self.GetOwner`)))
  (if (`NavMovementComponent.IsMovingOnGround` (`Character.CharacterMovement` _ascharacter))
    (`Character.LaunchCharacter` _ascharacter PushVector false false)))

(fn `TakeDamage`
  (params (Damage :type "Float (double-precision)") (AttackOwner :type "Actor Object Reference"))
  ;[1 1 1] Taking damage, check if the weapon do something, reduce Health from actor, call OnTakingDamage if the actor does something when taking damage. If the actor has no health call the OnDeath event
  (bind (_takingdamage_ _newdamage) (`self.WeaponTakingHitLogic` AttackOwner Damage))
  (if _takingdamage_
    (set `self.CurrentHp` (`KismetMathLibrary.FClamp` (- (`self.CurrentHp`) _newdamage) 0.0 (`self.MaxHp`)))
    (`self.OnTakingDamage` AttackOwner _newdamage)
    (if (<= (`self.CurrentHp`) 0.0)
      (`self.OnDeath` AttackOwner))))

(fn `WeaponTakingHitLogic`
  (params (Attacker :type "Actor Object Reference") (Damage :type "Float (double-precision)"))
  (returns (`TakingDamage?` :type Boolean) (NewDamage :type "Float (double-precision)"))
  (bind _ownerweapon (`self.OwnerWeapon`))
  ;[1 1 1] Check if the weapon change the damage taken and apply new value
  (`/Engine/EditorBlueprintResources/StandardMacros.IsValid` _ownerweapon
    (:`Is Valid`
      (bind (_takingdamage_ _newdamage) (message `/Game/Blueprint/Interface/BPI_WeaponAttack.OwnerTakeHit` _ownerweapon Attacker Damage))
      (return _takingdamage_ _newdamage))
    (:`Is Not Valid`
      (return true Damage))))