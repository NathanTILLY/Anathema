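; Actor component that manages the player's consumable skill weapon, from pickup and use to drop.
; Pickup attaches the weapon to the sword socket, binds its input and triggers a first-time tutorial through the game instance.
; Use swaps the anim class, hides the regular weapon and unbinds other actions before starting the attack.
; Attack end restores the last weapon and bindings, then destroys the consumable when no uses remain or rebinds it.
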(event `AttackDelay`
  (`KismetSystemLibrary.Delay` 3.0)
  (`self.AttackEnd`))

(fn `AttackEnd`
  (bind _player (`self.Player`))
  (bind _weaponslot (`self.WeaponSlot`))
  ;[1 1 1] When the attack is done
  (`/Engine/EditorBlueprintResources/StandardMacros.IsValid` _weaponslot
    (:`Is Valid`
      (`/Game/Blueprint/Weapons/Consumable/BP_ConsumableWeaponParent.AttackEnd` _weaponslot)
      (`/Game/Blueprint/Player/BP_Player.HideWeapon` _player)
      (`/Game/Blueprint/Player/BP_Player.SwitchWeapon` _player (`/Game/Blueprint/Player/BP_Player.LastWeaponIndex` _player))
      (`/Game/Blueprint/Player/BP_Player.BindSwitchWeapon` _player)
      (`/Game/Blueprint/Player/BP_Player.BindInteract` (`self.Player`))
      (if (<= (`/Game/Blueprint/Weapons/Consumable/BP_ConsumableWeaponParent.NumberOfUses` (`self.WeaponSlot`)) 0)
        (`/Game/Blueprint/Player/BP_Player.UnbindConsumableWeapon` (`self.Player`))
        (`Actor.K2_DestroyActor` (`self.WeaponSlot`))
        (else
          (`/Game/Blueprint/Player/BP_Player.BindConsumableWeapon` (`self.Player`)))))))

(fn `DropWeapon`
  (bind _weaponslot (`self.WeaponSlot`))
  (`Actor.K2_DetachFromActor` _weaponslot "KeepWorld" "KeepWorld" "KeepWorld")
  (`/Game/Blueprint/Weapons/Consumable/BP_ConsumableWeaponParent.Drop Weapon` _weaponslot (* (`Actor.GetActorForwardVector` (`self.Player`)) (`self.DropForce`))))

(fn `PickUpWeapon`
  (params (Weapon :type "/Game/Blueprint/Weapons/Consumable/BP_ConsumableWeaponParent Object Reference"))
  (locals (LocWeapon :type "/Game/Blueprint/Weapons/Consumable/BP_ConsumableWeaponParent Object Reference"))
  (bind _player (`self.Player`))
  (bind _asbp_game_instance (cast `/Game/Blueprint/BP_GameInstance` (`GameplayStatics.GetGameInstance`) :!pure true))
  ;[1 1 1] When picking up the weapon
  (`Actor.K2_AttachToComponent` Weapon (`self.SkeletalMesh`) "SwordSocket" "SnapToTarget" "SnapToTarget" "SnapToTarget" true)
  (bind _output_get (set `self.WeaponSlot` Weapon))
  (`Actor.SetOwner` _output_get _player)
  (`/Game/Blueprint/Player/BP_Player.BindConsumableWeapon` _player)
  (if (`/Game/Blueprint/BP_GameInstance.FirstTimePickUp` _asbp_game_instance)
    (set `/Game/Blueprint/BP_GameInstance.FirstTimePickUp` false _asbp_game_instance)
    (`/Game/Blueprint/BP_GameInstance.HowToConsumable` _asbp_game_instance)
    (`GameplayStatics.PlaySound2D` "/Game/Audio/Sound2_0/GrabWeapon_Cue.GrabWeapon_Cue" 1.0 1.0 0.0 null null)))

(fn `SetHitboxes`
  (params (`Active?` :type Boolean))
  (if `Active?`
    (`/Game/Blueprint/Weapons/Consumable/BP_ConsumableWeaponParent.CreateHitbox` (`self.WeaponSlot`))
    (else
      (`/Game/Blueprint/Weapons/Consumable/BP_ConsumableWeaponParent.DeleteHitbox` (`self.WeaponSlot`)))))

(fn `SetupComponent`
  (params (SkeletalMesh :type "SkeletalMeshComponent Object Reference") (Player :type "/Game/Blueprint/Player/BP_Player Object Reference"))
  ;[1 1 1] Set the player ref and his skeletal
  (set `self.SkeletalMesh` SkeletalMesh)
  (set `self.Player` Player))

(fn `UseWeapon`
  (bind _player (`self.Player`))
  ;[1 1 1] When pressing the skillWeapon button : Unbind the skill, set the new anim instance, hide the old weapon, unbind switching weapon and attacks, show the skill weapon and decrement the number of uses
  (clear `/Game/Blueprint/Player/BP_PlayerController.OnWeaponSkillPressed` (`/Game/Blueprint/Player/BP_Player.MyController` (`self.Player`)))
  (`SkeletalMeshComponent.SetAnimInstanceClass` (`self.SkeletalMesh`) (`/Game/Blueprint/Weapons/Consumable/BP_ConsumableWeaponParent.AnimInstance` (`self.WeaponSlot`)))
  (`/Game/Blueprint/Player/BP_Player.HideWeapon` _player)
  (`/Game/Blueprint/Player/BP_Player.UnbindSwitchWeapon` _player)
  (`/Game/Blueprint/Player/BP_Player.UnbindAttack` (`self.Player`))
  (`/Game/Blueprint/Player/BP_Player.UnbindInteract` (`self.Player`))
  (`/Game/Blueprint/Weapons/Consumable/BP_ConsumableWeaponParent.AttackStart` (`self.WeaponSlot`)))