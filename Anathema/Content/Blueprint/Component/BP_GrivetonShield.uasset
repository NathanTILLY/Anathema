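; BP_GrivetonShield is a shield component that filters damage to its owner by attacker type.
; Its OwnerTakeDamage override always calls the parent first, then keeps that result only for attackers of exact class BP_Player or of BP_TrapParent and its children.
; Any other attacker still registers as a hit, but its damage becomes zero.
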(fn `OwnerTakeDamage`
  (params (Attacker :type "Actor Object Reference") (Damage :type "Float (double-precision)"))
  (returns (`TakingDamage?` :type Boolean) (NewDamage :type "Float (double-precision)"))
  (bind _returnvalue (`GameplayStatics.GetObjectClass` Attacker))
  (bind (_takingdamage_ _newdamage) (`parent.OwnerTakeDamage` Attacker Damage))
  (if (or (== _returnvalue "/Game/Blueprint/Player/BP_Player.BP_Player_C") (`KismetMathLibrary.ClassIsChildOf` _returnvalue "/Game/Blueprint/Trap/BP_TrapParent.BP_TrapParent_C"))
    (return _takingdamage_ _newdamage)
    (else
      (return true 0.0))))