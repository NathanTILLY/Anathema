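; Cursed sword weapon component that spends the owner's souls on attacks and heals the owner on hit.
; Light, heavy and special attacks check CanAttack, set AttackState, call into WeaponData, then charge that state's soul cost through the SoulHandler component.
; DealDamage extends the parent with lifesteal, healing the LivingActor component for a quarter of current damage.
; Heavy and special attacks only look up their attack value, and SpecialAttackStop is empty.
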(fn `ConsumeSoul`
  (`/Game/Blueprint/Component/Actor/BP_AC_SoulHandler.ConsumeSoul` (`Actor.GetComponentByClass` (`self.GetOwner`) "/Game/Blueprint/Component/Actor/BP_AC_SoulHandler.BP_AC_SoulHandler_C") (`BlueprintMapLibrary.Map_Find` (`self.AttacksSoulCost`) (`self.AttackState`))))

(fn `DealDamage`
  (params (ActorHit :type "Actor Object Reference"))
  (`parent.DealDamage` ActorHit)
  (`/Game/Blueprint/Component/Actor/BP_AC_LivingActor.Heal` (`Actor.GetComponentByClass` (`self.GetOwner`) "/Game/Blueprint/Component/Actor/BP_AC_LivingActor.BP_AC_LivingActor_C") (* (`/Game/Data/Asset/BPDA_WeaponParent.CurrentDamage` (`self.WeaponData`)) 0.25)))

(fn `HeavyAttack`
  (bind _canattack_ (`self.CanAttack`))
  (if _canattack_
    (bind _output_get (set `self.AttackState` "NewEnumerator2"))
    (`/Game/Data/Asset/BPDA_WeaponParent.GetAttackValueByName` (`self.WeaponData`) (`|GetEnumeratorNameAsString` _output_get))
    (`self.ConsumeSoul`)))

(fn `LightAttack`
  (bind _canattack_ (`self.CanAttack`))
  (if _canattack_
    (bind _output_get (set `self.AttackState` "NewEnumerator1"))
    (`/Game/Data/Asset/BPDA_WeaponParent.LightAttack` (`self.WeaponData`) _output_get)
    (`self.ConsumeSoul`)))

(fn `SpecialAttack`
  (bind _canattack_ (`self.CanAttack`))
  (if _canattack_
    (bind _output_get (set `self.AttackState` "NewEnumerator3"))
    (`/Game/Data/Asset/BPDA_WeaponParent.GetAttackValueByName` (`self.WeaponData`) (`|GetEnumeratorNameAsString` _output_get))
    (`self.ConsumeSoul`)))

(fn `SpecialAttackStop`)