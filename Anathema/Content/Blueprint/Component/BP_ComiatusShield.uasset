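; Shield weapon component for Comiatus that provides light and heavy attacks.
; Each attack checks CanAttack, then calls SetAttackValue with itself as the hitbox mesh, an attack state and a push vector before calling the matching attack on WeaponData.
; Both attacks share the same horizontal push, and the event graph holds no active logic.
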(fn `HeavyAttack`
  (bind _canattack_ (`self.CanAttack`))
  (if _canattack_
    (`self.Set Attack Value` self "NewEnumerator2" (2000.0 2000.0 0.0))
    (`/Game/Data/Asset/BPDA_WeaponParent.HeavyAttack` (`self.WeaponData`))))

(fn `LightAttack`
  (bind _canattack_ (`self.CanAttack`))
  (if _canattack_
    (`self.Set Attack Value` self "NewEnumerator1" (2000.0 2000.0 0.0))
    (`/Game/Data/Asset/BPDA_WeaponParent.LightAttack` (`self.WeaponData`) "NewEnumerator1")))