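; BP_InvisibleCP is a checkpoint actor that saves the game when the player enters its trigger component R.
; BeginPlay caches the BP_GS_Gameplay game state and BP_FPS_NewPlayer game mode.
; Each BP_Player overlap calls SaveGame on the game state with the hardcoded "Save1" slot, then records that name as the game mode's current save.
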(event `self.ReceiveBeginPlay`
  (set `self.RefGameState` (cast `/Game/Blueprint/Player/BP_GS_Gameplay` (`GameplayStatics.GetGameState`) :!pure true))
  (set `self.RefGameMode` (cast `/Game/Blueprint/Player/BP_FPS_NewPlayer` (`GameplayStatics.GetGameMode`) :!pure true)))

(event `self.r.OnComponentBeginOverlap`
  (params (OverlappedComponent :type "PrimitiveComponent Object Reference") (OtherActor :type "Actor Object Reference") (OtherComp :type "PrimitiveComponent Object Reference") (OtherBodyIndex :type Integer) (bFromSweep :type Boolean) (SweepResult :type "HitResult Structure (by ref)"))
  (cast `/Game/Blueprint/Player/BP_Player` OtherActor)
  (`/Game/Blueprint/Player/BP_GS_Gameplay.SaveGame` (`self.RefGameState`) "Save1")
  (set `/Game/Blueprint/Player/BP_FPS_NewPlayer.CurrentSaveName` "Save1" (`self.RefGameMode`)))

(fn `UserConstructionScript`)