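; BP_DoorNextLevel is an interactable door that ends the current level and sends the player to the EndingRoom level.
; On interaction it clears the player's objectives, saves through the gameplay game state to the "Save1" slot and records that slot name on the game mode.
; It then shows a black screen widget, waits briefly, requests a non-blocking stream load of EndingRoom and immediately opens that level.
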(event `self.ReceiveBeginPlay`
  (set `self.RefGameState` (cast `/Game/Blueprint/Player/BP_GS_Gameplay` (`GameplayStatics.GetGameState`) :!pure true))
  (set `self.RefGameMode` (cast `/Game/Blueprint/Player/BP_FPS_NewPlayer` (`GameplayStatics.GetGameMode`) :!pure true)))

(event `/Game/Blueprint/Interface/BPI_Interact.Interact`
  (params (Player :type "Character Object Reference"))
  (`/Game/Blueprint/Component/Actor/BP_AC_Objectives.ClearObjectives` (`self.GetComponentByClass` Player "/Game/Blueprint/Component/Actor/BP_AC_Objectives.BP_AC_Objectives_C"))
  (`/Game/Blueprint/Player/BP_GS_Gameplay.SaveGame` (`self.RefGameState`) "Save1")
  (set `/Game/Blueprint/Player/BP_FPS_NewPlayer.CurrentSaveName` "Save1" (`self.RefGameMode`))
  (bind _returnvalue (`|CreateWidget` "/Game/Blueprint/UI/WBP_BlackScreen.WBP_BlackScreen_C"))
  (`UserWidget.AddToViewport` _returnvalue 0)
  (`KismetSystemLibrary.Delay` 0.5)
  (`GameplayStatics.LoadStreamLevelBySoftObjectPtr` "/Game/Levels/EndingRoom.EndingRoom" true)
  (`GameplayStatics.OpenLevelBySoftObjectPtr` "/Game/Levels/EndingRoom.EndingRoom"))

(fn `UserConstructionScript`
  (`parent.UserConstructionScript`))