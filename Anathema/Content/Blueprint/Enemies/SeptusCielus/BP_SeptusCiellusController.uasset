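; AI controller for the Septus Cielus enemy, running its behavior tree on possession and feeding it blackboard state.
; Perception latches CanSeePlayer once the player is sensed, and a Vegeta explosion cooldown flag starts shortly after possession.
; Tick clears the charge cooldown after a delay and, while the player is invincible, flags a mirage and targets the pawn's Dummy location if valid.
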(event `CooldownExplosionVegeta`
  (`BlackboardComponent.SetValueAsBool` (`self.Blackboard`) "CooldownVegeta" false)
  (`KismetSystemLibrary.Delay` 2.0)
  (`BlackboardComponent.SetValueAsBool` (`self.Blackboard`) "CooldownVegeta" true))

(event `self.ReceivePossess`
  (params (PossessedPawn :type "Pawn Object Reference"))
  (`self.RunBehaviorTree` "/Game/Blueprint/Enemies/SeptusCielus/BT_SeptusCielus.BT_SeptusCielus")
  (bind _asbp_septus_cielus (cast `/Game/Blueprint/Enemies/SeptusCielus/BP_SeptusCielus` (`self.K2_GetPawn`)))
  (set `self.MyPawn` _asbp_septus_cielus)
  (`self.SetActorTickEnabled` true)
  (`KismetSystemLibrary.Delay` 1.0)
  (`self.CooldownExplosionVegeta`))

(event `self.ReceiveTick`
  (params (DeltaSeconds :type "Float (single-precision)"))
  (bind _dummy (`/Game/Blueprint/Enemies/BP_AIParent.Dummy` (`self.MyPawn`)))
  (`|ExecutionSequence`
    (:`then_0`
      (if (`self.CooldownUpSmash`)
        (`KismetSystemLibrary.Delay` (`self.CooldownSpecial`))
        (`BlackboardComponent.SetValueAsBool` (`self.Blackboard`) "CooldownCharge" false)))
    (:`then_1`
      (if (`/Game/Blueprint/Component/Actor/BP_AC_LivingActor.Invincible?` (`/Game/Blueprint/Player/BP_Player.BP_AC_LivingActor` (cast `/Game/Blueprint/Player/BP_Player` (`GameplayStatics.GetPlayerPawn` 0) :!pure true)))
        (`BlackboardComponent.SetValueAsBool` (`self.Blackboard`) "MirageOn?" true)
        (`/Engine/EditorBlueprintResources/StandardMacros.IsValid` _dummy
          (:`Is Valid`
            (`BlackboardComponent.SetValueAsVector` (`self.Blackboard`) "TargetLocation" (`self.K2_GetActorLocation` _dummy))))
        (else
          (`BlackboardComponent.SetValueAsBool` (`self.Blackboard`) "MirageOn?" false))))))

(event `self.AIPerception.OnTargetPerceptionUpdated`
  (params (Actor :type "Actor Object Reference") (Stimulus :type "AIStimulus Structure"))
  (cast `/Game/Blueprint/Player/BP_Player` Actor)
  (bind _output_get (set `self.EntreDeux` (`.bSuccessfullySensed` (break `AIStimulus` Stimulus))))
  (if _output_get
    (`BlackboardComponent.SetValueAsBool` (`AIBlueprintHelperLibrary.GetBlackboard` null) "CanSeePlayer" true)))

(fn `UserConstructionScript`)