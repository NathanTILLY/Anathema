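; Hazard zone, filed under the SeptusCielus enemy, that launches a player upward and slams them back down.
; Sphere overlap with BP_Player spawns an emitter, inverts gravity scale and forces a jump, then after a delay applies extreme gravity.
; After a second delay, it spawns destruction particles at the zone, damages and stuns the player once, and destroys itself.
; Leaving the sphere resets gravity scale to normal, independently of the timed sequence.
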(event `self.Sphere.OnComponentBeginOverlap`
  (params (OverlappedComponent :type "PrimitiveComponent Object Reference") (OtherActor :type "Actor Object Reference") (OtherComp :type "PrimitiveComponent Object Reference") (OtherBodyIndex :type Integer) (bFromSweep :type Boolean) (SweepResult :type "HitResult Structure (by ref)"))
  (bind _as_bp_player (`self.As BP Player`))
  (bind _asbp_player (cast `/Game/Blueprint/Player/BP_Player` OtherActor))
  (set `self.As BP Player` _asbp_player)
  (`GameplayStatics.SpawnEmitterAtLocation` null (`self.K2_GetActorLocation`) (struct) (10.0 10.0 10.0))
  (set `CharacterMovementComponent.GravityScale` -1.5 (`Character.CharacterMovement` _asbp_player))
  (`/Game/Blueprint/Player/BP_Player.JumpPressed` _asbp_player)
  (`KismetSystemLibrary.Delay` 1.5)
  (set `CharacterMovementComponent.GravityScale` 100000.0 (`Character.CharacterMovement` (`self.As BP Player`)))
  (`KismetSystemLibrary.Delay` 0.7)
  (`/Engine/EditorBlueprintResources/StandardMacros.DoOnce` false
    (:`Completed`
      (`GameplayStatics.SpawnEmitterAtLocation` "/Game/VFX/Particles/Destruction/P_Destruction_Building_A.P_Destruction_Building_A" (`self.K2_GetActorLocation`) (struct) (5.0 5.0 5.0))
      (`/Game/Blueprint/Component/Actor/BP_AC_LivingActor.TakeDamage` (`/Game/Blueprint/Player/BP_Player.BP_AC_LivingActor` _as_bp_player) 10.0 null "NewEnumerator0")
      (`/Game/Blueprint/Player/BP_Player.Stun` _as_bp_player 1.0)
      (`self.K2_DestroyActor`))))

(event `self.Sphere.OnComponentEndOverlap`
  (params (OverlappedComponent :type "PrimitiveComponent Object Reference") (OtherActor :type "Actor Object Reference") (OtherComp :type "PrimitiveComponent Object Reference") (OtherBodyIndex :type Integer))
  (bind _asbp_player (cast `/Game/Blueprint/Player/BP_Player` OtherActor))
  (set `CharacterMovementComponent.GravityScale` 1.0 (`Character.CharacterMovement` _asbp_player)))

(fn `UserConstructionScript`)