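; Waiting Comiatus enemy Blueprint that provides Shockwave and ChargeAttack heavy attacks and builds its list of armor pieces.
; Both attacks set an Attack flag and send a heavy attack message to the current weapon after a short delay; only Shockwave clears the flag.
; ChargeAttack also holds a Blackboard cooldown key true for a timed period.
; CreateArmorList gathers valid pieces uniquely, and a knockback push is left unconnected.
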(event `self.ReceiveBeginPlay`
  (`parent.ReceiveBeginPlay`))

(event `/Game/Blueprint/Interface/BPI_Shockwave.Shockwave`
  (bind _currentweapon (`self.CurrentWeapon`))
  (set `self.Attack?` true)
  (`KismetSystemLibrary.Delay` 0.2)
  (set `self.Attack?` false)
  (`/Engine/EditorBlueprintResources/StandardMacros.IsValid` _currentweapon
    (:`Is Valid`
      (message `/Game/Blueprint/Interface/BPI_WeaponAttack.HeavyAttack` _currentweapon))))

(event `/Game/Blueprint/Interface/BPI_Charge.ChargeAttack`
  (bind _returnvalue (`AIBlueprintHelperLibrary.GetBlackboard` null))
  (bind _currentweapon (`self.CurrentWeapon`))
  (set `self.Attack?` true)
  (`KismetSystemLibrary.Delay` 0.2)
  (set `self.Attack?` true)
  (`/Engine/EditorBlueprintResources/StandardMacros.IsValid` _currentweapon
    (:`Is Valid`
      (message `/Game/Blueprint/Interface/BPI_WeaponAttack.HeavyAttack` _currentweapon)
      (`BlackboardComponent.SetValueAsBool` _returnvalue "CooldownCharge" true)
      (`KismetSystemLibrary.Delay` 8.0)
      (`BlackboardComponent.SetValueAsBool` _returnvalue "CooldownCharge" false))))

(fn `CreateArmorList`
  (for _array_element (`|MakeArray` null null null null null null null null null null null null null null null null null null null :!type "StaticMeshComponent Object Reference")
    (`/Engine/EditorBlueprintResources/StandardMacros.IsValid` _array_element
      (:`Is Valid`
        (`KismetArrayLibrary.Array_AddUnique` (`self.ArmorPiecesList`) _array_element))))
  (return))

(fn `UserConstructionScript`
  (`parent.UserConstructionScript`))