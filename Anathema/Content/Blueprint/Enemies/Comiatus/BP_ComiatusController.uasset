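; AI controller for the Comiatus enemy that runs its behavior tree and is set up to track sight of the player.
; On BeginPlay it starts BT_Comiatus and caches the controlled pawn as BP_Comiatus.
; The perception handler would write sensing of BP_Player to the CanSeePlayer blackboard key, but a constant branch condition keeps that write from running.
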(event `self.ReceiveBeginPlay`
  (`|ExecutionSequence`
    (:`then_0`
      (`self.RunBehaviorTree` "/Game/Blueprint/Enemies/Comiatus/BT_Comiatus.BT_Comiatus")
      (bind _asbp_comiatus (cast `/Game/Blueprint/Enemies/Comiatus/BP_Comiatus` (`self.K2_GetPawn`)))
      (set `self.MyPawn` _asbp_comiatus))))

(event `self.AIPerception.OnTargetPerceptionUpdated`
  (params (Actor :type "Actor Object Reference") (Stimulus :type "AIStimulus Structure"))
  (if (not true)
    (cast `/Game/Blueprint/Player/BP_Player` Actor)
    (`BlackboardComponent.SetValueAsBool` (`AIBlueprintHelperLibrary.GetBlackboard` null) "CanSeePlayer" (`.bSuccessfullySensed` (break `AIStimulus` Stimulus)))))

(fn `UserConstructionScript`)