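; AI controller for the Comiatus enemy that runs its behavior tree and manages the cooldown of its charge.
; On possess it starts BT_Comiatus and stores the controlled pawn as a BP_Comiatus.
; While CdCharge is true, Tick runs a fixed Delay, then clears the CooldownCharge blackboard key.
; Nothing in this controller sets or resets CdCharge.
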(event `self.ReceivePossess`
  (params (PossessedPawn :type "Pawn Object Reference"))
  (`self.RunBehaviorTree` "/Game/Blueprint/Enemies/ComiatusFolder/Comiatus/BT_Comiatus.BT_Comiatus")
  (bind _asbp_comiatus (cast `/Game/Blueprint/Enemies/ComiatusFolder/Comiatus/BP_Comiatus` (`self.K2_GetPawn`)))
  (set `self.MyPawn` _asbp_comiatus))

(event `self.ReceiveTick`
  (params (DeltaSeconds :type "Float (single-precision)"))
  (if (`self.CdCharge`)
    ;[1 1 1] duration of the CD of the charge
    (`KismetSystemLibrary.Delay` 10.0)
    (`BlackboardComponent.SetValueAsBool` (`AIBlueprintHelperLibrary.GetBlackboard` null) "CooldownCharge" false)))

(fn `UserConstructionScript`)