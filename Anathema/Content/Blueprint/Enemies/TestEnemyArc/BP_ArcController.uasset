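; AI controller for an arc enemy that approaches the player along a curved path.
; On possession it copies the enemy's ThetaAngle, caches the player after a short delay and enables tick.
; Each tick moves toward a point offset at that angle from the player direction, switching to a direct approach once Manhattan distance is close.
; The forward trace's result, BaseDist and the empty GetArcValue do not affect movement.
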(event `self.ReceivePossess`
  (params (PossessedPawn :type "Pawn Object Reference"))
  (bind _asbp_enemi_arc (cast `/Game/Blueprint/Enemies/TestEnemyArc/BP_EnemiArc` PossessedPawn)
    (:`then`
      (set `self.ThetaGiven` (`/Game/Blueprint/Enemies/TestEnemyArc/BP_EnemiArc.ThetaAngle` _asbp_enemi_arc)))
    (:`CastFailed`
      _))
  (set `self.MyPawn` PossessedPawn)
  (`KismetSystemLibrary.Delay` 0.2)
  (bind _asbp_player (cast `/Game/Blueprint/Player/BP_Player` (`GameplayStatics.GetPlayerPawn` 0)))
  (set `self.Player` _asbp_player)
  (`self.ResetBaseDist`)
  (`self.SetActorTickEnabled` true))

(event `self.ReceiveTick`
  (params (DeltaSeconds :type "Float (single-precision)"))
  (bind _mypawn (`self.MyPawn`))
  (bind _returnvalue (`self.K2_GetActorLocation` _mypawn))
  (`KismetSystemLibrary.LineTraceSingle` :`Start` _returnvalue :`End` (+ _returnvalue (* (`self.GetActorForwardVector` _mypawn) 300.0)) :`TraceChannel` "TraceTypeQuery1" :`DrawDebugType` "ForDuration" :`DrawTime` 0.2)
  (`self.MoveToPlayer`))

(fn `GetArcValue`)

(fn `MoveToPlayer`
  (bind (_returnvalue_x _returnvalue_y) (`KismetMathLibrary.BreakVector` (`self.K2_GetActorLocation` (`self.Player`))))
  (bind (_returnvalue_x_2 _returnvalue_y_2) (`KismetMathLibrary.BreakVector` (`self.K2_GetActorLocation` (`self.MyPawn`))))
  (bind _returnvalue (- _returnvalue_x _returnvalue_x_2))
  (bind _returnvalue_2 (- _returnvalue_y _returnvalue_y_2))
  (bind _output_get (set `self.CurrentDist` (+ (`KismetMathLibrary.Abs` _returnvalue) (`KismetMathLibrary.Abs` _returnvalue_2))))
  (if (> _output_get 500.0)
    (`self.MoveToLocation` (+ (`self.K2_GetActorLocation` (`self.MyPawn`)) (`KismetMathLibrary.Conv_Vector2DToVector` (* (`KismetMathLibrary.Normal2D` (`KismetMathLibrary.GetRotated2D` (`KismetMathLibrary.MakeVector2D` _returnvalue _returnvalue_2) (`self.ThetaGiven`))) 350.0))) 1.0 true true false true null)
    (else
      (`self.MoveToLocation` (`self.K2_GetActorLocation` (`self.Player`)) 50.0 true true false true null))))

(fn `ResetBaseDist`
  (bind (_returnvalue_x _returnvalue_y) (`KismetMathLibrary.BreakVector` (`self.K2_GetActorLocation` (`self.Player`))))
  (bind (_returnvalue_x_2 _returnvalue_y_2) (`KismetMathLibrary.BreakVector` (`self.K2_GetActorLocation` (`self.MyPawn`))))
  (set `self.BaseDist` (`KismetMathLibrary.Abs` (+ (- _returnvalue_x _returnvalue_x_2) (- _returnvalue_y _returnvalue_y_2)))))

(fn `UserConstructionScript`)