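; AI controller for the BP_Comiatus enemy that runs the BT_Comiatus behavior tree when it possesses the pawn.
; On Tick, a set CdCharge flag starts a 30-second delay that then clears the CooldownCharge blackboard key.
; Tick also mirrors the player's Invincible state into the MirageOn? key, pointing TargetLocation at the pawn's Dummy actor, when valid, during invincibility.
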(event `self.ReceivePossess`
  (params (PossessedPawn :type "Pawn Object Reference"))
  (`self.RunBehaviorTree` "/Game/Blueprint/Enemies/ComiatusFolder/Comiatus/BT_Comiatus.BT_Comiatus")
  (bind _asbp_comiatus (cast `/Game/Blueprint/Enemies/ComiatusFolder/Comiatus/BP_Comiatus` (`self.K2_GetPawn`)))
  (set `self.MyPawn` _asbp_comiatus))

(event `self.ReceiveTick`
  (params (DeltaSeconds :type "Float (single-precision)"))
  (bind _dummy (`/Game/Blueprint/Enemies/BP_AIParent.Dummy` (`self.MyPawn`)))
  (`|ExecutionSequence`
    (:`then_0`
      (if (`self.CdCharge`)
        ;[1 1 1] duration of the CD of the charge
        (`KismetSystemLibrary.Delay` 30.0)
        (`BlackboardComponent.SetValueAsBool` (`AIBlueprintHelperLibrary.GetBlackboard` null) "CooldownCharge" false)))
    (:`then_1`
      (if (`/Game/Blueprint/Component/Actor/BP_AC_LivingActor.Invincible?` (`/Game/Blueprint/Player/BP_Player.BP_AC_LivingActor` (cast `/Game/Blueprint/Player/BP_Player` (`GameplayStatics.GetPlayerPawn` 0) :!pure true)))
        (`BlackboardComponent.SetValueAsBool` (`self.Blackboard`) "MirageOn?" true)
        (`/Engine/EditorBlueprintResources/StandardMacros.IsValid` _dummy
          (:`Is Valid`
            (`BlackboardComponent.SetValueAsVector` (`self.Blackboard`) "TargetLocation" (`self.K2_GetActorLocation` _dummy))))
        (else
          (`BlackboardComponent.SetValueAsBool` (`self.Blackboard`) "MirageOn?" false))))))

(fn `UserConstructionScript`)