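; AI controller for Griveton patrol minions, running their behavior tree and setting walk speed on possession.
; It stores the patrol chief in the blackboard and on Tick updates ChiefLocation to a random navigable point near it, clearing TheChiefIsMoving after a short delay.
; Player perception updates set CanSeePlayer and, on both sensing and losing, claim one of the player's limited tickets if any remain, flagging Ticket in the blackboard.
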(event `self.ReceivePossess`
  (params (PossessedPawn :type "Pawn Object Reference"))
  (`|ExecutionSequence`
    (:`then_0`
      (`self.RunBehaviorTree` "/Game/Blueprint/Enemies/GrivetonPatrouille/BT_GrivetonMinionPatrol.BT_GrivetonMinionPatrol")
      (bind _asbp_griveton_minion_patrol (cast `/Game/Blueprint/Enemies/GrivetonPatrouille/BP_GrivetonMinionPatrol` (`self.K2_GetPawn`)))
      (set `self.MyPawns` _asbp_griveton_minion_patrol)
      (`BlackboardComponent.SetValueAsObject` (`AIBlueprintHelperLibrary.GetBlackboard` null) "ChiefPatrol" (`/Game/Blueprint/Enemies/GrivetonPatrouille/BP_GrivetonMinionPatrol.PatrolChief` (`self.MyPawns`))))
    (:`then_1`
      (set `CharacterMovementComponent.MaxWalkSpeed` (`self.Speed`) (`Character.CharacterMovement` (`self.MyPawns`))))))

(event `self.AIPerception.OnTargetPerceptionUpdated`
  (params (Actor :type "Actor Object Reference") (Stimulus :type "AIStimulus Structure"))
  (bind _asbp_player (cast `/Game/Blueprint/Player/BP_Player` Actor))
  (set `self.PlayerRef` _asbp_player)
  (`BlackboardComponent.SetValueAsBool` (`AIBlueprintHelperLibrary.GetBlackboard` null) "CanSeePlayer" (`.bSuccessfullySensed` (break `AIStimulus` Stimulus)))
  (`self.TakeTicket`))

(event `self.ReceiveTick`
  (params (DeltaSeconds :type "Float (single-precision)"))
  (`BlackboardComponent.SetValueAsVector` (`AIBlueprintHelperLibrary.GetBlackboard` null) "ChiefLocation" (`NavigationSystemV1.K2_GetRandomLocationInNavigableRadius` (`self.K2_GetActorLocation` (`/Game/Blueprint/Enemies/GrivetonPatrouille/BP_GrivetonMinionPatrol.PatrolChief` (`self.MyPawns`))) 50.0 null null))
  (`KismetSystemLibrary.Delay` 0.1)
  (set `/Game/Blueprint/Enemies/GrivetonPatrouille/BP_GrivetonMinionPatrol.TheChiefIsMoving` false (`self.MyPawns`)))

(fn `TakeTicket`
  (bind _tickets (`/Game/Blueprint/Player/BP_Player.Tickets` (`self.PlayerRef`)))
  (if (> _tickets 0)
    (set `/Game/Blueprint/Player/BP_Player.Tickets` (- _tickets 1) (`self.PlayerRef`))
    (`BlackboardComponent.SetValueAsBool` (`AIBlueprintHelperLibrary.GetBlackboard` null) "Ticket" true)))

(fn `UserConstructionScript`)