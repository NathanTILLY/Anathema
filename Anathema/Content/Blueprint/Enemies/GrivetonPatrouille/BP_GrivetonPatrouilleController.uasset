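; AI controller for the GrivetonPatrouille patrolling enemy, driving it through a behavior tree.
; On possess it runs the tree, seeds the blackboard with the pawn's patrol path looping flag and wait time plus an initial direction, and sets walk speed.
; AI perception updates write whether the player is currently sensed to the blackboard.
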(event `self.ReceivePossess`
  (params (PossessedPawn :type "Pawn Object Reference"))
  (bind _returnvalue (`AIBlueprintHelperLibrary.GetBlackboard` null))
  (`|ExecutionSequence`
    (:`then_0`
      (`self.RunBehaviorTree` "/Game/Blueprint/Enemies/GrivetonPatrouille/BT_GrivetonPatrouille.BT_GrivetonPatrouille")
      (bind _asbp_griveton_patrouille (cast `/Game/Blueprint/Enemies/GrivetonPatrouille/BP_GrivetonPatrouille` (`self.K2_GetPawn`)))
      (bind _output_get (set `self.MyPawns` _asbp_griveton_patrouille))
      (`BlackboardComponent.SetValueAsBool` (`AIBlueprintHelperLibrary.GetBlackboard` null) "PathLooping" (`/Game/Blueprint/Enemies/GrivetonPatrouille/BP_PatrolPath.IsLooping` (`/Game/Blueprint/Enemies/BP_EnemyParent.PatrolPath` _output_get)))
      (`BlackboardComponent.SetValueAsInt` _returnvalue "Direction" 1)
      (`BlackboardComponent.SetValueAsFloat` _returnvalue "WaitTime" (`/Game/Blueprint/Enemies/GrivetonPatrouille/BP_PatrolPath.WaitTime` (`/Game/Blueprint/Enemies/BP_EnemyParent.PatrolPath` (`self.MyPawns`)))))
    (:`then_1`
      (set `CharacterMovementComponent.MaxWalkSpeed` (`self.Speed`) (`Character.CharacterMovement` (`self.MyPawns`))))))

(event `self.AIPerception.OnTargetPerceptionUpdated`
  (params (Actor :type "Actor Object Reference") (Stimulus :type "AIStimulus Structure"))
  (cast `/Game/Blueprint/Player/BP_Player` Actor)
  (`BlackboardComponent.SetValueAsBool` (`AIBlueprintHelperLibrary.GetBlackboard` null) "CanSeePlayer" (`.bSuccessfullySensed` (break `AIStimulus` Stimulus))))

(fn `UserConstructionScript`)