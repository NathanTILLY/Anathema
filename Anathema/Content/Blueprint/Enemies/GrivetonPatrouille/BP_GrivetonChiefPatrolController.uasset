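; AI controller for the Griveton Chief patrol enemy that runs its behavior tree and reacts to sighting the player.
; On possess it seeds the blackboard from the pawn's patrol path (looping, wait time) plus a starting direction, then sets walk speed.
; Perception updates on the player write CanSeePlayer and call TakeTicket, which consumes one of the player's limited tickets, if any remain, and flags it on the blackboard.
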(event `self.ReceivePossess`
  (params (PossessedPawn :type "Pawn Object Reference"))
  (bind _returnvalue (`AIBlueprintHelperLibrary.GetBlackboard` null))
  (`|ExecutionSequence`
    (:`then_0`
      (`self.RunBehaviorTree` "/Game/Blueprint/Enemies/GrivetonPatrouille/BT_GrivetonChiefPatrol.BT_GrivetonChiefPatrol")
      (bind _asbp_griveton_chief_patrol (cast `/Game/Blueprint/Enemies/GrivetonPatrouille/BP_GrivetonChiefPatrol` (`self.K2_GetPawn`)))
      (bind _output_get (set `self.MyPawns` _asbp_griveton_chief_patrol))
      (`BlackboardComponent.SetValueAsBool` (`AIBlueprintHelperLibrary.GetBlackboard` null) "PathLooping" (`/Game/Blueprint/Enemies/GrivetonPatrouille/BP_PatrolPath.IsLooping` (`/Game/Blueprint/Enemies/GrivetonPatrouille/BP_GrivetonChiefPatrol.PatrolPathGriveton` _output_get)))
      (`BlackboardComponent.SetValueAsInt` _returnvalue "Direction" 1)
      (`BlackboardComponent.SetValueAsFloat` _returnvalue "WaitTime" (`/Game/Blueprint/Enemies/GrivetonPatrouille/BP_PatrolPath.WaitTime` (`/Game/Blueprint/Enemies/GrivetonPatrouille/BP_GrivetonChiefPatrol.PatrolPathGriveton` (`self.MyPawns`)))))
    (:`then_1`
      (set `CharacterMovementComponent.MaxWalkSpeed` (`self.Speed`) (`Character.CharacterMovement` (`self.MyPawns`))))))

(event `self.AIPerception.OnTargetPerceptionUpdated`
  (params (Actor :type "Actor Object Reference") (Stimulus :type "AIStimulus Structure"))
  (bind _asbp_player (cast `/Game/Blueprint/Player/BP_Player` Actor))
  (set `self.PlayerRef` _asbp_player)
  (`BlackboardComponent.SetValueAsBool` (`AIBlueprintHelperLibrary.GetBlackboard` null) "CanSeePlayer" (`.bSuccessfullySensed` (break `AIStimulus` Stimulus)))
  (`self.TakeTicket`))

(fn `TakeTicket`
  (bind _tickets (`/Game/Blueprint/Player/BP_Player.Tickets` (`self.PlayerRef`)))
  (if (> _tickets 0)
    (set `/Game/Blueprint/Player/BP_Player.Tickets` (- _tickets 1) (`self.PlayerRef`))
    (`BlackboardComponent.SetValueAsBool` (`AIBlueprintHelperLibrary.GetBlackboard` null) "Ticket" true)))

(fn `UserConstructionScript`)