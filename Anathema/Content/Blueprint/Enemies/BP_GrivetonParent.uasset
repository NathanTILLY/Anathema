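; Parent Blueprint for Griveton enemies, modular armored foes with a shield weapon driving delayed light and heavy attacks.
; Player hits above a threshold pulse a blackboard stun and montage; other damage bursts the armor, which timeline-interpolates back and reattaches to saved sockets.
; Death awards souls to the killer, explodes the armor and fades it through dynamic materials before destruction.
; Capsule hits push other living actors while the Launched flag is set.
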(event `self.ReceiveBeginPlay`
  (bind _output_get (set `self.CurrentWeapon` (`self.GrivetonShield`)))
  (bind _output_get_2 (set `/Game/Blueprint/Component/Actor/BP_AC_LivingActor.OwnerWeapon` _output_get (`self.BP_AC_LivingActor`)))
  (`/Game/Blueprint/Component/BP_WeaponComponent.Implement` _output_get_2 (`self.Mesh`))
  (`self.CreateArmorList`)
  (for _array_element (`self.ArmorPiecesList`)
    (for (_array_element_2 _array_index) (`MeshComponent.GetMaterials` _array_element)
      (bind _returnvalue (`KismetMaterialLibrary.CreateDynamicMaterialInstance` _array_element_2))
      (`KismetArrayLibrary.Array_AddUnique` (`self.MaterialsList`) _returnvalue)
      (`PrimitiveComponent.SetMaterial` _array_element _array_index _returnvalue)))
  (`KismetSystemLibrary.Delay` 0.2)
  (bind _asbp_player (cast `/Game/Blueprint/Player/BP_Player` (`GameplayStatics.GetPlayerPawn` 0)))
  (set `self.As BP Player` _asbp_player))

(event `self.BP_AC_LivingActor.OnTakingDamage`
  (params (AttackOwner :type "Actor Object Reference") (DamageTaken :type "Float (single-precision)") (AttackType :type "/Game/Blueprint/Enum/E_AttackType Enum" :default "NewEnumerator0"))
  (if (== (`GameplayStatics.GetObjectClass` AttackOwner) "/Game/Blueprint/Player/BP_Player.BP_Player_C")
    (`|ExecutionSequence`
      (:`then_0`
        (bind _output_get (set `self.IsStun?` (>= DamageTaken 1.5)))
        (if _output_get
          (`BlackboardComponent.SetValueAsBool` (`AIBlueprintHelperLibrary.GetBlackboard` null) "IsStun?" (`self.IsStun?`))
          (`AnimInstance.Montage_Play` (`SkeletalMeshComponent.GetAnimInstance` (`self.Mesh`)) "/Game/Animations/Enemies/AM_Test.AM_Test" 1.0 "MontageLength" 0.0 true)
          (bind _output_get_2 (set `self.IsStun?` false))
          (`BlackboardComponent.SetValueAsBool` (`AIBlueprintHelperLibrary.GetBlackboard` null) "IsStun?" _output_get_2)))
      (:`then_1`
        (bind _output_get_3 (set `self.ExplosionVector` (`KismetMathLibrary.Normal` (- (`self.K2_GetActorLocation` AttackOwner) (`self.K2_GetActorLocation`)))))
        (set `self.ExplosionVector` (`KismetMathLibrary.MakeVector` (.x _output_get_3) (.y _output_get_3) 0.5)))
      (:`then_2`
        (`GameplayStatics.PlaySoundAtLocation` "/Game/Sound/SC_Coup.SC_Coup" (0.0 0.0 0.0) (struct) 1.0 1.0 0.0 null null null)))
    (else
      (`self.ArmorBreak`))))

(event `self.BP_AC_LivingActor.OnDeath`
  (params (AttackOwner :type "Actor Object Reference"))
  (bind _returnvalue (`self.GetComponentByClass` AttackOwner "/Game/Blueprint/Component/Actor/BP_AC_SoulHandler.BP_AC_SoulHandler_C"))
  (bind _capsulecomponent (`self.CapsuleComponent`))
  (bind _currentweapon (`self.CurrentWeapon`))
  (`|ExecutionSequence`
    (:`then_0`
      (`/Engine/EditorBlueprintResources/StandardMacros.IsValid` _returnvalue
        (:`Is Valid`
          (`/Game/Blueprint/Component/Actor/BP_AC_SoulHandler.GainSoul` _returnvalue (`self.SoulValue`)))
        (:`Is Not Valid`
          _))
      (`/Engine/EditorBlueprintResources/StandardMacros.IsValid` _capsulecomponent
        (:`Is Valid`
          (`PrimitiveComponent.SetCollisionEnabled` _capsulecomponent "NoCollision"))
        (:`Is Not Valid`
          _))
      (`/Engine/EditorBlueprintResources/StandardMacros.IsValid` _currentweapon
        (:`Is Valid`
          (`ActorComponent.K2_DestroyComponent` _currentweapon))
        (:`Is Not Valid`
          _))
      (`SceneComponent.SetHiddenInGame` (`self.Mesh`) true false)
      (`self.ArmorExplode`)
      (`KismetSystemLibrary.Delay` 3.0)
      (bind (_direction _value) (`Timeline|Fade_0`)
        (:`Update`
          (for _array_element (`self.MaterialsList`)
            (`MaterialInstanceDynamic.SetScalarParameterValue` _array_element "Fade" _value)))
        (:`Finished`
          (`self.K2_DestroyActor`))))
    (:`then_1`
      (`GameplayStatics.PlaySoundAtLocation` "/Game/Sound/SC_MortGriv.SC_MortGriv" (0.0 0.0 0.0) (struct) 1.0 1.0 0.0 null null null))))

(event `self.MeleeAttack`
  (bind _currentweapon (`self.CurrentWeapon`))
  (set `self.Attack?` true)
  (`KismetSystemLibrary.Delay` 0.2)
  (set `self.Attack?` false)
  (`/Engine/EditorBlueprintResources/StandardMacros.IsValid` _currentweapon
    (:`Is Valid`
      (`/Game/Blueprint/Component/BP_WeaponComponent.LightAttack` _currentweapon))))

(event `self.ChargeAttack`
  (bind _currentweapon (`self.CurrentWeapon`))
  (set `self.Attack?` true)
  (`KismetSystemLibrary.Delay` 0.2)
  (set `self.Attack?` false)
  (`/Engine/EditorBlueprintResources/StandardMacros.IsValid` _currentweapon
    (:`Is Valid`
      (`/Game/Blueprint/Component/BP_WeaponComponent.HeavyAttack` _currentweapon))))

(event `self.OnLaunched`
  (params (LaunchVelocity :type "Vector Structure") (bXYOverride :type Boolean) (bZOverride :type Boolean))
  ;[1 1 1] Stop Movement to avoid bug when launched
  (set `self.Launched?` false)
  (`Controller.StopMovement` (`self.GetController`)))

(event `self.OnLanded`
  (params (Hit :type "HitResult Structure (by ref)"))
  ;[1 1 1] Launched is false after landing
  (set `self.Launched?` false))

(event `self.CapsuleComponent.OnComponentHit`
  (params (HitComponent :type "PrimitiveComponent Object Reference") (OtherActor :type "Actor Object Reference") (OtherComp :type "PrimitiveComponent Object Reference") (NormalImpulse :type "Vector Structure") (Hit :type "HitResult Structure (by ref)"))
  (bind _returnvalue (`self.GetComponentByClass` OtherActor "/Game/Blueprint/Component/Actor/BP_AC_LivingActor.BP_AC_LivingActor_C"))
  (bind (_returnvalue_x _returnvalue_y) (`KismetMathLibrary.BreakVector` (* (`KismetMathLibrary.Normal` (- (`self.K2_GetActorLocation` OtherActor) (`self.K2_GetActorLocation`))) (500.0 500.0 0.0))))
  ;[1 1 1] Push other enemies while launched
  (`/Engine/EditorBlueprintResources/StandardMacros.IsValid` OtherActor
    (:`Is Valid`
      (if (and (`self.Launched?`) (`KismetSystemLibrary.IsValid` _returnvalue))
        (`/Game/Blueprint/Component/Actor/BP_AC_LivingActor.Pushed` _returnvalue (`KismetMathLibrary.MakeVector` _returnvalue_x _returnvalue_y 100.0))))))

(event `ArmorBreak`
  (bind _currentweapon (`self.CurrentWeapon`))
  (bind _capsulecomponent (`self.CapsuleComponent`))
  (bind _currentweapon_2 (`self.CurrentWeapon`))
  (bind _capsulecomponent_2 (`self.CapsuleComponent`))
  (set `self.IsStun?` true)
  (for (_array_element _array_index) (`self.ArmorPiecesList`)
    (`KismetArrayLibrary.Array_Insert` (`self.ArmorPiecesOriginalTransform`) (`SceneComponent.K2_GetComponentToWorld` _array_element) _array_index))
  (`/Engine/EditorBlueprintResources/StandardMacros.IsValid` _capsulecomponent
    (:`Is Valid`
      (`PrimitiveComponent.SetCollisionEnabled` _capsulecomponent "PhysicsOnly")
      (`/Engine/EditorBlueprintResources/StandardMacros.IsValid` _currentweapon_2
        (:`Is Valid`
          (`SceneComponent.SetHiddenInGame` _currentweapon_2 true false)
          (`SceneComponent.SetHiddenInGame` (`self.Mesh`) true false)
          (`self.ArmorExplode`)
          (`KismetSystemLibrary.Delay` 2.0)
          (for _array_element_2 (`self.ArmorPiecesList`)
            (`PrimitiveComponent.SetCollisionProfileName` _array_element_2 "WorldDynamic" true)
            (`PrimitiveComponent.SetSimulatePhysics` _array_element_2 false))
          ;[1 1 1] Armor pieces going back to their original places
          (bind (_direction _travelvalue) (`Timeline|PiecesComingBack_0`)
            (:`Update`
              (for (_array_element_3 _array_index_2) (`self.ArmorPiecesList`)
                (bind (_output_location _output_rotation) (`KismetMathLibrary.BreakTransform` (`|GetArrayItem` (`self.ArmorPiecesOriginalTransform`) _array_index_2)))
                (`SceneComponent.K2_SetWorldLocation` _array_element_3 (`KismetMathLibrary.VInterpTo` (`SceneComponent.K2_GetComponentLocation` _array_element_3) _output_location _travelvalue 0.1) false false)
                (`SceneComponent.K2_SetWorldRotation` _array_element_3 (`KismetMathLibrary.RInterpTo` (`SceneComponent.K2_GetComponentRotation` _array_element_3) _output_rotation _travelvalue 0.1) false false)))
            (:`Finished`
              (`/Engine/EditorBlueprintResources/StandardMacros.IsValid` _capsulecomponent_2
                (:`Is Valid`
                  (`PrimitiveComponent.SetCollisionEnabled` _capsulecomponent_2 "QueryAndPhysics")
                  (`/Engine/EditorBlueprintResources/StandardMacros.IsValid` _currentweapon
                    (:`Is Valid`
                      (`SceneComponent.SetHiddenInGame` _currentweapon false false)
                      (`SceneComponent.SetHiddenInGame` (`self.Mesh`) false false)
                      (`self.SetActorTickEnabled` (`self.GetController`) true)
                      (set `self.IsStun?` false)
                      (for (_array_element_4 _array_index_3) (`self.ArmorPiecesList`)
                        (`SceneComponent.K2_AttachToComponent` _array_element_4 (`self.Mesh`) (`|GetArrayItem` (`self.BoneArmorAttachedToList`) _array_index_3) "SnapToTarget" "SnapToTarget" "SnapToTarget" true)))))))))))))

(fn `CreateArmorList`
  (bind _grivetonshield (`self.GrivetonShield`))
  (for _array_element (`|MakeArray` (`self.LegHL`) (`self.ForearmL`) (`self.Chestplate`) (`self.Tunic`) (`self.ShoulderPlateR`) (`self.ForearmR`) (`self.ShoulderPlateL`) (`self.LegHR`) (`self.LegLR`) (`self.KneeR`) (`self.FootR`) (`self.FootL`) (`self.LegLL`) (`self.KneeL`) (`self.Head`) (`self.Hair_Side`) _grivetonshield (`/Game/Blueprint/Component/BP_WeaponComponent.ShieldRef` _grivetonshield) :!type "StaticMeshComponent Object Reference")
    (`/Engine/EditorBlueprintResources/StandardMacros.IsValid` _array_element
      (:`Is Valid`
        (`KismetArrayLibrary.Array_AddUnique` (`self.ArmorPiecesList`) _array_element)
        (`KismetArrayLibrary.Array_Add` (`self.BoneArmorAttachedToList`) (`SceneComponent.GetAttachSocketName` _array_element)))))
  (return))

(fn `HeavyAttack`
  (returns (`CanAttack?` :type Boolean))
  (return false))

(fn `LightAttack`
  (returns (`CanAttack?` :type Boolean))
  (return false))

(fn `OnSpecialAttack`
  (returns (`CanAttack?` :type Boolean))
  (return false))

(fn `OnSpecialAttackReleased`
  (returns (`CanAttack?` :type Boolean))
  (return false))

(fn `OwnerTakeHit`
  (params (Attacker :type "Actor Object Reference") (Damage :type "Float (double-precision)"))
  (returns (`TakingDamage?` :type Boolean) (NewDamage :type "Float (double-precision)"))
  (return false 0.0))

(fn `UserConstructionScript`)