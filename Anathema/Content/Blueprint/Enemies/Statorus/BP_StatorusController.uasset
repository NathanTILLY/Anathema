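; AI controller for the Statorus enemy that runs the BT_Statorus behavior tree on possession and caches the controlled pawn as BP_Statorus.
; An AI Perception handler is built to copy whether a sensed BP_Player is successfully detected into the CanSeePlayer blackboard key.
; That update sits behind a constant branch condition that never passes, so perception does not currently write to the blackboard.
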(event `self.ReceivePossess`
  (params (PossessedPawn :type "Pawn Object Reference"))
  (`self.RunBehaviorTree` "/Game/Blueprint/Enemies/Statorus/BT_Statorus.BT_Statorus")
  (bind _asbp_statorus (cast `/Game/Blueprint/Enemies/Statorus/BP_Statorus` (`self.K2_GetPawn`)))
  (set `self.MyPawn` _asbp_statorus))

(event `self.AIPerception.OnTargetPerceptionUpdated`
  (params (Actor :type "Actor Object Reference") (Stimulus :type "AIStimulus Structure"))
  (if (not true)
    (cast `/Game/Blueprint/Player/BP_Player` Actor)
    (`BlackboardComponent.SetValueAsBool` (`AIBlueprintHelperLibrary.GetBlackboard` null) "CanSeePlayer" (`.bSuccessfullySensed` (break `AIStimulus` Stimulus)))))

(fn `UserConstructionScript`)