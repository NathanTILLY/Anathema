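; BP_Statorus is an enemy with a one-time berserk phase at half health or below.
; Capsule hit events compare current HP to max HP from BPACLivingActor and check the IsBerserkUsed flag, which must be true to trigger despite its name.
; After a short delay, it doubles the current weapon's light and heavy attack damage, then clears the flag.
; The step labeled Animation contains only that delay.
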(event `self.ReceiveBeginPlay`
  (`parent.ReceiveBeginPlay`))

(event `self.CapsuleComponent.OnComponentHit`
  (params (HitComponent :type "PrimitiveComponent Object Reference") (OtherActor :type "Actor Object Reference") (OtherComp :type "PrimitiveComponent Object Reference") (NormalImpulse :type "Vector Structure") (Hit :type "HitResult Structure (by ref)"))
  (bind _bp_ac_livingactor (`self.BP_AC_LivingActor`))
  (bind _currentweapon (`self.CurrentWeapon`))
  (if (<= (`/Game/Blueprint/Component/Actor/BP_AC_LivingActor.CurrentHp` _bp_ac_livingactor) (/ (`/Game/Blueprint/Component/Actor/BP_AC_LivingActor.MaxHp` _bp_ac_livingactor) 2.0))
    (if (`self.IsBerserkUsed?`)
      ;[1 1 1] Animation
      (`KismetSystemLibrary.Delay` 1.0)
      ;[0.3281 0.2731 1] Berserk
      (set `/Game/Blueprint/Weapons/BP_WeaponParent.LightAttackDamage` (* (`/Game/Blueprint/Weapons/BP_WeaponParent.LightAttackDamage` _currentweapon) 2.0) _currentweapon)
      (set `/Game/Blueprint/Weapons/BP_WeaponParent.HeavyAttackDamage` (* (`/Game/Blueprint/Weapons/BP_WeaponParent.HeavyAttackDamage` _currentweapon) 2.0) _currentweapon)
      (set `self.IsBerserkUsed?` false))))

(fn `UserConstructionScript`
  (`parent.UserConstructionScript`))