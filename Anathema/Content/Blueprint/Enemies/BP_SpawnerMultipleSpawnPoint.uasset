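; Enemy spawner actor that spawns a set number of AI pawns across several spawn points once the player enters its box.
; The box overlap starts a delayed loop that spawns MobASpawn every TempsDeSpawn seconds until the counter, debug-printed each time, reaches NbrDeSpawn.
; Location and rotation come from separate random picks in SpawnLocation, so they can belong to different points.
; The counter never resets.
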(event `self.Box.OnComponentBeginOverlap`
  (params (OverlappedComponent :type "PrimitiveComponent Object Reference") (OtherActor :type "Actor Object Reference") (OtherComp :type "PrimitiveComponent Object Reference") (OtherBodyIndex :type Integer) (bFromSweep :type Boolean) (SweepResult :type "HitResult Structure (by ref)"))
  (bind _spawnlocation (`self.SpawnLocation`))
  (bind _nbrdejaspawn (`self.NbrDejaSpawn`))
  (bind _rootcomponent (`Actor.RootComponent` (`|GetArrayItem` _spawnlocation (`KismetMathLibrary.RandomInteger` (`KismetArrayLibrary.Array_Length` _spawnlocation)))))
  (cast `/Game/Blueprint/Player/BP_Player` OtherActor)
  (if (< (`self.NbrDejaSpawn`) (`self.NbrDeSpawn`)) :!label _label
    (`/Engine/EditorBlueprintResources/StandardMacros.IncrementFloat` _nbrdejaspawn
      (:`  `
        (`KismetSystemLibrary.PrintString` (`KismetStringLibrary.Conv_DoubleToString` _nbrdejaspawn) true true (struct :`R` 1.0 :`G` 0.053367 :`A` 1.0))
        (`AIBlueprintHelperLibrary.SpawnAIFromClass` (`self.MobASpawn`) null (`SceneComponent.K2_GetComponentLocation` _rootcomponent) (`SceneComponent.K2_GetComponentRotation` _rootcomponent) false null)
        (`KismetSystemLibrary.Delay` (`self.tempsDeSpawn`))
        (goto _label)))))

(fn `UserConstructionScript`)