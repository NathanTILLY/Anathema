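; AI controller for the GrivetonQuiAttend enemy that runs the BT_GrivetonAttend behavior tree and sets the pawn's walk speed on possession.
; Perception updates on the player write CanSeePlayer to the Blackboard.
; On sighting, it tries to take one of the tickets stored on the player, decrementing that count and setting the Ticket key.
; This controller never returns tickets or clears that key.
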(event `self.ReceivePossess`
  (params (PossessedPawn :type "Pawn Object Reference"))
  (`|ExecutionSequence`
    (:`then_0`
      (`self.RunBehaviorTree` "/Game/Blueprint/Enemies/GrivetonQuiAttend/BT_GrivetonAttend.BT_GrivetonAttend")
      (bind _ascharacter (cast `Character` (`self.K2_GetPawn`)))
      (set `self.PawnTest` _ascharacter))
    (:`then_1`
      (set `CharacterMovementComponent.MaxWalkSpeed` (`self.Speed`) (`Character.CharacterMovement` (`self.PawnTest`))))))

(event `self.AIPerception.OnTargetPerceptionUpdated`
  (params (Actor :type "Actor Object Reference") (Stimulus :type "AIStimulus Structure"))
  (bind _asbp_player (cast `/Game/Blueprint/Player/BP_Player` Actor))
  (set `self.PlayerRef` _asbp_player)
  (bind _output_get (set `self.EntreDeux` (`.bSuccessfullySensed` (break `AIStimulus` Stimulus))))
  (if _output_get
    (`BlackboardComponent.SetValueAsBool` (`AIBlueprintHelperLibrary.GetBlackboard` null) "CanSeePlayer" true)
    (`self.TakeTicket`)
    (else
      (`BlackboardComponent.SetValueAsBool` (`AIBlueprintHelperLibrary.GetBlackboard` null) "CanSeePlayer" false))))

(fn `TakeTicket`
  (bind _tickets (`/Game/Blueprint/Player/BP_Player.Tickets` (`self.PlayerRef`)))
  (if (> _tickets 0)
    (set `/Game/Blueprint/Player/BP_Player.Tickets` (- _tickets 1) (`self.PlayerRef`))
    (`BlackboardComponent.SetValueAsBool` (`AIBlueprintHelperLibrary.GetBlackboard` null) "Ticket" true)))

(fn `UserConstructionScript`)