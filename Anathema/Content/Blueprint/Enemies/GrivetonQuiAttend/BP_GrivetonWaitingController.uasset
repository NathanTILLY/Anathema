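; AI controller for the waiting Griveton enemy, running its behavior tree and flagging when it spots the player.
; On possess it stores a random arc angle in the blackboard and caches the pawn and player references.
; Perception latches CanSeePlayer to true on a successful sense.
; Arc writes TargetLocation as a fixed-distance offset from the pawn toward the player, rotated by that angle for an angled approach.
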(event `self.ReceivePossess`
  (params (PossessedPawn :type "Pawn Object Reference"))
  (`self.RunBehaviorTree` "/Game/Blueprint/Enemies/GrivetonQuiAttend/BT_GrivetonWaiting.BT_GrivetonWaiting")
  (bind _output_get (set `self.AngleArc` (`KismetMathLibrary.RandomFloatInRange` -45.0 45.0)))
  (`BlackboardComponent.SetValueAsFloat` (`AIBlueprintHelperLibrary.GetBlackboard` null) "Angle" _output_get)
  (bind _asbp_griveton_waiting (cast `/Game/Blueprint/Enemies/GrivetonQuiAttend/BP_Griveton_Waiting` (`self.K2_GetPawn`)))
  (set `self.PawnRef` _asbp_griveton_waiting)
  (`KismetSystemLibrary.Delay` 0.2)
  (bind _asbp_player (cast `/Game/Blueprint/Player/BP_Player` (`GameplayStatics.GetPlayerPawn` 0)))
  (set `self.PlayerRef` _asbp_player)
  (`self.SetActorTickEnabled` true))

(event `self.AIPerception.OnTargetPerceptionUpdated`
  (params (Actor :type "Actor Object Reference") (Stimulus :type "AIStimulus Structure"))
  (cast `/Game/Blueprint/Player/BP_Player` Actor)
  (bind _output_get (set `self.EntreDeux` (`.bSuccessfullySensed` (break `AIStimulus` Stimulus))))
  (if _output_get
    (`BlackboardComponent.SetValueAsBool` (`AIBlueprintHelperLibrary.GetBlackboard` null) "CanSeePlayer" true)))

(fn `Arc`
  (bind (_returnvalue_x _returnvalue_y) (`KismetMathLibrary.BreakVector` (`self.K2_GetActorLocation` (`self.PlayerRef`))))
  (bind (_returnvalue_x_2 _returnvalue_y_2) (`KismetMathLibrary.BreakVector` (`self.K2_GetActorLocation` (`self.PawnRef`))))
  (`BlackboardComponent.SetValueAsVector` (`AIBlueprintHelperLibrary.GetBlackboard` null) "TargetLocation" (+ (`self.K2_GetActorLocation` (`self.PawnRef`)) (`KismetMathLibrary.Conv_Vector2DToVector` (* (`KismetMathLibrary.Normal2D` (`KismetMathLibrary.GetRotated2D` (`KismetMathLibrary.MakeVector2D` (- _returnvalue_x _returnvalue_x_2) (- _returnvalue_y _returnvalue_y_2)) (`self.AngleArc`))) 350.0)))))

(fn `UserConstructionScript`)