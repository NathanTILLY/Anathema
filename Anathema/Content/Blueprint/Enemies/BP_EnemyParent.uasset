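; Base enemy Blueprint that spawns and wields a socketed weapon, exposing melee, charge and hitbox events.
; BP_AC_LivingActor events drive reactions: heavy hits pulse a blackboard stun flag, play a montage and store a knockback direction.
; Death grants souls to the killer, destroys the weapon and blasts modular body parts apart with physics, fading their shared dynamic material.
; While launched, AI movement stops and collisions push other living actors.
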(event `self.ReceiveBeginPlay`
  (bind _returnvalue (`|SpawnActorFromClass` (`self.WeaponClass`) (`self.GetTransform`) "Undefined" "OverrideRootScale" self null))
  (bind _output_get (set `self.CurrentWeapon` _returnvalue))
  (`self.K2_AttachToComponent` _output_get (`self.Mesh`) "WeaponSocket" "SnapToTarget" "SnapToTarget" "SnapToTarget" true)
  (`/Game/Blueprint/Interface/BPI_WeaponAttack.PickUp` (`self.CurrentWeapon`) self null)
  (bind _returnvalue_2 (`KismetMaterialLibrary.CreateDynamicMaterialInstance` (`PrimitiveComponent.GetMaterial` (`self.Head`) 0)))
  (bind _output_get_2 (set `self.Material` _returnvalue_2))
  (`PrimitiveComponent.SetMaterial` (`self.Head`) 0 _output_get_2)
  (`PrimitiveComponent.SetMaterial` (`self.Visor`) 0 _output_get_2)
  (`PrimitiveComponent.SetMaterial` (`self.KneeL`) 0 _output_get_2)
  (`PrimitiveComponent.SetMaterial` (`self.LegLL`) 0 _output_get_2)
  (`PrimitiveComponent.SetMaterial` (`self.FootL`) 0 _output_get_2)
  (`PrimitiveComponent.SetMaterial` (`self.FootR`) 0 _output_get_2)
  (`PrimitiveComponent.SetMaterial` (`self.KneeR`) 0 _output_get_2)
  (`PrimitiveComponent.SetMaterial` (`self.LegLR`) 0 _output_get_2)
  (`PrimitiveComponent.SetMaterial` (`self.LegHR`) 0 _output_get_2)
  (`PrimitiveComponent.SetMaterial` (`self.ShoulderPlateL`) 0 _output_get_2)
  (`PrimitiveComponent.SetMaterial` (`self.ForearmPlateR`) 0 _output_get_2)
  (`PrimitiveComponent.SetMaterial` (`self.ShoulderPlateR`) 0 _output_get_2)
  (`PrimitiveComponent.SetMaterial` (`self.Tunic`) 0 _output_get_2)
  (`PrimitiveComponent.SetMaterial` (`self.ForearmPlateL`) 0 _output_get_2)
  (`PrimitiveComponent.SetMaterial` (`self.ForearmR`) 0 _output_get_2)
  (`PrimitiveComponent.SetMaterial` (`self.Chestplate`) 0 _output_get_2)
  (`PrimitiveComponent.SetMaterial` (`self.ForearmL`) 0 _output_get_2)
  (`PrimitiveComponent.SetMaterial` (`self.LegHL`) 0 _output_get_2))

(event `self.BP_AC_LivingActor.OnTakingDamage`
  (params (AttackOwner :type "Actor Object Reference") (DamageTaken :type "Float (single-precision)"))
  (bind _output_get (set `self.IsStun?` (>= DamageTaken 1.5)))
  (if _output_get
    (`BlackboardComponent.SetValueAsBool` (`AIBlueprintHelperLibrary.GetBlackboard` null) "IsStun?" (`self.IsStun?`))
    (`AnimInstance.Montage_Play` (`SkeletalMeshComponent.GetAnimInstance` (`self.Mesh`)) "/Game/Animations/Enemies/AM_Test.AM_Test" 1.0 "MontageLength" 0.0 true)
    (bind _output_get_2 (set `self.IsStun?` false))
    (`BlackboardComponent.SetValueAsBool` (`AIBlueprintHelperLibrary.GetBlackboard` null) "IsStun?" _output_get_2)
    (bind _output_get_3 (set `self.ExplosionVector` (`KismetMathLibrary.Normal` (- (`self.K2_GetActorLocation` AttackOwner) (`self.K2_GetActorLocation`)))))
    (set `self.ExplosionVector` (`KismetMathLibrary.MakeVector` (.x _output_get_3) (.y _output_get_3) 0.5))))

(event `self.BP_AC_LivingActor.OnDeath`
  (params (AttackOwner :type "Actor Object Reference"))
  (bind _returnvalue (`self.GetComponentByClass` AttackOwner "/Game/Blueprint/Component/Actor/BP_AC_SoulHandler.BP_AC_SoulHandler_C"))
  (bind _currentweapon (`self.CurrentWeapon`))
  (bind _capsulecomponent (`self.CapsuleComponent`))
  (bind _chestplate (`self.Chestplate`))
  (bind _returnvalue_2 (* (`self.ExplosionVector`) -500000.0))
  (`/Engine/EditorBlueprintResources/StandardMacros.IsValid` _returnvalue
    (:`Is Valid`
      (`/Game/Blueprint/Component/Actor/BP_AC_SoulHandler.GainSoul` _returnvalue (`self.SoulValue`)))
    (:`Is Not Valid`
      _))
  (`/Engine/EditorBlueprintResources/StandardMacros.IsValid` _capsulecomponent
    (:`Is Valid`
      (`PrimitiveComponent.SetCollisionEnabled` _capsulecomponent "NoCollision")
      (`/Engine/EditorBlueprintResources/StandardMacros.IsValid` _currentweapon
        (:`Is Valid`
          (`self.K2_DestroyActor` _currentweapon)
          (`SceneComponent.SetHiddenInGame` (`self.Mesh`) true false)
          (`|ExecutionSequence`
            (:`then_0`
              (`PrimitiveComponent.SetCollisionProfileName` _chestplate "IgnorePawn" true)
              (`PrimitiveComponent.SetSimulatePhysics` _chestplate true)
              (`PrimitiveComponent.AddForce` _chestplate _returnvalue_2 "None" false)
              (`KismetSystemLibrary.Delay` 6.0 :!label _label)
              (bind (_direction _value) (`Timeline|Fade`)
                (:`Update`
                  (`MaterialInstanceDynamic.SetScalarParameterValue` (`self.Material`) "Fade" _value)
                  (`KismetSystemLibrary.Delay` 10.0)
                  (`self.K2_DestroyActor`))))
            (:`then_1`
              (for _array_element (`|MakeArray` null (`self.FootL`) (`self.FootR`) (`self.ForearmL`) (`self.ForearmPlateL`) (`self.ForearmPlateR`) (`self.ForearmR`) null null (`self.Head`) (`self.KneeL`) (`self.KneeR`) (`self.LegHL`) (`self.LegHR`) (`self.LegLL`) (`self.LegLR`) (`self.ShoulderPlateL`) (`self.ShoulderPlateR`) (`self.Tunic`) (`self.Visor`))
                (`/Engine/EditorBlueprintResources/StandardMacros.IsValid` _array_element
                  (:`Is Valid`
                    (`PrimitiveComponent.SetCollisionProfileName` _array_element "IgnorePawn" true)
                    (`PrimitiveComponent.SetSimulatePhysics` _array_element true)
                    (`PrimitiveComponent.AddForce` _array_element _returnvalue_2 "None" false)
                    (goto _label)))))))))))

(event `/Game/Blueprint/Interface/BPI_UsingWeapon.ActiveWeapon`
  (bind _currentweapon (`self.CurrentWeapon`))
  (`/Engine/EditorBlueprintResources/StandardMacros.IsValid` _currentweapon
    (:`Is Valid`
      (`/Game/Blueprint/Weapons/BP_WeaponParent.SetHitboxState` _currentweapon true))))

(event `/Game/Blueprint/Interface/BPI_UsingWeapon.InactiveWeapon`
  (bind _currentweapon (`self.CurrentWeapon`))
  (`/Engine/EditorBlueprintResources/StandardMacros.IsValid` _currentweapon
    (:`Is Valid`
      (`/Game/Blueprint/Weapons/BP_WeaponParent.SetHitboxState` _currentweapon false)
      (set `/Game/Blueprint/Weapons/BP_WeaponParent.CurrentDamage` (`/Game/Blueprint/Weapons/BP_WeaponParent.LightAttackDamage` _currentweapon) _currentweapon))))

(event `self.MeleeAttack`
  (bind _currentweapon (`self.CurrentWeapon`))
  (set `self.Attack?` true)
  (`KismetSystemLibrary.Delay` 0.2)
  (set `self.Attack?` false)
  (`/Engine/EditorBlueprintResources/StandardMacros.IsValid` _currentweapon
    (:`Is Valid`
      (message `/Game/Blueprint/Interface/BPI_WeaponAttack.LightAttack` _currentweapon))))

(event `self.ChargeAttack`
  (bind _currentweapon (`self.CurrentWeapon`))
  (set `self.Attack?` true)
  (`KismetSystemLibrary.Delay` 0.2)
  (set `self.Attack?` false)
  (`/Engine/EditorBlueprintResources/StandardMacros.IsValid` _currentweapon
    (:`Is Valid`
      (message `/Game/Blueprint/Interface/BPI_WeaponAttack.HeavyAttack` _currentweapon))))

(event `self.OnLaunched`
  (params (LaunchVelocity :type "Vector Structure") (bXYOverride :type Boolean) (bZOverride :type Boolean))
  ;[1 1 1] Stop Movement to avoid bug when launched
  (set `self.Launched?` true)
  (`Controller.StopMovement` (`self.GetController`)))

(event `self.OnLanded`
  (params (Hit :type "HitResult Structure (by ref)"))
  ;[1 1 1] Launched is false after landing
  (set `self.Launched?` false))

(event `self.CapsuleComponent.OnComponentHit`
  (params (HitComponent :type "PrimitiveComponent Object Reference") (OtherActor :type "Actor Object Reference") (OtherComp :type "PrimitiveComponent Object Reference") (NormalImpulse :type "Vector Structure") (Hit :type "HitResult Structure (by ref)"))
  (bind _returnvalue (`self.GetComponentByClass` OtherActor "/Game/Blueprint/Component/Actor/BP_AC_LivingActor.BP_AC_LivingActor_C"))
  (bind (_returnvalue_x _returnvalue_y) (`KismetMathLibrary.BreakVector` (* (`KismetMathLibrary.Normal` (- (`self.K2_GetActorLocation` OtherActor) (`self.K2_GetActorLocation`))) (500.0 500.0 0.0))))
  ;[1 1 1] Push other enemies while launched
  (`/Engine/EditorBlueprintResources/StandardMacros.IsValid` OtherActor
    (:`Is Valid`
      (if (and (`self.Launched?`) (`KismetSystemLibrary.IsValid` _returnvalue))
        (`/Game/Blueprint/Component/Actor/BP_AC_LivingActor.Pushed` _returnvalue (`KismetMathLibrary.MakeVector` _returnvalue_x _returnvalue_y 100.0))))))

(fn `HeavyAttack`
  (returns (`CanAttack?` :type Boolean))
  (return false))

(fn `LightAttack`
  (returns (`CanAttack?` :type Boolean))
  (return false))

(fn `OnSpecialAttack`
  (returns (`CanAttack?` :type Boolean))
  (return false))

(fn `OnSpecialAttackReleased`
  (returns (`CanAttack?` :type Boolean))
  (return false))

(fn `OwnerTakeHit`
  (params (Attacker :type "Actor Object Reference") (Damage :type "Float (double-precision)"))
  (returns (`TakingDamage?` :type Boolean) (NewDamage :type "Float (double-precision)"))
  (return false 0.0))

(fn `UserConstructionScript`)