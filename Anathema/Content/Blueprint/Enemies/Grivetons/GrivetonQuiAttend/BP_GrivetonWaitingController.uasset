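; AI controller for the waiting Griveton enemy, running its behavior tree and switching to an empty one on death.
; Perception latches CanSeePlayer, while Tick randomly rates Dangerosity Low or Medium from the player's attack state.
; When the player is invincible, Tick flags a mirage and targets the pawn's Dummy if valid.
; Arc sets TargetLocation along the player direction, rotated by a random angle chosen at possession.
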(event `RemoveBtOnDeath`
  (if (<= (`/Game/Blueprint/Component/Actor/BP_AC_LivingActor.CurrentHp` (`/Game/Blueprint/Enemies/BP_AIParent.BP_AC_LivingActor` (`self.MyPawn`))) 0.0)
    (`self.RunBehaviorTree` "/Game/Blueprint/Enemies/SeptusCielus/BT_Nothing.BT_Nothing")))

(event `self.ReceivePossess`
  (params (PossessedPawn :type "Pawn Object Reference"))
  (`self.RunBehaviorTree` "/Game/Blueprint/Enemies/Grivetons/GrivetonQuiAttend/BT_GrivetonWaiting.BT_GrivetonWaiting")
  (set `self.MyPawn` (cast `/Game/Blueprint/Enemies/Grivetons/GrivetonQuiAttend/BP_GrivetonWaiting` (`self.K2_GetPawn`) :!pure true))
  (bind _output_get (set `self.AngleArc` (`KismetMathLibrary.RandomFloatInRange` -45.0 45.0)))
  (`BlackboardComponent.SetValueAsFloat` (`AIBlueprintHelperLibrary.GetBlackboard` null) "Angle" _output_get)
  (bind _asbp_griveton_waiting (cast `/Game/Blueprint/Enemies/Grivetons/GrivetonQuiAttend/BP_GrivetonWaiting` (`self.K2_GetPawn`)))
  (set `self.PawnRef` _asbp_griveton_waiting)
  (`KismetSystemLibrary.Delay` 0.2)
  (bind _asbp_player (cast `/Game/Blueprint/Player/BP_Player` (`GameplayStatics.GetPlayerPawn` 0) :!label _label)
    (:`then`
      (set `self.PlayerRef` _asbp_player)
      (`self.SetActorTickEnabled` true))
    (:`CastFailed`
      (`KismetSystemLibrary.Delay` 0.2)
      (goto _label))))

(event `self.AIPerception.OnTargetPerceptionUpdated`
  (params (Actor :type "Actor Object Reference") (Stimulus :type "AIStimulus Structure"))
  (cast `/Game/Blueprint/Player/BP_Player` Actor)
  (bind _output_get (set `self.EntreDeux` (`.bSuccessfullySensed` (break `AIStimulus` Stimulus))))
  (if _output_get
    (`BlackboardComponent.SetValueAsBool` (`AIBlueprintHelperLibrary.GetBlackboard` null) "CanSeePlayer" true)))

(event `self.ReceiveTick`
  (params (DeltaSeconds :type "Float (single-precision)"))
  (bind _asbp_player (cast `/Game/Blueprint/Player/BP_Player` (`GameplayStatics.GetPlayerPawn` 0) :!pure true))
  (`|ExecutionSequence`
    (:`then_0`
      (switch `/Game/Blueprint/Enum/E_PlayerAttackStateTest` (`/Game/Blueprint/Component/BP_WeaponComponent.AttackState` (`/Game/Blueprint/Player/BP_Player.CurrentWeapon` (`self.PlayerRef`)))
        (:`NewEnumerator0`
          (bind _output_get (set `self.Dangerosity` "Low" :!label _label_2))
          (`BlackboardComponent.SetValueAsName` (`self.Blackboard`) "Dangerosity" _output_get))
        (:`NewEnumerator1`
          (bind _output_get_2 (set `self.50%Chance` (== (`KismetMathLibrary.RandomInteger` 2) 1) :!label _label_3))
          (if _output_get_2
            (bind _output_get_3 (set `self.Dangerosity` "Medium"))
            (`BlackboardComponent.SetValueAsName` (`self.Blackboard`) "Dangerosity" _output_get_3)
            (else
              (goto _label_2))))
        (:`NewEnumerator2`
          (goto _label_3))
        (:`NewEnumerator3`
          (goto _label_2))))
    (:`then_1`
      (`/Engine/EditorBlueprintResources/StandardMacros.IsValid` _asbp_player
        (:`Is Valid`
          (if (`/Game/Blueprint/Component/Actor/BP_AC_LivingActor.Invincible?` (`/Game/Blueprint/Player/BP_Player.BP_AC_LivingActor` _asbp_player))
            (`BlackboardComponent.SetValueAsBool` (`self.Blackboard`) "MirageOn?" true)
            (bind _dummy (`/Game/Blueprint/Enemies/BP_AIParent.Dummy` (stale `self.ReceivePossess` _asbp_griveton_waiting)))
            (`/Engine/EditorBlueprintResources/StandardMacros.IsValid` _dummy
              (:`Is Valid`
                (`BlackboardComponent.SetValueAsVector` (`self.Blackboard`) "TargetLocation" (`self.K2_GetActorLocation` _dummy))))
            (else
              (`BlackboardComponent.SetValueAsBool` (`self.Blackboard`) "MirageOn?" false))))))))

(fn `Arc`
  (bind (_returnvalue_x _returnvalue_y) (`KismetMathLibrary.BreakVector` (`self.K2_GetActorLocation` (`self.PlayerRef`))))
  (bind (_returnvalue_x_2 _returnvalue_y_2) (`KismetMathLibrary.BreakVector` (`self.K2_GetActorLocation` (`self.PawnRef`))))
  (`BlackboardComponent.SetValueAsVector` (`AIBlueprintHelperLibrary.GetBlackboard` null) "TargetLocation" (+ (`self.K2_GetActorLocation` (`self.PawnRef`)) (`KismetMathLibrary.Conv_Vector2DToVector` (* (`KismetMathLibrary.Normal2D` (`KismetMathLibrary.GetRotated2D` (`KismetMathLibrary.MakeVector2D` (- _returnvalue_x _returnvalue_x_2) (- _returnvalue_y _returnvalue_y_2)) (`self.AngleArc`))) 350.0)))))

(fn `UserConstructionScript`)