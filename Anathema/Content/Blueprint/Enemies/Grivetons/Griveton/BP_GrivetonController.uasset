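; AI controller for the Griveton enemy that runs its behavior tree and feeds combat awareness of the player into the blackboard.
; Each tick it maps the player's weapon attack state to a Dangerosity level.
; While the player is invincible, it flags MirageOn? and targets the Griveton's Dummy, if valid.
; The Arc function sets TargetLocation at a fixed-length step toward the player, rotated by a random angle chosen on possess.
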(event `self.ReceivePossess`
  (params (PossessedPawn :type "Pawn Object Reference"))
  (`self.RunBehaviorTree` "/Game/Blueprint/Enemies/Grivetons/Griveton/BT_Griveton.BT_Griveton")
  (set `self.AngleArc` (`KismetMathLibrary.RandomFloatInRange` -45.0 45.0))
  (bind _asbp_griveton (cast `/Game/Blueprint/Enemies/Grivetons/Griveton/BP_Griveton` (`self.K2_GetPawn`)))
  (set `self.PawnRef` _asbp_griveton)
  (`KismetSystemLibrary.Delay` 0.2)
  (bind _asbp_player (cast `/Game/Blueprint/Player/BP_Player` (`GameplayStatics.GetPlayerPawn` 0)))
  (set `self.PlayerRef` _asbp_player)
  (`self.SetActorTickEnabled` true))

(event `self.ReceiveTick`
  (params (DeltaSeconds :type "Float (single-precision)"))
  (bind _blackboard (`self.Blackboard`))
  (`|ExecutionSequence`
    (:`then_0`
      (switch `/Game/Blueprint/Enum/E_PlayerAttackStateTest` (`/Game/Blueprint/Component/BP_WeaponComponent.AttackState` (`/Game/Blueprint/Player/BP_Player.CurrentWeapon` (`self.PlayerRef`)))
        (:`NewEnumerator0`
          (bind _output_get (set `self.Dangerosity` "Low"))
          (`BlackboardComponent.SetValueAsName` _blackboard "Dangerosity" _output_get))
        (:`NewEnumerator1`
          (bind _output_get_2 (set `self.Dangerosity` "Medium" :!label _label))
          (`BlackboardComponent.SetValueAsName` _blackboard "Dangerosity" _output_get_2))
        (:`NewEnumerator2`
          (bind _output_get_3 (set `self.Dangerosity` "High"))
          (`BlackboardComponent.SetValueAsName` _blackboard "Dangerosity" _output_get_3))
        (:`NewEnumerator3`
          (goto _label))))
    (:`then_1`
      (if (`/Game/Blueprint/Component/Actor/BP_AC_LivingActor.Invincible?` (`/Game/Blueprint/Player/BP_Player.BP_AC_LivingActor` (cast `/Game/Blueprint/Player/BP_Player` (`GameplayStatics.GetPlayerPawn` 0) :!pure true)))
        (`BlackboardComponent.SetValueAsBool` (`self.Blackboard`) "MirageOn?" true)
        (bind _dummy (`/Game/Blueprint/Enemies/BP_AIParent.Dummy` (stale `self.ReceivePossess` _asbp_griveton)))
        (`/Engine/EditorBlueprintResources/StandardMacros.IsValid` _dummy
          (:`Is Valid`
            (`BlackboardComponent.SetValueAsVector` (`self.Blackboard`) "TargetLocation" (`self.K2_GetActorLocation` _dummy))))
        (else
          (`BlackboardComponent.SetValueAsBool` (`self.Blackboard`) "MirageOn?" false))))))

(fn `Arc`
  (bind (_returnvalue_x _returnvalue_y) (`KismetMathLibrary.BreakVector` (`self.K2_GetActorLocation` (`self.PlayerRef`))))
  (bind (_returnvalue_x_2 _returnvalue_y_2) (`KismetMathLibrary.BreakVector` (`self.K2_GetActorLocation` (`self.PawnRef`))))
  (`BlackboardComponent.SetValueAsVector` (`AIBlueprintHelperLibrary.GetBlackboard` null) "TargetLocation" (+ (`self.K2_GetActorLocation` (`self.PawnRef`)) (`KismetMathLibrary.Conv_Vector2DToVector` (* (`KismetMathLibrary.Normal2D` (`KismetMathLibrary.GetRotated2D` (`KismetMathLibrary.MakeVector2D` (- _returnvalue_x _returnvalue_x_2) (- _returnvalue_y _returnvalue_y_2)) (`self.AngleArc`))) 350.0)))))

(fn `UserConstructionScript`)