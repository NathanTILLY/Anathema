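; Griveton enemy Blueprint that adds a chance-based stun reaction to damage for its AI.
; The Stunned event flags heavy hits and, on a coin flip, raises the "IsStun?" Blackboard key, then clears it after a short delay matching the stun animation.
; OwnerTakeHit always returns no damage taken, while BeginPlay and Tick add no behavior.
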(event `self.ReceiveTick`
  (params (DeltaSeconds :type "Float (single-precision)")))

(event `self.Stunned`
  (params (DamageTaken :type "Float (single-precision)") (AttackType :type "/Game/Blueprint/Enum/E_AttackType Enum" :default "NewEnumerator0"))
  (bind _output_get (set `self.IsStun?` (>= DamageTaken 3.0)))
  (if _output_get
    (if (== (`KismetMathLibrary.RandomInteger` 2) 1)
      (`BlackboardComponent.SetValueAsBool` (`AIBlueprintHelperLibrary.GetBlackboard` null) "IsStun?" (`self.IsStun?`))
      ;[1 1 1] durée animation stun
      (`KismetSystemLibrary.Delay` 0.5)
      (bind _output_get_2 (set `self.IsStun?` false))
      (`BlackboardComponent.SetValueAsBool` (`AIBlueprintHelperLibrary.GetBlackboard` null) "IsStun?" _output_get_2))))

(fn `OwnerTakeHit`
  (params (Attacker :type "Actor Object Reference") (Damage :type "Float (double-precision)"))
  (returns (`TakingDamage?` :type Boolean) (NewDamage :type "Float (double-precision)"))
  (return false 0.0))

(fn `UserConstructionScript`
  (`parent.UserConstructionScript`))