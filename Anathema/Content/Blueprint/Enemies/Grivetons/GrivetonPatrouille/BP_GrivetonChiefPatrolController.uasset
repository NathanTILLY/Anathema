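; AI controller for the chief Griveton patrol enemy, running its patrol behavior tree and seeding the Blackboard from the pawn's patrol path.
; On possess it sets walk speed and, if minions are requested, spawns a single patrol minion linked to the chief, as the loop zeroes the count.
; Perception flags player sighting; Tick rates threat from the player's attack state and handles a mirage dummy target while the player is invincible.
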(event `self.ReceivePossess`
  (params (PossessedPawn :type "Pawn Object Reference"))
  (bind _returnvalue (`AIBlueprintHelperLibrary.GetBlackboard` null))
  (`|ExecutionSequence`
    (:`then_0`
      (`self.RunBehaviorTree` "/Game/Blueprint/Enemies/Grivetons/GrivetonPatrouille/BT_GrivetonChiefPatrol.BT_GrivetonChiefPatrol")
      (bind _output_get (set `self.PawnRef` (cast `/Game/Blueprint/Enemies/Grivetons/GrivetonPatrouille/BP_GrivetonChiefPatrol` (`self.K2_GetPawn`) :!pure true)))
      (`KismetSystemLibrary.Delay` 0.01)
      (`BlackboardComponent.SetValueAsBool` (`AIBlueprintHelperLibrary.GetBlackboard` null) "PathLooping" (`/Game/Blueprint/Enemies/Grivetons/GrivetonPatrouille/BP_PatrolPath.IsLooping` (`/Game/Blueprint/Enemies/Grivetons/GrivetonPatrouille/BP_GrivetonChiefPatrol.PatrolPathGriveton` _output_get)))
      (`BlackboardComponent.SetValueAsInt` _returnvalue "Direction" 1)
      (`BlackboardComponent.SetValueAsFloat` _returnvalue "WaitTime" (`/Game/Blueprint/Enemies/Grivetons/GrivetonPatrouille/BP_PatrolPath.WaitTime` (`/Game/Blueprint/Enemies/Grivetons/GrivetonPatrouille/BP_GrivetonChiefPatrol.PatrolPathGriveton` (`self.PawnRef`))))
      (while (> (`/Game/Blueprint/Enemies/Grivetons/GrivetonPatrouille/BP_GrivetonChiefPatrol.NumberOfMinions` (`self.PawnRef`)) 0)
        (bind _returnvalue_2 (`|SpawnActorFromClass` "/Game/Blueprint/Enemies/Grivetons/GrivetonPatrouille/BP_GrivetonMinionPatrol.BP_GrivetonMinionPatrol_C" (`KismetMathLibrary.MakeTransform` (`KismetMathLibrary.MakeVector` (+ (.x (.location (`self.GetTransform` (`self.PawnRef`)))) 300.0) (+ (.y (.location (`self.GetTransform` (`self.PawnRef`)))) 300.0) (.z (.location (`self.GetTransform` (`self.PawnRef`))))) (.rotation (`self.GetTransform` (`self.PawnRef`))) (.scale (`self.GetTransform` (`self.PawnRef`)))) "AdjustIfPossibleButAlwaysSpawn" "OverrideRootScale" null null))
        (`KismetArrayLibrary.Array_Add` (`self.Minions`) _returnvalue_2)
        (set `/Game/Blueprint/Enemies/Grivetons/GrivetonPatrouille/BP_GrivetonMinionPatrol.PatrolChief` (`self.PawnRef`) _returnvalue_2)
        (set `/Game/Blueprint/Enemies/Grivetons/GrivetonPatrouille/BP_GrivetonChiefPatrol.NumberOfMinions` 0 (`self.PawnRef`))))
    (:`then_1`
      (set `CharacterMovementComponent.MaxWalkSpeed` (`self.Speed`) (`Character.CharacterMovement` (`self.PawnRef`))))))

(event `self.AIPerception.OnTargetPerceptionUpdated`
  (params (Actor :type "Actor Object Reference") (Stimulus :type "AIStimulus Structure"))
  (bind _asbp_player (cast `/Game/Blueprint/Player/BP_Player` Actor))
  (set `self.PlayerRef` _asbp_player)
  (`BlackboardComponent.SetValueAsBool` (`AIBlueprintHelperLibrary.GetBlackboard` null) "CanSeePlayer" (`.bSuccessfullySensed` (break `AIStimulus` Stimulus)))
  (`self.SetActorTickEnabled` true))

(event `CustomEvent`
  (for _array_element (`self.Minions`)
    (set `/Game/Blueprint/Enemies/Grivetons/GrivetonPatrouille/BP_GrivetonMinionPatrol.TheChiefIsMoving` false _array_element)))

(event `self.ReceiveTick`
  (params (DeltaSeconds :type "Float (single-precision)"))
  (bind _playerref (`self.PlayerRef`))
  (bind _blackboard (`self.Blackboard`))
  (`|ExecutionSequence`
    (:`then_0`
      (switch `/Game/Blueprint/Enum/E_PlayerAttackStateTest` (`/Game/Blueprint/Component/BP_WeaponComponent.AttackState` (`/Game/Blueprint/Player/BP_Player.CurrentWeapon` _playerref))
        (:`NewEnumerator0`
          (bind _output_get (set `self.Dangerosity` "Low"))
          (`BlackboardComponent.SetValueAsName` _blackboard "Dangerosity" _output_get))
        (:`NewEnumerator1`
          (bind _output_get_2 (set `self.Dangerosity` "Medium" :!label _label))
          (`BlackboardComponent.SetValueAsName` _blackboard "Dangerosity" _output_get_2))
        (:`NewEnumerator2`
          (bind _output_get_3 (set `self.Dangerosity` "High"))
          (`BlackboardComponent.SetValueAsName` _blackboard "Dangerosity" _output_get_3))
        (:`NewEnumerator3`
          (goto _label))))
    (:`then_1`
      (if (`/Game/Blueprint/Component/Actor/BP_AC_LivingActor.Invincible?` (`/Game/Blueprint/Player/BP_Player.BP_AC_LivingActor` (cast `/Game/Blueprint/Player/BP_Player` (`GameplayStatics.GetPlayerPawn` 0) :!pure true)))
        (`BlackboardComponent.SetValueAsBool` (`self.Blackboard`) "MirageOn?" true)
        (`/Engine/EditorBlueprintResources/StandardMacros.IsValid` null
          (:`Is Valid`
            (`BlackboardComponent.SetValueAsVector` (`self.Blackboard`) "TargetLocation" (`self.K2_GetActorLocation` (`/Game/Blueprint/Enemies/BP_AIParent.Dummy` (cast `/Game/Blueprint/Enemies/Grivetons/GrivetonPatrouille/BP_GrivetonChiefPatrol` (`self.K2_GetPawn`) :!pure true))))))
        (else
          (`BlackboardComponent.SetValueAsBool` (`self.Blackboard`) "MirageOn?" false))))
    (:`then_2`
      (`KismetSystemLibrary.PrintString` (`KismetSystemLibrary.GetDisplayName` _playerref)))))

(fn `UserConstructionScript`)