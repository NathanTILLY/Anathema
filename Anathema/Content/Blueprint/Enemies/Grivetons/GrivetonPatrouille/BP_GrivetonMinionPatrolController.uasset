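; AI controller for Griveton patrol minions that runs their behavior tree and sets their walk speed on possession.
; Perception updates record whether the player is seen in the blackboard and enable Tick.
; Tick writes a random reachable point near the patrol chief as the chief location and clears the minion's chief-moving flag after a short delay.
; It also mirrors player invincibility into a mirage flag, supplying a dummy's location as target.
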(event `self.ReceivePossess`
  (params (PossessedPawn :type "Pawn Object Reference"))
  (`|ExecutionSequence`
    (:`then_0`
      (`self.RunBehaviorTree` "/Game/Blueprint/Enemies/Grivetons/GrivetonPatrouille/BT_GrivetonMinionPatrol.BT_GrivetonMinionPatrol")
      (bind _asbp_griveton_minion_patrol (cast `/Game/Blueprint/Enemies/Grivetons/GrivetonPatrouille/BP_GrivetonMinionPatrol` (`self.K2_GetPawn`)))
      (set `self.MyPawns` _asbp_griveton_minion_patrol)
      (`BlackboardComponent.SetValueAsObject` (`AIBlueprintHelperLibrary.GetBlackboard` null) "ChiefPatrol" (`/Game/Blueprint/Enemies/Grivetons/GrivetonPatrouille/BP_GrivetonMinionPatrol.PatrolChief` (`self.MyPawns`))))
    (:`then_1`
      (set `CharacterMovementComponent.MaxWalkSpeed` (`self.Speed`) (`Character.CharacterMovement` (`self.MyPawns`))))))

(event `self.AIPerception.OnTargetPerceptionUpdated`
  (params (Actor :type "Actor Object Reference") (Stimulus :type "AIStimulus Structure"))
  (bind _asbp_player (cast `/Game/Blueprint/Player/BP_Player` Actor))
  (set `self.PlayerRef` _asbp_player)
  (`BlackboardComponent.SetValueAsBool` (`AIBlueprintHelperLibrary.GetBlackboard` null) "CanSeePlayer" (`.bSuccessfullySensed` (break `AIStimulus` Stimulus)))
  (`self.SetActorTickEnabled` true))

(event `self.ReceiveTick`
  (params (DeltaSeconds :type "Float (single-precision)"))
  (`|ExecutionSequence`
    (:`then_0`
      (`BlackboardComponent.SetValueAsVector` (`AIBlueprintHelperLibrary.GetBlackboard` null) "ChiefLocation" (`NavigationSystemV1.K2_GetRandomReachablePointInRadius` (`self.K2_GetActorLocation` (`/Game/Blueprint/Enemies/Grivetons/GrivetonPatrouille/BP_GrivetonMinionPatrol.PatrolChief` (`self.MyPawns`))) 100.0 null null))
      (`KismetSystemLibrary.Delay` 0.1)
      (set `/Game/Blueprint/Enemies/Grivetons/GrivetonPatrouille/BP_GrivetonMinionPatrol.TheChiefIsMoving` false (`self.MyPawns`)))
    (:`then_1`
      (if (`/Game/Blueprint/Component/Actor/BP_AC_LivingActor.Invincible?` (`/Game/Blueprint/Player/BP_Player.BP_AC_LivingActor` (cast `/Game/Blueprint/Player/BP_Player` (`GameplayStatics.GetPlayerPawn` 0) :!pure true)))
        (`BlackboardComponent.SetValueAsBool` (`self.Blackboard`) "MirageOn?" true)
        (`/Engine/EditorBlueprintResources/StandardMacros.IsValid` null
          (:`Is Valid`
            (`BlackboardComponent.SetValueAsVector` (`self.Blackboard`) "TargetLocation" (`self.K2_GetActorLocation` (`/Game/Blueprint/Enemies/BP_AIParent.Dummy` (stale `self.ReceivePossess` _asbp_griveton_minion_patrol))))))
        (else
          (`BlackboardComponent.SetValueAsBool` (`self.Blackboard`) "MirageOn?" false))))))

(fn `UserConstructionScript`)