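; BP_GrivetonChiefPatrol is the chief patrol Griveton enemy, adding a stun reaction to heavy hits.
; When its BP_AC_LivingActor component reports damage at or above a fixed threshold, it sets a stun flag on itself and on the AI Blackboard.
; A short delay, matching the stun animation's duration, then clears both flags.
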(event `self.BP_AC_LivingActor.OnTakingDamage`
  (params (AttackOwner :type "Actor Object Reference") (DamageTaken :type "Float (single-precision)") (AttackType :type "/Game/Blueprint/Enum/E_AttackType Enum" :default "NewEnumerator0"))
  (bind _output_get (set `self.IsStun?` (>= DamageTaken 1.5)))
  (if _output_get
    (`BlackboardComponent.SetValueAsBool` (`AIBlueprintHelperLibrary.GetBlackboard` null) "IsStun?" (`self.IsStun?`))
    ;[1 1 1] durée animation stun
    (`KismetSystemLibrary.Delay` 1.0)
    (bind _output_get_2 (set `self.IsStun?` false))
    (`BlackboardComponent.SetValueAsBool` (`AIBlueprintHelperLibrary.GetBlackboard` null) "IsStun?" _output_get_2)))

(fn `UserConstructionScript`
  (`parent.UserConstructionScript`))