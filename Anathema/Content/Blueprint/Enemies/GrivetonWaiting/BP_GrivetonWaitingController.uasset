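; AI controller for the waiting Griveton enemy that runs its behavior tree and sets the pawn's walk speed on possess.
; Perception flags the player as seen in the blackboard, with no branch that clears it.
; Each tick it decrements the player's shared Tickets count whenever positive and sets the Ticket key.
; It also updates TargetLocation to a fixed-distance point toward the player, rotated by a per-enemy random angle for an arcing approach.
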(event `self.ReceiveTick`
  (params (DeltaSeconds :type "Float (single-precision)"))
  (`self.TakeTicket`)
  (`self.Arc`))

(event `self.ReceivePossess`
  (params (PossessedPawn :type "Pawn Object Reference"))
  (`|ExecutionSequence`
    (:`then_0`
      (`self.RunBehaviorTree` "/Game/Blueprint/Enemies/GrivetonWaiting/BT_GrivetonWaiting.BT_GrivetonWaiting")
      (bind _ascharacter (cast `Character` (`self.K2_GetPawn`)))
      (set `self.PawnRef` _ascharacter)
      (bind _asbp_player (cast `/Game/Blueprint/Player/BP_Player` (`GameplayStatics.GetPlayerPawn` 0)))
      (set `self.PlayerRef` _asbp_player)
      (set `self.AngleArc` (`KismetMathLibrary.RandomFloatInRange` -45.0 45.0))
      (`self.SetActorTickEnabled` true))
    (:`then_1`
      (set `CharacterMovementComponent.MaxWalkSpeed` (`self.Speed`) (`Character.CharacterMovement` (`self.PawnRef`))))))

(event `self.AIPerception.OnTargetPerceptionUpdated`
  (params (Actor :type "Actor Object Reference") (Stimulus :type "AIStimulus Structure"))
  (bind _output_get (set `self.EntreDeux` (`.bSuccessfullySensed` (break `AIStimulus` Stimulus))))
  (if _output_get
    (`BlackboardComponent.SetValueAsBool` (`AIBlueprintHelperLibrary.GetBlackboard` null) "CanSeePlayer" true)))

(fn `Arc`
  (bind (_returnvalue_x _returnvalue_y) (`KismetMathLibrary.BreakVector` (`self.K2_GetActorLocation` (`self.PlayerRef`))))
  (bind (_returnvalue_x_2 _returnvalue_y_2) (`KismetMathLibrary.BreakVector` (`self.K2_GetActorLocation` (`self.PawnRef`))))
  (`BlackboardComponent.SetValueAsVector` (`AIBlueprintHelperLibrary.GetBlackboard` null) "TargetLocation" (+ (`self.K2_GetActorLocation` (`self.PawnRef`)) (`KismetMathLibrary.Conv_Vector2DToVector` (* (`KismetMathLibrary.Normal2D` (`KismetMathLibrary.GetRotated2D` (`KismetMathLibrary.MakeVector2D` (- _returnvalue_x _returnvalue_x_2) (- _returnvalue_y _returnvalue_y_2)) (`self.AngleArc`))) 350.0)))))

(fn `TakeTicket`
  (bind _tickets (`/Game/Blueprint/Player/BP_Player.Tickets` (`self.PlayerRef`)))
  (if (> _tickets 0)
    (set `/Game/Blueprint/Player/BP_Player.Tickets` (- _tickets 1) (`self.PlayerRef`))
    (`BlackboardComponent.SetValueAsBool` (`AIBlueprintHelperLibrary.GetBlackboard` null) "Ticket" true)))

(fn `UserConstructionScript`)