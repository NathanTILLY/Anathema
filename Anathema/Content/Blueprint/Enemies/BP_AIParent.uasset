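; Parent Blueprint for AI enemies, providing shared armor break-apart logic and stub combat functions.
; CreateArmorList gathers valid pieces from a fixed set into a unique list.
; ArmorExplode switches those pieces to IgnorePawn collision, enables physics and pushes them with a large force opposite ExplosionVector.
; Attack and hit functions return only false or zero, and the event graph has no active logic.
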(fn `ArmorExplode`
  (for _array_element (`self.ArmorPiecesList`)
    (`/Engine/EditorBlueprintResources/StandardMacros.IsValid` _array_element
      (:`Is Valid`
        (`PrimitiveComponent.SetCollisionProfileName` _array_element "IgnorePawn" true)
        (`PrimitiveComponent.SetSimulatePhysics` _array_element true)
        (`PrimitiveComponent.AddForce` _array_element (* (`self.ExplosionVector`) -500000.0) "None" false)))))

(fn `CreateArmorList`
  (for _array_element (`|MakeArray` null null null null null null null null null null null null null null null null null null null :!type "StaticMeshComponent Object Reference")
    (`/Engine/EditorBlueprintResources/StandardMacros.IsValid` _array_element
      (:`Is Valid`
        (`KismetArrayLibrary.Array_AddUnique` (`self.ArmorPiecesList`) _array_element))))
  (return))

(fn `HeavyAttack`
  (returns (`CanAttack?` :type Boolean))
  (return false))

(fn `LightAttack`
  (returns (`CanAttack?` :type Boolean))
  (return false))

(fn `OnSpecialAttack`
  (returns (`CanAttack?` :type Boolean))
  (return false))

(fn `OnSpecialAttackReleased`
  (returns (`CanAttack?` :type Boolean))
  (return false))

(fn `OwnerTakeHit`
  (params (Attacker :type "Actor Object Reference") (Damage :type "Float (double-precision)"))
  (returns (`TakingDamage?` :type Boolean) (NewDamage :type "Float (double-precision)"))
  (return false 0.0))

(fn `UserConstructionScript`)