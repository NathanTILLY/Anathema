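; Player-attached manager that runs Griveton enemy waves with war horn and music once the king has talked.
; Its sphere flags overlapped BP_PeriodicSpawner actors, and waves spawn only at those.
; The first wave polls until all Grivetons are gone, removes the objectives widget, then after a delay and health check calls PeriodicWavesStart.
; That event's counter increment is unwired, so it spawns one round and never schedules another.
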(event `self.Sphere.OnComponentBeginOverlap`
  (params (OverlappedComponent :type "PrimitiveComponent Object Reference") (OtherActor :type "Actor Object Reference") (OtherComp :type "PrimitiveComponent Object Reference") (OtherBodyIndex :type Integer) (bFromSweep :type Boolean) (SweepResult :type "HitResult Structure (by ref)"))
  (bind _asbp_periodic_spawner (cast `/Game/Blueprint/Spawners/BP_PeriodicSpawner` OtherActor))
  (set `/Game/Blueprint/Spawners/BP_PeriodicSpawner.InRangeOfPlayer` true _asbp_periodic_spawner))

(event `self.Sphere.OnComponentEndOverlap`
  (params (OverlappedComponent :type "PrimitiveComponent Object Reference") (OtherActor :type "Actor Object Reference") (OtherComp :type "PrimitiveComponent Object Reference") (OtherBodyIndex :type Integer))
  (bind _asbp_periodic_spawner (cast `/Game/Blueprint/Spawners/BP_PeriodicSpawner` OtherActor))
  (set `/Game/Blueprint/Spawners/BP_PeriodicSpawner.InRangeOfPlayer` false _asbp_periodic_spawner))

(event `self.ReceiveBeginPlay`
  (set `self.RefPlayer` (cast `/Game/Blueprint/Player/BP_Player` (`GameplayStatics.GetPlayerCharacter` 0) :!pure true))
  (`self.K2_AttachToActor` (`self.RefPlayer`) "SwordSocket" "SnapToTarget" "SnapToTarget" "KeepRelative"))

(event `self.ReceiveTick`
  (params (DeltaSeconds :type "Float (single-precision)"))
  (bind _wbp_objectives (`/Game/Blueprint/BP_GameInstance.WBP_Objectives` (cast `/Game/Blueprint/BP_GameInstance` (`GameplayStatics.GetGameInstance`) :!pure true)))
  (bind _currenthp (`/Game/Blueprint/Component/Actor/BP_AC_LivingActor.CurrentHp` (`/Game/Blueprint/Player/BP_Player.BP_AC_LivingActor` (`self.RefPlayer`))))
  ;[1 1 1] Première itération qui se déclenche lorque le roi a finit de nous parler
  (if (`self.KingHasTalked`)
    (`/Engine/EditorBlueprintResources/StandardMacros.DoOnce` false
      (:`Completed`
        (`GameplayStatics.PlaySoundAtLocation` "/Game/Audio/SFX/Sound/A_CorDeGuerre.A_CorDeGuerre" (`self.K2_GetActorLocation` (`self.RefPlayer`)) (struct) 1.0 1.0 0.0 null null null)
        (bind _returnvalue (`AddComponent|NODE_AddAudioComponent-0` :`self` (`GameplayStatics.GetPlayerPawn` 0)))
        (set `self.MusicPlaying` _returnvalue)
        (bind _outactors (`GameplayStatics.GetAllActorsOfClass` "/Game/Blueprint/Spawners/BP_PeriodicSpawner.BP_PeriodicSpawner_C"))
        (if (< (`self.NumberOfAlreadySpawned`) (`self.NumberToSpawn`)) :!label _label
          (for _array_element _outactors
            (if (`/Game/Blueprint/Spawners/BP_PeriodicSpawner.InRangeOfPlayer` _array_element)
              (`AIBlueprintHelperLibrary.SpawnAIFromClass` "/Game/Blueprint/Enemies/Grivetons/Griveton/BP_Griveton.BP_Griveton_C" null (`self.K2_GetActorLocation` _array_element) (struct) false null)))
          (`/Engine/EditorBlueprintResources/StandardMacros.IncrementInt` (`self.NumberOfAlreadySpawned`)
            (:`  `
              (goto _label)))
          (else
            (bind _outactors_2 (`GameplayStatics.GetAllActorsOfClass` "/Game/Blueprint/Enemies/Grivetons/Griveton/BP_Griveton.BP_Griveton_C" :!label _label_2))
            (if (== (`KismetArrayLibrary.Array_Length` _outactors_2) 0)
              (`AudioComponent.FadeOut` (`self.MusicPlaying`) 0.0 0.0 "Linear")
              (`AddComponent|NODE_AddAudioComponent-1` :`self` (`GameplayStatics.GetPlayerPawn` 0))
              (`KismetSystemLibrary.Delay` 0.5)
              (`/Game/Blueprint/UI/WBP_Objectives.FadeOut` _wbp_objectives)
              (`KismetSystemLibrary.Delay` 0.5)
              (`Widget.RemoveFromParent` _wbp_objectives)
              (set `self.NumberOfAlreadySpawned` 0)
              (`KismetSystemLibrary.Delay` (`self.PeriodicSpawnTime`))
              (if (> _currenthp 10.0) :!label _label_3
                (`self.PeriodicWavesStart`)
                (else
                  (if (<= _currenthp 10.0) :!label _label_4
                    (`KismetSystemLibrary.Delay` 2.0)
                    (goto _label_4)
                    (else
                      (goto _label_3)))))
              (else
                (`KismetSystemLibrary.Delay` 1.0)
                (goto _label_2)))))))))

(event `PeriodicWavesStart`
  (bind _currenthp (`/Game/Blueprint/Component/Actor/BP_AC_LivingActor.CurrentHp` (`/Game/Blueprint/Player/BP_Player.BP_AC_LivingActor` (`self.RefPlayer`))))
  ;[1 1 1] Boucle qui se répète tous les tant de temps
  (`GameplayStatics.PlaySoundAtLocation` "/Game/Audio/SFX/Sound/A_CorDeGuerre.A_CorDeGuerre" (`self.K2_GetActorLocation` (`self.RefPlayer`)) (struct) 1.0 1.0 0.0 null null null)
  (`KismetSystemLibrary.Delay` 1.0)
  (bind _returnvalue (`AddComponent|NODE_AddAudioComponent-2` :`self` (`GameplayStatics.GetPlayerPawn` 0)))
  (set `self.MusicPlaying` _returnvalue)
  (bind _outactors (`GameplayStatics.GetAllActorsOfClass` "/Game/Blueprint/Spawners/BP_PeriodicSpawner.BP_PeriodicSpawner_C"))
  (if (< (`self.NumberOfAlreadySpawned`) (`self.NumberToSpawn`))
    (for _array_element _outactors
      (if (`/Game/Blueprint/Spawners/BP_PeriodicSpawner.InRangeOfPlayer` _array_element)
        (`AIBlueprintHelperLibrary.SpawnAIFromClass` "/Game/Blueprint/Enemies/Grivetons/Griveton/BP_Griveton.BP_Griveton_C" null (`self.K2_GetActorLocation` _array_element) (struct) false null)))
    (else
      (bind _outactors_2 (`GameplayStatics.GetAllActorsOfClass` "/Game/Blueprint/Enemies/Grivetons/Griveton/BP_Griveton.BP_Griveton_C" :!label _label_5))
      (if (== (`KismetArrayLibrary.Array_Length` _outactors_2) 0)
        (`AudioComponent.FadeOut` (`self.MusicPlaying`) 0.0 0.0 "Linear")
        (`AddComponent|NODE_AddAudioComponent-3` :`self` (`GameplayStatics.GetPlayerPawn` 0))
        (set `self.NumberOfAlreadySpawned` 0)
        (`KismetSystemLibrary.Delay` (`self.PeriodicSpawnTime`))
        (if (> _currenthp 10.0) :!label _label_6
          (`self.PeriodicWavesStart`)
          (else
            (if (<= _currenthp 10.0) :!label _label_7
              (`KismetSystemLibrary.Delay` 2.0)
              (goto _label_7)
              (else
                (goto _label_6)))))
        (else
          (`KismetSystemLibrary.Delay` 1.0)
          (goto _label_5))))))

(fn `UserConstructionScript`)