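; Trigger-box spawner that spawns AI mobs at random points from a list when BP_Player overlaps it.
; On overlap it destroys the linked AutreSpawn actor if valid, then starts a delayed loop bounded by the NbrDejaSpawn counter and NbrDeSpawn limit.
; Each pass spawns MobASpawn using random SpawnLocation entries for position and rotation, applying slight random uniform scale to successful spawns.
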(event `self.Box.OnComponentBeginOverlap`
  (params (OverlappedComponent :type "PrimitiveComponent Object Reference") (OtherActor :type "Actor Object Reference") (OtherComp :type "PrimitiveComponent Object Reference") (OtherBodyIndex :type Integer) (bFromSweep :type Boolean) (SweepResult :type "HitResult Structure (by ref)"))
  (bind _autrespawn (`self.AutreSpawn`))
  (bind _spawnlocation (`self.SpawnLocation`))
  (bind _rootcomponent (`Actor.RootComponent` (`|GetArrayItem` _spawnlocation (`KismetMathLibrary.RandomInteger` (`KismetArrayLibrary.Array_Length` _spawnlocation)))))
  (cast `/Game/Blueprint/Player/BP_Player` OtherActor)
  (`|ExecutionSequence`
    (:`then_0`
      (`/Engine/EditorBlueprintResources/StandardMacros.IsValid` _autrespawn
        (:`Is Valid`
          (`self.K2_DestroyActor` _autrespawn))))
    (:`then_1`
      (if (<= (`self.NbrDejaSpawn`) (`self.NbrDeSpawn`)) :!label _label
        (`KismetSystemLibrary.Delay` (`self.tempsDeSpawn`))
        (`/Engine/EditorBlueprintResources/StandardMacros.IncrementInt` (`self.NbrDejaSpawn`)
          (:`  `
            (bind _returnvalue (`AIBlueprintHelperLibrary.SpawnAIFromClass` (`self.MobASpawn`) null (`SceneComponent.K2_GetComponentLocation` _rootcomponent) (`SceneComponent.K2_GetComponentRotation` _rootcomponent) false null))
            (`/Engine/EditorBlueprintResources/StandardMacros.IsValid` _returnvalue
              (:`Is Valid`
                (bind _output_get (set `self.CurrentScale` (`KismetMathLibrary.RandomFloatInRange` 0.9 1.1)))
                (`self.SetActorScale3D` _returnvalue (`KismetMathLibrary.MakeVector` _output_get _output_get _output_get))
                (goto _label))
              (:`Is Not Valid`
                (goto _label)))))))))

(fn `UserConstructionScript`)