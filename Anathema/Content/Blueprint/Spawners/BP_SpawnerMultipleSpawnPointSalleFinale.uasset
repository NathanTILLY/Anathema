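; Final-room mob spawner that spawns AI pawns at random points from a list once the player overlaps its box.
; A self-looping chain spawns randomly scaled mobs at random intervals up to a quota, then polls for increases, but ends if a spawn fails.
; NumberToAddEvent raises the quota by the Phase2 or Phase3 amount, depending on whether the first chain is destroyed.
; Location and rotation use separate random picks, so they can come from different points.
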(event `self.Box.OnComponentBeginOverlap`
  (params (OverlappedComponent :type "PrimitiveComponent Object Reference") (OtherActor :type "Actor Object Reference") (OtherComp :type "PrimitiveComponent Object Reference") (OtherBodyIndex :type Integer) (bFromSweep :type Boolean) (SweepResult :type "HitResult Structure (by ref)"))
  (bind _spawnlocation (`self.SpawnLocation`))
  (bind _rootcomponent (`Actor.RootComponent` (`|GetArrayItem` _spawnlocation (`KismetMathLibrary.RandomInteger` (`KismetArrayLibrary.Array_Length` _spawnlocation)))))
  (cast `/Game/Blueprint/Player/BP_Player` OtherActor)
  (if (< (`self.NbrDejaSpawn`) (`self.NbrDeSpawn`)) :!label _label
    (`/Engine/EditorBlueprintResources/StandardMacros.IncrementInt` (`self.NbrDejaSpawn`)
      (:`  `
        (bind _returnvalue (`AIBlueprintHelperLibrary.SpawnAIFromClass` (`self.MobASpawn`) null (`SceneComponent.K2_GetComponentLocation` _rootcomponent) (`SceneComponent.K2_GetComponentRotation` _rootcomponent) false null))
        (`/Engine/EditorBlueprintResources/StandardMacros.IsValid` _returnvalue
          (:`Is Valid`
            (bind _output_get (set `self.CurrentScale` (`KismetMathLibrary.RandomFloatInRange` 0.9 1.1)))
            (`self.SetActorScale3D` _returnvalue (`KismetMathLibrary.MakeVector` _output_get _output_get _output_get))
            (`KismetSystemLibrary.Delay` (`KismetMathLibrary.RandomFloatInRange` 0.0 2.0))
            (goto _label)))))
    (else
      (`KismetSystemLibrary.Delay` 0.2)
      (goto _label))))

(event `NumberToAddEvent`
  (if (`/Game/Blueprint/Objets/BP_Chaine.IsChainDestroyed?` (`self.RefFirstChaine`))
    (set `self.NbrDeSpawn` (+ (`self.NbrDeSpawn`) (`self.Phase3`)))
    (else
      (set `self.NbrDeSpawn` (+ (`self.NbrDeSpawn`) (`self.Phase2`))))))

(fn `UserConstructionScript`)