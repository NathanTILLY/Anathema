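; Scenario actor that breaks open a tent curtain, apparently once the tracked tents in ListTent have been destroyed.
; It binds each tent's OnDestroyed at BeginPlay and removes destroyed entries from the list by matching object names.
; Tick infers an empty list from a blank display name after looping, then enables physics on the curtain's destructible, applies impulse damage and destroys it after a short delay.
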(event `self.ReceiveBeginPlay`
  (for _array_element (`self.ListTent`)
    (add `self.OnDestroyed` _array_element (delegate `CustomEvent_0`))))

(event `CustomEvent_0` :!signature `self.OnDestroyed`
  (params (DestroyedActor :type "Actor Object Reference"))
  (for (_array_element _array_index) (`self.ListTent`)
    (if (`KismetStringLibrary.EqualEqual_StrStr` (`KismetSystemLibrary.GetObjectName` _array_element) (`KismetSystemLibrary.GetObjectName` DestroyedActor))
      (`KismetArrayLibrary.Array_Remove` (`self.ListTent`) _array_index))))

(event `self.ReceiveTick`
  (params (DeltaSeconds :type "Float (single-precision)"))
  (bind _refcurtaintent (`self.RefCurtainTent`))
  (for _array_element (`self.ListTent`)
    _)
  (if (`KismetStringLibrary.IsEmpty` (`KismetSystemLibrary.GetDisplayName` _array_element))
    (`PrimitiveComponent.SetSimulatePhysics` (`DestructibleActor.DestructibleComponent` _refcurtaintent) true)
    (`DestructibleComponent.ApplyDamage` (`DestructibleActor.DestructibleComponent` _refcurtaintent) 1000.0 (`SceneComponent.K2_GetComponentLocation` (`Actor.RootComponent` _refcurtaintent)) (* (`SceneComponent.GetForwardVector` (`Actor.RootComponent` _refcurtaintent)) 1000.0) 5000.0)
    (`KismetSystemLibrary.Delay` 1.0)
    (`self.K2_DestroyActor` (`self.RefCurtainTent`))))

(fn `UserConstructionScript`)