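; Destructible pillar for the final boss room that collapses once the referenced RefSol actor reports it is destroyed.
; Tick polls that flag, then enables physics on the mesh and applies heavy damage with a forward impulse, repeating while the flag holds.
; After a short delay, a one-shot timeline fades the dynamic material created at BeginPlay, then destroys the actor.
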(event `self.ReceiveBeginPlay`
  (bind _returnvalue (`PrimitiveComponent.CreateDynamicMaterialInstance` (`self.Destructible`) 0 null "None")))

(event `self.ReceiveTick`
  (params (DeltaSeconds :type "Float (single-precision)"))
  (bind _refsol (`self.RefSol`))
  (bind _destructible (`self.Destructible`))
  (`/Engine/EditorBlueprintResources/StandardMacros.IsValid` _refsol
    (:`Is Valid`
      (if (`/Game/Blueprint/FinalRoom/SolBoss/BP_sol.Destroyed` _refsol)
        (`PrimitiveComponent.SetSimulatePhysics` _destructible true)
        (`DestructibleComponent.ApplyDamage` _destructible 10000.0 (`SceneComponent.K2_GetComponentLocation` _destructible) (* (`SceneComponent.GetForwardVector` _destructible) 500.0) 1000.0)
        (`KismetSystemLibrary.Delay` 2.5)
        (`/Engine/EditorBlueprintResources/StandardMacros.DoOnce` false
          (:`Completed`
            (`/Engine/EditorBlueprintResources/StandardMacros.FlipFlop`
              (:`A`
                (bind (_direction _value) (`Timeline|Timeline_0` :!label _label)
                  (:`Update`
                    (`MaterialInstanceDynamic.SetScalarParameterValue` (stale `self.ReceiveBeginPlay` _returnvalue) "Fade" (`KismetMathLibrary.Lerp` 1.0 0.0 _value)))
                  (:`Finished`
                    (`self.K2_DestroyActor`))))
              (:`B`
                (goto _label :!via `ReverseFromEnd`)))))))))

(fn `UserConstructionScript`)