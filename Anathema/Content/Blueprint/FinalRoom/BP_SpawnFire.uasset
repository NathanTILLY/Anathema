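; Trigger actor in the final room that lights a series of fires when the player enters its box.
; Two delay-staggered loops run side by side over ListFireSystem, one from each end, working toward the middle.
; Each step shows and restarts a fire's particle system and enables its box collision as query-only.
; Incr1 is never reset here, whereas Incr2 restarts from the last index on each overlap.
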(event `self.Box.OnComponentBeginOverlap`
  (params (OverlappedComponent :type "PrimitiveComponent Object Reference") (OtherActor :type "Actor Object Reference") (OtherComp :type "PrimitiveComponent Object Reference") (OtherBodyIndex :type Integer) (bFromSweep :type Boolean) (SweepResult :type "HitResult Structure (by ref)"))
  (bind _listfiresystem (`self.ListFireSystem`))
  (bind _listfiresystem_2 (`self.ListFireSystem`))
  (bind _returnvalue (`KismetArrayLibrary.Array_LastIndex` _listfiresystem))
  (bind _output (`|GetArrayItem` _listfiresystem (`self.Incr2`)))
  (bind _output_2 (`|GetArrayItem` _listfiresystem_2 (`self.Incr1`)))
  (bind _firesystem (`/Game/Blueprint/FinalRoom/BP_FireSystem.FireSystem` _output))
  (bind _firesystem_2 (`/Game/Blueprint/FinalRoom/BP_FireSystem.FireSystem` _output_2))
  (cast `/Game/Blueprint/Player/BP_Player` OtherActor)
  (`|ExecutionSequence`
    (:`then_0`
      ;[1 1 1] Fait apparaitre les FireSystem les uns après les autres
      (`SceneComponent.SetVisibility` _firesystem_2 true false :!label _label)
      (`PrimitiveComponent.SetCollisionEnabled` (`/Game/Blueprint/FinalRoom/BP_FireSystem.Box` _output_2) "QueryOnly")
      (`NiagaraComponent.ResetSystem` _firesystem_2)
      (`/Engine/EditorBlueprintResources/StandardMacros.IncrementInt` (`self.Incr1`)
        (:`  `
          (`KismetSystemLibrary.Delay` 0.1)
          (if (not (>= (`self.Incr1`) (/ (`KismetArrayLibrary.Array_LastIndex` _listfiresystem_2) 2)))
            (goto _label)))))
    (:`then_1`
      ;[1 1 1] Fait apparaitre les FireSystem les uns après les autres
      (set `self.Incr2` _returnvalue)
      (`SceneComponent.SetVisibility` _firesystem true false :!label _label_2)
      (`NiagaraComponent.ResetSystem` _firesystem)
      (`PrimitiveComponent.SetCollisionEnabled` (`/Game/Blueprint/FinalRoom/BP_FireSystem.Box` _output) "QueryOnly")
      (`/Engine/EditorBlueprintResources/StandardMacros.DecrementInt` (`self.Incr2`)
        (:`  `
          (`KismetSystemLibrary.Delay` 0.1)
          (if (not (< (`self.Incr2`) (/ _returnvalue 2)))
            (goto _label_2)))))))

(fn `UserConstructionScript`)