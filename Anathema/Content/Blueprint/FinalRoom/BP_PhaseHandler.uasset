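; BP_PhaseHandler sequences the phases of the final room, removing defenses around two chains and a wall.
; Leaving trigger component R destroys it and starts waiting for RefBloc to spawn.
; Timed delays then remove the first protection and both chains' invincibility, the second protection after the first chain breaks, and the wall after the second breaks.
; Each condition is polled with a looping Delay rather than events.
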(event `self.r.OnComponentEndOverlap`
  (params (OverlappedComponent :type "PrimitiveComponent Object Reference") (OtherActor :type "Actor Object Reference") (OtherComp :type "PrimitiveComponent Object Reference") (OtherBodyIndex :type Integer))
  (`/Engine/EditorBlueprintResources/StandardMacros.IsValid` (`self.r`)
    (:`Is Valid`
      (`ActorComponent.K2_DestroyComponent` (`self.r`))
      (if (`/Game/Blueprint/FinalRoom/BP_SpawnBloc.BlocHasSpawned` (`self.RefBloc`)) :!label _label
        (`KismetSystemLibrary.Delay` (`self.FirstChainInvicibilityTime`))
        (`self.K2_DestroyActor` (`self.ChainProtectionToDestroyFirst`))
        (set `/Game/Blueprint/Component/Actor/BP_AC_LivingActor.Invincible?` false (`self.GetComponentByClass` (`self.RefChainDestroyedFirst`) "/Game/Blueprint/Component/Actor/BP_AC_LivingActor.BP_AC_LivingActor_C"))
        (set `/Game/Blueprint/Component/Actor/BP_AC_LivingActor.Invincible?` false (`self.GetComponentByClass` (`self.RefSecondeChainDestroyed`) "/Game/Blueprint/Component/Actor/BP_AC_LivingActor.BP_AC_LivingActor_C"))
        (if (`/Game/Blueprint/Objets/BP_Chaine.IsChainDestroyed?` (`self.RefChainDestroyedFirst`)) :!label _label_2
          (`KismetSystemLibrary.Delay` (`self.SecondChainInvicibilityTime`))
          (`self.K2_DestroyActor` (`self.ChainProtectionToDestroySecond`))
          (if (`/Game/Blueprint/Objets/BP_Chaine.IsChainDestroyed?` (`self.RefSecondeChainDestroyed`)) :!label _label_3
            (`KismetSystemLibrary.Delay` (`self.WallInvicibilityTime`))
            (`self.K2_DestroyActor` (`self.RefWall`))
            (else
              (`KismetSystemLibrary.Delay` 0.2)
              (goto _label_3)))
          (else
            (`KismetSystemLibrary.Delay` 0.2)
            (goto _label_2)))
        (else
          (`KismetSystemLibrary.Delay` 0.2)
          (goto _label))))))

(fn `UserConstructionScript`)