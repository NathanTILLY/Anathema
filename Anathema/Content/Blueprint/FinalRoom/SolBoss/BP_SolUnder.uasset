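; BP_SolUnder is an actor tied to a BP_Sol in the final boss room that plays destruction effects and hurts the player.
; Tick watches the referenced BP_Sol's Destroyed flag, then after a delay spawns staggered building-destruction emitters at five LocationExplosion actors.
; That chain has no one-shot guard, so it keeps retriggering while the flag holds.
; Separately, the first player overlap with its Box briefly stuns and damages the player, gated by DoOnce.
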(event `self.ReceiveBeginPlay`
  (set `self.As BP Player` (cast `/Game/Blueprint/Player/BP_Player` (`GameplayStatics.GetPlayerPawn` 0) :!pure true)))

(event `self.ReceiveTick`
  (params (DeltaSeconds :type "Float (single-precision)"))
  (bind _refbpsol (`self.RefBpSol`))
  (`/Engine/EditorBlueprintResources/StandardMacros.IsValid` _refbpsol
    (:`Is Valid`
      (if (`/Game/Blueprint/FinalRoom/SolBoss/BP_sol.Destroyed` _refbpsol)
        (`KismetSystemLibrary.Delay` 2.0)
        (`GameplayStatics.SpawnEmitterAtLocation` "/Game/VFX/Particles/Destruction/P_Destruction_Building_A.P_Destruction_Building_A" (`self.K2_GetActorLocation` (`|GetArrayItem` (`self.LocationExplosion`))) (struct :`Pitch` 90.0) (20.0 20.0 20.0))
        (`KismetSystemLibrary.Delay` 0.1)
        (`GameplayStatics.SpawnEmitterAtLocation` "/Game/VFX/Particles/Destruction/P_Destruction_Building_A.P_Destruction_Building_A" (`self.K2_GetActorLocation` (`|GetArrayItem` (`self.LocationExplosion`) 1)) (struct :`Pitch` 90.0) (20.0 20.0 20.0))
        (`KismetSystemLibrary.Delay` 0.1)
        (`GameplayStatics.SpawnEmitterAtLocation` "/Game/VFX/Particles/Destruction/P_Destruction_Building_A.P_Destruction_Building_A" (`self.K2_GetActorLocation` (`|GetArrayItem` (`self.LocationExplosion`) 2)) (struct :`Pitch` 90.0) (20.0 20.0 20.0))
        (`KismetSystemLibrary.Delay` 0.1)
        (`GameplayStatics.SpawnEmitterAtLocation` "/Game/VFX/Particles/Destruction/P_Destruction_Building_A.P_Destruction_Building_A" (`self.K2_GetActorLocation` (`|GetArrayItem` (`self.LocationExplosion`) 3)) (struct :`Pitch` 90.0) (20.0 20.0 20.0))
        (`KismetSystemLibrary.Delay` 0.1)
        (`GameplayStatics.SpawnEmitterAtLocation` "/Game/VFX/Particles/Destruction/P_Destruction_Building_A.P_Destruction_Building_A" (`self.K2_GetActorLocation` (`|GetArrayItem` (`self.LocationExplosion`) 4)) (struct :`Pitch` 90.0) (20.0 20.0 20.0))))))

(event `self.Box.OnComponentBeginOverlap`
  (params (OverlappedComponent :type "PrimitiveComponent Object Reference") (OtherActor :type "Actor Object Reference") (OtherComp :type "PrimitiveComponent Object Reference") (OtherBodyIndex :type Integer) (bFromSweep :type Boolean) (SweepResult :type "HitResult Structure (by ref)"))
  (bind _as_bp_player (`self.As BP Player`))
  (cast `/Game/Blueprint/Player/BP_Player` OtherActor)
  (`/Engine/EditorBlueprintResources/StandardMacros.DoOnce` false
    (:`Completed`
      (`/Game/Blueprint/Player/BP_Player.Stun` _as_bp_player 0.5)
      (`/Game/Blueprint/Component/Actor/BP_AC_LivingActor.TakeDamage` (`/Game/Blueprint/Player/BP_Player.BP_AC_LivingActor` _as_bp_player) 5.0 null "NewEnumerator0"))))

(fn `UserConstructionScript`)