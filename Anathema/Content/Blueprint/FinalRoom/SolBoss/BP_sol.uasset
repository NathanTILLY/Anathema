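; BP_sol is a destructible floor piece in the final boss room that breaks under too much load and triggers a spawn.
; A sphere overlap counts AI and players; exceeding the threshold removes the walkable component and shatters the destructible with physics and damage.
; It notifies the game instance, then after a delay fades the debris through a dynamic material timeline before destroying itself.
; Alongside the fade, it calls Spawning on the referenced Septus spawner.
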(event `self.ReceiveBeginPlay`
  (bind _returnvalue (`PrimitiveComponent.CreateDynamicMaterialInstance` (`self.DestructibleSol1`) 0 null "None")))

(event `self.Sphere.OnComponentBeginOverlap`
  (params (OverlappedComponent :type "PrimitiveComponent Object Reference") (OtherActor :type "Actor Object Reference") (OtherComp :type "PrimitiveComponent Object Reference") (OtherBodyIndex :type Integer) (bFromSweep :type Boolean) (SweepResult :type "HitResult Structure (by ref)"))
  (bind _walkable1 (`self.Walkable1`))
  (bind _destructiblesol1 (`self.DestructibleSol1`))
  (`|ExecutionSequence`
    (:`then_0`
      (cast `/Game/Blueprint/Enemies/BP_AIParent` OtherActor))
    (:`then_1`
      (cast `/Game/Blueprint/Player/BP_Player` OtherActor)))
  (`/Engine/EditorBlueprintResources/StandardMacros.IncrementInt` (`self.Compteur1`)
    (:`  `
      (if (> (`self.Compteur1`) (`self.NumberToDestroy`))
        (`/Engine/EditorBlueprintResources/StandardMacros.IsValid` _walkable1
          (:`Is Valid`
            (`ActorComponent.K2_DestroyComponent` _walkable1)
            (`PrimitiveComponent.SetSimulatePhysics` _destructiblesol1 true)
            (`DestructibleComponent.ApplyDamage` _destructiblesol1 10000.0 (`SceneComponent.K2_GetComponentLocation` _destructiblesol1) (* (`SceneComponent.GetForwardVector` _destructiblesol1) 2000.0) 100.0)
            (set `self.Destroyed` true)
            (`/Game/Blueprint/BP_GameInstance.PropertyDestroyed` (cast `/Game/Blueprint/BP_GameInstance` (`GameplayStatics.GetGameInstance`) :!pure true))
            (`KismetSystemLibrary.Delay` 2.5)
            (`|ExecutionSequence`
              (:`then_0`
                (`/Engine/EditorBlueprintResources/StandardMacros.FlipFlop`
                  (:`A`
                    (bind (_direction _value) (`Timeline|Timeline_0` :!via `PlayFromStart` :!label _label)
                      (:`Update`
                        (`MaterialInstanceDynamic.SetScalarParameterValue` (stale `self.ReceiveBeginPlay` _returnvalue) "Fade" (`KismetMathLibrary.Lerp` 1.0 0.0 _value)))
                      (:`Finished`
                        (`self.K2_DestroyActor`))))
                  (:`B`
                    (goto _label :!via `ReverseFromEnd`))))
              (:`then_1`
                (`KismetSystemLibrary.Delay` 1.0)
                (`/Game/Blueprint/Objets/SolBoss/BP_SpawnSeptus.Spawning` (`self.RefSpawnSeptus`))
                (`KismetSystemLibrary.PrintString` "sol a spawning")))))))))

(event `self.Sphere.OnComponentEndOverlap`
  (params (OverlappedComponent :type "PrimitiveComponent Object Reference") (OtherActor :type "Actor Object Reference") (OtherComp :type "PrimitiveComponent Object Reference") (OtherBodyIndex :type Integer))
  (`|ExecutionSequence`
    (:`then_0`
      (cast `/Game/Blueprint/Enemies/BP_AIParent` OtherActor))
    (:`then_1`
      (cast `/Game/Blueprint/Player/BP_Player` OtherActor)))
  (`/Engine/EditorBlueprintResources/StandardMacros.DecrementInt` (`self.Compteur1`)))

(fn `UserConstructionScript`)