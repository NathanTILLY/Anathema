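; BP_ExplosionBoss is a short-lived expanding explosion actor, apparently for the final room boss, that damages the player it engulfs.
; On BeginPlay a timeline scales the Sphere component up to a hundred times unit scale, then destroys the actor.
; The sphere's begin overlap casts to BP_Player and uses a DoOnce to apply fixed damage through its BPACLivingActor component only once, with a debug print.
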(event `self.ReceiveBeginPlay`
  (bind (_direction _newtrack_0) (`Timeline|Timeline_0`)
    (:`Update`
      (bind _returnvalue (`KismetMathLibrary.Lerp` 1.0 100.0 _newtrack_0))
      (`SceneComponent.SetRelativeScale3D` (`self.Sphere`) (`KismetMathLibrary.MakeVector` _returnvalue _returnvalue _returnvalue)))
    (:`Finished`
      (`self.K2_DestroyActor`))))

(event `self.Sphere.OnComponentBeginOverlap`
  (params (OverlappedComponent :type "PrimitiveComponent Object Reference") (OtherActor :type "Actor Object Reference") (OtherComp :type "PrimitiveComponent Object Reference") (OtherBodyIndex :type Integer) (bFromSweep :type Boolean) (SweepResult :type "HitResult Structure (by ref)"))
  (bind _asbp_player (cast `/Game/Blueprint/Player/BP_Player` OtherActor))
  (`/Engine/EditorBlueprintResources/StandardMacros.DoOnce` false
    (:`Completed`
      (`/Game/Blueprint/Component/Actor/BP_AC_LivingActor.TakeDamage` (`/Game/Blueprint/Player/BP_Player.BP_AC_LivingActor` _asbp_player) 20.0 null "NewEnumerator0")
      (`KismetSystemLibrary.PrintString` "gothit"))))

(fn `UserConstructionScript`)