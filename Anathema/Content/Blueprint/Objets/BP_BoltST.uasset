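; Bolt pickup for the ballista that triggers a minion ambush when collected, usable once RefCanDestroyGate is activated.
; Box overlap shows and hides an interact widget; Interact sets HasBolt on RefBalista and removes the bolt.
; It then spawns an encirclement actor and random, scale-varied AI at preset points, clearing the encirclement after a delay.
; If both cogs are also held, it later shows an all-parts message and destroys itself.
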(event `self.Box.OnComponentBeginOverlap`
  (params (OverlappedComponent :type "PrimitiveComponent Object Reference") (OtherActor :type "Actor Object Reference") (OtherComp :type "PrimitiveComponent Object Reference") (OtherBodyIndex :type Integer) (bFromSweep :type Boolean) (SweepResult :type "HitResult Structure (by ref)"))
  (if (`/Game/Blueprint/UI/Subtitles/BP_CanDestroyGateST.HasBeenActivated` (`self.RefCanDestroyGate`))
    (`/Engine/EditorBlueprintResources/StandardMacros.DoOnce` false :!label _label
      (:`Completed`
        (cast `/Game/Blueprint/Player/BP_Player` OtherActor)
        (bind _returnvalue (`|CreateWidget` "/Game/Blueprint/UI/WBP_Interact.WBP_Interact_C"))
        (`KismetSystemLibrary.Delay` 0.002)
        (bind _output_get (set `self.RefInteract` _returnvalue))
        (`UserWidget.AddToViewport` _output_get 0)))))

(event `self.Box.OnComponentEndOverlap`
  (params (OverlappedComponent :type "PrimitiveComponent Object Reference") (OtherActor :type "Actor Object Reference") (OtherComp :type "PrimitiveComponent Object Reference") (OtherBodyIndex :type Integer))
  (bind _refinteract (`self.RefInteract`))
  (if (`/Game/Blueprint/UI/Subtitles/BP_CanDestroyGateST.HasBeenActivated` (`self.RefCanDestroyGate`))
    (cast `/Game/Blueprint/Player/BP_Player` OtherActor)
    (`/Engine/EditorBlueprintResources/StandardMacros.IsValid` _refinteract
      (:`Is Valid`
        (`Widget.RemoveFromParent` _refinteract)
        (goto _label :!via `Reset`)))))

(event `self.ReceiveBeginPlay`
  (`KismetSystemLibrary.Delay` 0.1)
  (bind _asbp_player (cast `/Game/Blueprint/Player/BP_Player` (`GameplayStatics.GetPlayerPawn` 0)))
  (set `self.As BP Player` _asbp_player))

(event `/Game/Blueprint/Interface/BPI_Interact.Interact`
  (params (Player :type "Character Object Reference"))
  (bind _refbalista (`self.RefBalista`))
  (bind _spawnlocation (`self.SpawnLocation`))
  (bind _mobaspawn (`self.MobASpawn`))
  (bind _rootcomponent (`Actor.RootComponent` (`|GetArrayItem` _spawnlocation (`KismetMathLibrary.RandomInteger` (`KismetArrayLibrary.Array_Length` _spawnlocation)))))
  (if (`/Game/Blueprint/UI/Subtitles/BP_CanDestroyGateST.HasBeenActivated` (`self.RefCanDestroyGate`))
    (`|ExecutionSequence`
      (:`then_0`
        (set `/Game/Blueprint/Objets/BP_Balista.HasBolt?` true (`self.RefBalista`)))
      (:`then_1`
        (`ActorComponent.K2_DestroyComponent` (`self.Bolt`))
        (`ActorComponent.K2_DestroyComponent` (`self.Box`))
        (bind _returnvalue (`|CreateWidget` "/Game/Blueprint/UI/Subtitles/WBP_MinnionsKillHim.WBP_MinnionsKillHim_C"))
        (`UserWidget.AddToViewport` _returnvalue 0)
        (bind _returnvalue_2 (`|SpawnActorFromClass` "/Game/Blueprint/Objets/BP_EncirclementST.BP_EncirclementST_C" (`KismetMathLibrary.MakeTransform` (-4864.0 -1044.0 752.0) (struct :`Yaw` -90.0) (13.0 13.0 13.0)) "Undefined" "OverrideRootScale" null null))
        (if (< (`self.NbrDejaSpawn`) (`self.NbrDeSpawn`)) :!label _label_2
          (`/Engine/EditorBlueprintResources/StandardMacros.IncrementInt` (`self.NbrDejaSpawn`)
            (:`  `
              (bind _returnvalue_3 (`AIBlueprintHelperLibrary.SpawnAIFromClass` (`|GetArrayItem` _mobaspawn (`KismetMathLibrary.RandomIntegerInRange` 0 (`KismetArrayLibrary.Array_LastIndex` _mobaspawn))) null (`SceneComponent.K2_GetComponentLocation` _rootcomponent) (`SceneComponent.K2_GetComponentRotation` _rootcomponent) false null))
              (`/Engine/EditorBlueprintResources/StandardMacros.IsValid` _returnvalue_3
                (:`Is Valid`
                  (bind _output_get (set `self.CurrentScale` (`KismetMathLibrary.RandomFloatInRange` 0.9 1.1)))
                  (`self.SetActorScale3D` _returnvalue_3 (`KismetMathLibrary.MakeVector` _output_get _output_get _output_get))
                  (goto _label_2))
                (:`Is Not Valid`
                  (goto _label_2)))))
          (else
            (`KismetSystemLibrary.Delay` 30.0)
            (`self.K2_DestroyActor` null)
            (`self.K2_DestroyActor` _returnvalue_2)
            (`self.K2_DestroyActor` null)
            (`self.K2_DestroyActor` null)
            (`Widget.RemoveFromParent` _returnvalue))))
      (:`then_2`
        (if (`/Game/Blueprint/Objets/BP_Balista.HasCog1?` _refbalista)
          (if (`/Game/Blueprint/Objets/BP_Balista.HasCog2?` _refbalista)
            (if (`/Game/Blueprint/Objets/BP_Balista.HasBolt?` _refbalista)
              (`KismetSystemLibrary.Delay` 30.0)
              (bind _returnvalue_4 (`|CreateWidget` "/Game/Blueprint/UI/Subtitles/WBP_HaveAllParts.WBP_HaveAllParts_C"))
              (`UserWidget.AddToViewport` _returnvalue_4 0)
              (`KismetSystemLibrary.Delay` 10.0)
              (`Widget.RemoveFromParent` _returnvalue_4)
              (`self.K2_DestroyActor`))))))))

(event `self.ReceiveDestroyed`
  (set `/Game/Blueprint/Objets/BP_Balista.HasBolt?` true (`self.RefBalista`)))

(fn `UserConstructionScript`)