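; BP_HealTotem is a single-use interactable totem that heals the player who interacts with it.
; On first interaction it spawns two particle effects, plays a heal sound at the world origin and calls Heal on the player's BP_AC_LivingActor component with HealValue.
; It destroys two static meshes immediately, then after a two-second delay hides the particles and destroys its spotlight.
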(event `/Game/Blueprint/Interface/BPI_Interact.Interact`
  (params (Player :type "Character Object Reference"))
  (bind _returnvalue (`self.K2_GetActorLocation`))
  (`/Engine/EditorBlueprintResources/StandardMacros.DoOnce` false
    (:`Completed`
      (`|ExecutionSequence`
        (:`then_0`
          (bind _returnvalue_2 (`GameplayStatics.SpawnEmitterAtLocation` "/Game/VFX/AuraEffect/PS_AuraCircle.PS_AuraCircle" _returnvalue))
          (`KismetSystemLibrary.Delay` 2.0 :!label _label)
          (`SceneComponent.SetVisibility` _returnvalue_2 false false)
          (`SceneComponent.SetVisibility` (stale _returnvalue_3) false false)
          (`ActorComponent.K2_DestroyComponent` (`self.SpotLight`)))
        (:`then_1`
          (bind _returnvalue_3 (`GameplayStatics.SpawnEmitterAtLocation` "/Game/VFX/AuraEffect/PS_7emeciel.PS_7emeciel" _returnvalue))
          (goto _label))
        (:`then_2`
          (`GameplayStatics.PlaySoundAtLocation` "/Game/Audio/Sound/heal.heal" (0.0 0.0 0.0) (struct) 1.0 1.0 0.0 null null null)
          (`/Game/Blueprint/Component/Actor/BP_AC_LivingActor.Heal` (`self.GetComponentByClass` Player "/Game/Blueprint/Component/Actor/BP_AC_LivingActor.BP_AC_LivingActor_C") (`self.HealValue`))
          (`ActorComponent.K2_DestroyComponent` (`self.StaticMesh1`))
          (`ActorComponent.K2_DestroyComponent` (`self.StaticMesh2`)))))))

(fn `UserConstructionScript`)