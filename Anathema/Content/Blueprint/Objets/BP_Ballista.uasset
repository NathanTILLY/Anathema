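; Interactable ballista that the player repairs with a bolt and two cogs, then fires once.
; Interact branches on CurrentState: Broken shows a missing-parts widget or swaps to repaired meshes behind a black screen.
; Repaired plays the firing animation, spawns BP_BoltProjectile from the arrow and becomes HasShot.
; OnSpawn restores visuals for a given state, and ShowInteractWidget hides the prompt after firing.
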(event `/Game/Blueprint/Interface/BPI_Interact.Interact`
  (params (Player :type "Character Object Reference"))
  (bind _arrow (`self.Arrow`))
  ;[1 1 1] Player Interact with the actor
  (bind _asbp_player (cast `/Game/Blueprint/Player/BP_Player` Player))
  (set `self.PlayerRef` _asbp_player)
  (`|ExecutionSequence`
    (:`then_0`
      ;[1 1 1] Shoot the bolt when the balista is repaired and the player interact with it
      (if (`|EnumEquality` (`self.CurrentState`) "NewEnumerator1")
        (`/Engine/EditorBlueprintResources/StandardMacros.DoOnce` false
          (:`Completed`
            (`|ExecutionSequence`
              (:`then_0`
                (`SkeletalMeshComponent.PlayAnimation` (`self.RepairedBalista`) "/Game/Meshes/Baliste/BallisteRepairedBody_Anim.BallisteRepairedBody_Anim" false)
                (`KismetSystemLibrary.Delay` 0.3)
                (`|SpawnActorFromClass` "/Game/Blueprint/Objets/BP_BoltProjectile.BP_BoltProjectile_C" (`KismetMathLibrary.MakeTransform` (+ (+ (`SceneComponent.K2_GetComponentLocation` _arrow) (0.0 0.0 -10.0)) (* (`SceneComponent.GetForwardVector` _arrow) 50.0)) (`SceneComponent.K2_GetComponentRotation` _arrow)) "Undefined" "OverrideRootScale" null null)
                (`ActorComponent.K2_DestroyComponent` (`self.Bolt`))
                (`ActorComponent.K2_DestroyComponent` (`self.Box`))
                (set `self.CurrentState` "NewEnumerator2"))
              (:`then_1`
                (`GameplayStatics.PlaySoundAtLocation` "/Game/Audio/Sound2_0/SoundUseCue/BalisteShoot.BalisteShoot" (0.0 0.0 0.0) (struct) 1.0 1.0 0.0 null null null)))))))
    (:`then_1`
      (if (`|EnumEquality` (`self.CurrentState`) "NewEnumerator0")
        ;[1 1 1] Repair the Ballista
        (if (and (`self.HasBolt?`) (`self.HasCog1?`) (`self.HasCog2?`))
          (`/Engine/EditorBlueprintResources/StandardMacros.DoOnce` false
            (:`Completed`
              (`|ExecutionSequence`
                (:`then_0`
                  (bind _returnvalue (`|CreateWidget` "/Game/Blueprint/UI/WBP_BlackScreen.WBP_BlackScreen_C"))
                  (`UserWidget.AddToViewport` _returnvalue 0)
                  (`KismetSystemLibrary.Delay` 0.1)
                  (`SceneComponent.SetVisibility` (`self.RepairedBalista`) true false)
                  (`SceneComponent.SetVisibility` (`self.BaseRepaired`) true false)
                  (`SceneComponent.SetVisibility` (`self.Bolt`) true false)
                  (`ActorComponent.K2_DestroyComponent` (`self.BrokenBalista`))
                  (set `self.CurrentState` "NewEnumerator1")
                  (`KismetSystemLibrary.Delay` 2.5)
                  (`Widget.RemoveFromParent` _returnvalue)
                  (if (`self.SubtitleMode`)
                    (bind _returnvalue_2 (`|CreateWidget` "/Game/Blueprint/UI/Subtitles/WBP_FireBalista.WBP_FireBalista_C"))
                    (`UserWidget.AddToViewport` _returnvalue_2 0)))
                (:`then_1`
                  (`GameplayStatics.PlaySoundAtLocation` "/Game/Audio/Sound2_0/SoundUseCue/BalisteCharge.BalisteCharge" (0.0 0.0 0.0) (struct) 1.0 1.0 0.0 null null null)))))
          (else
            ;[1 1 1] Missing some part to repair
            (bind _returnvalue_3 (`|CreateWidget` "/Game/Blueprint/UI/WBP_MissingParts.WBP_MissingParts_C"))
            (`UserWidget.AddToViewport` _returnvalue_3 0)
            (`KismetSystemLibrary.Delay` 2.5)
            (`Widget.RemoveFromParent` _returnvalue_3)))))))

(fn `OnSpawn`
  (params (NewState :type "/Game/Blueprint/Enum/E_BallistaState Enum" :default "NewEnumerator0"))
  (bind _output_get (set `self.CurrentState` NewState))
  (switch `/Game/Blueprint/Enum/E_BallistaState` _output_get
    (:`NewEnumerator1`
      (`SceneComponent.SetVisibility` (`self.RepairedBalista`) true false)
      (`SceneComponent.SetVisibility` (`self.BaseRepaired`) true false)
      (`SceneComponent.SetVisibility` (`self.Bolt`) true false)
      (`ActorComponent.K2_DestroyComponent` (`self.BrokenBalista`)))
    (:`NewEnumerator2`
      (`SceneComponent.SetVisibility` (`self.RepairedBalista`) true false)
      (`SceneComponent.SetVisibility` (`self.BaseRepaired`) true false)
      (`ActorComponent.K2_DestroyComponent` (`self.BrokenBalista`)))))

(fn `ShowInteractWidget`
  (returns (`Show?` :type Boolean))
  (if (`|EnumEquality` (`self.CurrentState`) "NewEnumerator2")
    (return false)
    (else
      (return true))))

(fn `UserConstructionScript`)