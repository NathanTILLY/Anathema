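; BP_Spawner is a trigger that spawns a group of AI mobs when BP_Player enters its Box.
; Each mob is a random class from MobASpawn, placed at a random point inside the SpawnLocation actor's bounds and slightly randomized in scale.
; A short Delay loop staggers spawns until NbrSpawn reaches NbrASpawn, stopping early if one fails.
; The counter never resets, so re-entry after completion still spawns one more.
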(event `self.Box.OnComponentBeginOverlap`
  (params (OverlappedComponent :type "PrimitiveComponent Object Reference") (OtherActor :type "Actor Object Reference") (OtherComp :type "PrimitiveComponent Object Reference") (OtherBodyIndex :type Integer) (bFromSweep :type Boolean) (SweepResult :type "HitResult Structure (by ref)"))
  (bind _mobaspawn (`self.MobASpawn`))
  (bind _spawnlocation (`self.SpawnLocation`))
  (bind (_origin _boxextent) (`self.GetActorBounds` _spawnlocation false false))
  (cast `/Game/Blueprint/Player/BP_Player` OtherActor)
  (`KismetSystemLibrary.Delay` 0.016 :!label _label)
  (`/Engine/EditorBlueprintResources/StandardMacros.IncrementInt` (`self.NbrSpawn`)
    (:`  `
      (bind _returnvalue (`AIBlueprintHelperLibrary.SpawnAIFromClass` (`|GetArrayItem` _mobaspawn (`KismetMathLibrary.RandomIntegerInRange` 0 (`KismetArrayLibrary.Array_LastIndex` _mobaspawn))) null (+ _origin (`KismetMathLibrary.MakeVector` (`KismetMathLibrary.RandomFloatInRange` (* (.x _boxextent) -1.0) (.x _boxextent)) (`KismetMathLibrary.RandomFloatInRange` (* (.y _boxextent) -1.0) (.y _boxextent)) (`KismetMathLibrary.RandomFloatInRange` (* (.z _boxextent) -1.0) (.z _boxextent)))) (`SceneComponent.K2_GetComponentRotation` (`Actor.RootComponent` _spawnlocation)) false null))
      (`/Engine/EditorBlueprintResources/StandardMacros.IsValid` _returnvalue
        (:`Is Valid`
          (bind _output_get (set `self.CurrentScale` (`KismetMathLibrary.RandomFloatInRange` 0.9 1.1)))
          (`self.SetActorScale3D` _returnvalue (`KismetMathLibrary.MakeVector` _output_get _output_get _output_get))
          (if (< (`self.NbrSpawn`) (`self.NbrASpawn`))
            (goto _label)))))))

(fn `UserConstructionScript`)