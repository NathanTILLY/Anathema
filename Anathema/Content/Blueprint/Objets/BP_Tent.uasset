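; BP_Tent is a destructible tent that breaks apart and disappears when its BP_AC_LivingActor component signals death.
; On death, the DestructibleComponent simulates physics and takes heavy damage with a forward impulse; fracturing switches its collision to physics only.
; After a short delay, a FlipFlop starts the Fader timeline, which lowers the Fade parameter on a dynamic material instance before destroying the actor.
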(event `self.ReceiveBeginPlay`
  (bind _returnvalue (`PrimitiveComponent.CreateDynamicMaterialInstance` (`self.DestructibleComponent`) 0 null "None")))

(event `self.BP_AC_LivingActor.OnDeath`
  (params (AttackOwner :type "Actor Object Reference"))
  (bind _destructiblecomponent (`self.DestructibleComponent`))
  (`PrimitiveComponent.SetSimulatePhysics` _destructiblecomponent true)
  (`DestructibleComponent.ApplyDamage` _destructiblecomponent 1000.0 (`SceneComponent.K2_GetComponentLocation` _destructiblecomponent) (* (`SceneComponent.GetForwardVector` _destructiblecomponent) 1000.0) 5000.0)
  (`KismetSystemLibrary.Delay` 2.0)
  (`/Engine/EditorBlueprintResources/StandardMacros.FlipFlop`
    (:`A`
      (bind (_direction _value) (`Timeline|fader` :!via `PlayFromStart` :!label _label)
        (:`Update`
          (`MaterialInstanceDynamic.SetScalarParameterValue` (stale `self.ReceiveBeginPlay` _returnvalue) "Fade" (`KismetMathLibrary.Lerp` 1.0 0.0 _value)))
        (:`Finished`
          (`self.K2_DestroyActor`))))
    (:`B`
      (goto _label :!via `ReverseFromEnd`))))

(event `self.DestructibleComponent.OnComponentFracture`
  (params (HitPoint :type "Vector Structure (by ref)") (HitDirection :type "Vector Structure (by ref)"))
  (`PrimitiveComponent.SetCollisionEnabled` (`self.DestructibleComponent`) "PhysicsOnly"))

(fn `UserConstructionScript`)