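; Destructible curtain (BP_TentCurtainST) that breaks apart once the actors in its ListTent array are destroyed.
; BeginPlay binds each listed actor's OnDestroyed event and caches the player pawn, which is not used afterwards.
; Each destruction removes that actor by name, then treats an empty display name after looping the remainder as list empty.
; The DestructibleComponent then simulates physics, takes damage with a forward impulse, and is destroyed shortly after.
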(event `self.ReceiveBeginPlay`
  (`|ExecutionSequence`
    (:`then_0`
      (`KismetSystemLibrary.Delay` 0.1)
      (bind _asbp_player (cast `/Game/Blueprint/Player/BP_Player` (`GameplayStatics.GetPlayerPawn` 0)))
      (set `self.As BP Player` _asbp_player))
    (:`then_1`
      (for _array_element (`self.ListTent`)
        (add `Actor.OnDestroyed` _array_element (delegate `CustomEvent_0`))))))

(event `CustomEvent_0`
  (params (DestroyedActor :type "Actor Object Reference"))
  (bind _destructiblecomponent (`self.DestructibleComponent`))
  (for (_array_element _array_index) (`self.ListTent`)
    (if (`KismetStringLibrary.EqualEqual_StrStr` (`KismetSystemLibrary.GetObjectName` _array_element) (`KismetSystemLibrary.GetObjectName` DestroyedActor))
      (`KismetArrayLibrary.Array_Remove` (`self.ListTent`) _array_index)
      (for _array_element_2 (`self.ListTent`)
        _)
      (if (`KismetStringLibrary.IsEmpty` (`KismetSystemLibrary.GetDisplayName` _array_element_2))
        (`PrimitiveComponent.SetSimulatePhysics` _destructiblecomponent true)
        (`DestructibleComponent.ApplyDamage` _destructiblecomponent 1000.0 (`SceneComponent.K2_GetComponentLocation` _destructiblecomponent) (* (`SceneComponent.GetForwardVector` _destructiblecomponent) 1000.0) 10.0)
        (`KismetSystemLibrary.Delay` 1.0)
        (`ActorComponent.K2_DestroyComponent` (`self.DestructibleComponent`))))))

(event `self.ReceiveTick`
  (params (DeltaSeconds :type "Float (single-precision)")))

(fn `UserConstructionScript`)