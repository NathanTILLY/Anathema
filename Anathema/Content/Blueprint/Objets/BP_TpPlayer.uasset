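; BP_TpPlayer is an interactable object that teleports the player to TPPoint, once only.
; After a short delay, Interact makes the player invincible through BP_AC_LivingActor and shows a timed WBP_BlackScreen.
; When the screen time elapses, it moves the player's capsule and destroys every BP_Griveton.
; It then restores vulnerability, reapplies the location with TPPoint's rotation, and destroys the BPSpawnerEgouts actors.
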(event `self.ReceiveBeginPlay`
  (set `self.Ref Game State` (cast `/Game/Blueprint/Player/BP_GS_Gameplay` (`GameplayStatics.GetGameState`) :!pure true))
  (set `self.RefGameMode` (cast `/Game/Blueprint/Player/BP_FPS_NewPlayer` (`GameplayStatics.GetGameMode`) :!pure true)))

(event `/Game/Blueprint/Interface/BPI_Interact.Interact`
  (params (Player :type "Character Object Reference"))
  (bind _capsulecomponent (`Character.CapsuleComponent` Player))
  (bind _tppoint (`self.TPPoint`))
  (`KismetSystemLibrary.Delay` 0.5)
  (`/Engine/EditorBlueprintResources/StandardMacros.DoOnce` false
    (:`Completed`
      (set `/Game/Blueprint/Component/Actor/BP_AC_LivingActor.Invincible?` true (`self.GetComponentByClass` Player "/Game/Blueprint/Component/Actor/BP_AC_LivingActor.BP_AC_LivingActor_C"))
      (bind _returnvalue (`|CreateWidget` "/Game/Blueprint/UI/WBP_BlackScreen.WBP_BlackScreen_C"))
      (set `/Game/Blueprint/UI/WBP_BlackScreen.Temps` (`self.BlackScreenTime`) _returnvalue)
      (`UserWidget.AddToViewport` _returnvalue 0)
      (`KismetSystemLibrary.Delay` (`self.BlackScreenTime`))
      (`SceneComponent.K2_SetRelativeLocation` _capsulecomponent (`self.K2_GetActorLocation` (`self.TPPoint`)) false true)
      (bind _outactors (`GameplayStatics.GetAllActorsOfClass` "/Game/Blueprint/Enemies/Grivetons/Griveton/BP_Griveton.BP_Griveton_C"))
      (for _array_element _outactors
        (`self.K2_DestroyActor` _array_element))
      (`KismetSystemLibrary.Delay` 0.5)
      (set `/Game/Blueprint/Component/Actor/BP_AC_LivingActor.Invincible?` false (`self.GetComponentByClass` Player "/Game/Blueprint/Component/Actor/BP_AC_LivingActor.BP_AC_LivingActor_C"))
      (`SceneComponent.K2_SetRelativeLocation` _capsulecomponent (`self.K2_GetActorLocation` _tppoint) false true)
      (`SceneComponent.K2_SetRelativeRotation` _capsulecomponent (`self.K2_GetActorRotation` _tppoint) false false)
      (for _array_element_2 (`self.BP_spawnerEgouts`)
        (`self.K2_DestroyActor` _array_element_2)))))

(event `self.Box.OnComponentBeginOverlap`
  (params (OverlappedComponent :type "PrimitiveComponent Object Reference") (OtherActor :type "Actor Object Reference") (OtherComp :type "PrimitiveComponent Object Reference") (OtherBodyIndex :type Integer) (bFromSweep :type Boolean) (SweepResult :type "HitResult Structure (by ref)")))

(fn `UserConstructionScript`
  (`parent.UserConstructionScript`))