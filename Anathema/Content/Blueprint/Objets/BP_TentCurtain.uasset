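; BP_TentCurtain is a destructible curtain that breaks apart once the tents linked to it are destroyed.
; On BeginPlay it binds to OnDestroyed of each actor in ListTent, then removes each destroyed tent by name match.
; An empty display name after looping the remaining list serves as the all-gone check.
; It then enables physics, applies a forward damage impulse, and removes the destructible component after a short delay.
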(event `self.ReceiveBeginPlay`
  (for _array_element (`self.ListTent`)
    (add `Actor.OnDestroyed` _array_element (delegate `TentDestroyed`))))

(event `TentDestroyed`
  (params (DestroyedActor :type "Actor Object Reference"))
  (bind _destructiblecomponent (`self.DestructibleComponent`))
  ;[1 1 1] Remove tent from the list
  (for (_array_element _array_index) (`self.ListTent`)
    (if (`KismetStringLibrary.EqualEqual_StrStr` (`KismetSystemLibrary.GetObjectName` _array_element) (`KismetSystemLibrary.GetObjectName` DestroyedActor))
      (`KismetArrayLibrary.Array_Remove` (`self.ListTent`) _array_index)
      (for _array_element_2 (`self.ListTent`)
        _)
      (if (`KismetStringLibrary.IsEmpty` (`KismetSystemLibrary.GetDisplayName` _array_element_2))
        (`PrimitiveComponent.SetSimulatePhysics` _destructiblecomponent true)
        (`DestructibleComponent.ApplyDamage` _destructiblecomponent 1000.0 (`SceneComponent.K2_GetComponentLocation` _destructiblecomponent) (* (`SceneComponent.GetForwardVector` _destructiblecomponent) 1000.0) 10.0)
        (`KismetSystemLibrary.Delay` 1.0)
        (`ActorComponent.K2_DestroyComponent` (`self.DestructibleComponent`))))))

(fn `UserConstructionScript`)