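; BP_Grille is a gate ("grille") that rises when its OpenGrille event is called.
; The construction script sets OpenPosition 600 units above the actor's location.
; OpenGrille plays a timeline that moves the static mesh toward that point each update through VInterpTo, using the timeline track as DeltaTime rather than the frame delta.
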(event `OpenGrille`
  (bind (_direction _newtrack_0) (`Timeline|Timeline_0`)
    (:`Update`
      (`SceneComponent.K2_SetWorldLocation` (`self.StaticMesh`) (`KismetMathLibrary.VInterpTo` (`SceneComponent.K2_GetComponentLocation` (`self.StaticMesh`)) (`self.OpenPosition`) _newtrack_0 0.1) false false))))

(fn `UserConstructionScript`
  (bind (_returnvalue_x _returnvalue_y _returnvalue_z) (`KismetMathLibrary.BreakVector` (`self.K2_GetActorLocation`)))
  (set `self.OpenPosition` (`KismetMathLibrary.MakeVector` _returnvalue_x _returnvalue_y (+ _returnvalue_z 600.0))))