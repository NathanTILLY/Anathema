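; BP_Balista is an interactable ballista that is completed from parts and then fires a bolt projectile.
; Once the bolt and both cog flags are set, the first Interact applies the part materials and a later one spawns BP_BoltProjectile from the Arrow component.
; Firing destroys the Bolt component and clears HasCog2.
; Any missing part, including right after firing, shows a temporary WBP_MissingParts widget.
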(event `/Game/Blueprint/Interface/BPI_Interact.Interact`
  (params (Player :type "Character Object Reference"))
  (bind _bolt (`self.Bolt`))
  (bind _arrow (`self.Arrow`))
  (`|ExecutionSequence`
    (:`then_0`
      (if (`self.HasBolt?`)
        (if (`self.HasCog1?`)
          (if (`self.HasCog2?`)
            (if (`self.PartsSpawned?`)
              (`|SpawnActorFromClass` "/Game/Blueprint/Objets/BP_BoltProjectile.BP_BoltProjectile_C" (`KismetMathLibrary.MakeTransform` (+ (+ (`SceneComponent.K2_GetComponentLocation` _arrow) (0.0 0.0 -10.0)) (* (`SceneComponent.GetForwardVector` _arrow) 50.0)) (`SceneComponent.K2_GetComponentRotation` _arrow)) "Undefined" "OverrideRootScale" null null)
              (`ActorComponent.K2_DestroyComponent` (`self.Bolt`))
              (set `self.HasCog2?` false))))))
    (:`then_1`
      (if (`self.HasBolt?`)
        (if (`self.HasCog1?`)
          (if (`self.HasCog2?`)
            (`PrimitiveComponent.SetMaterial` _bolt 0 "/Game/Meshes/Weapon/Crossbow/Crossbow_Textures/Crossbow_Wood.Crossbow_Wood")
            (`PrimitiveComponent.SetMaterial` _bolt 1 "/Game/Meshes/Weapon/Crossbow/Crossbow_Textures/Crossbow_Metal.Crossbow_Metal")
            (`PrimitiveComponent.SetMaterial` (`self.CogRight`) 0 "/Game/Meshes/Modular_Kit/Ville_Walls/Materials/Wood.Wood")
            (`PrimitiveComponent.SetMaterial` (`self.CogLeft`) 0 "/Game/Meshes/Modular_Kit/Ville_Walls/Materials/Wood.Wood")
            (set `self.PartsSpawned?` true)
            (else
              (bind _returnvalue (`|CreateWidget` "/Game/Blueprint/UI/WBP_MissingParts.WBP_MissingParts_C" :!label _label))
              (`UserWidget.AddToViewport` _returnvalue 0)
              (`KismetSystemLibrary.Delay` 2.5)
              (`Widget.RemoveFromParent` _returnvalue)))
          (else
            (goto _label)))
        (else
          (goto _label))))))

(fn `UserConstructionScript`)