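; BP_Bolt is an interactable bolt pickup that flags the referenced ballista as having its bolt and triggers a timed survival encounter.
; On Interact, it removes its mesh, shows the WBP_Survive widget, spawns BP_Encirclement at a hard-coded location and spawns a batch of AI mobs at randomly picked spawn points.
; After a fixed delay, it removes the encirclement and widget, then destroys itself.
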(event `/Game/Blueprint/Interface/BPI_Interact.Interact`
  (params (Player :type "Character Object Reference"))
  (bind _spawnlocation (`self.SpawnLocation`))
  (bind _rootcomponent (`Actor.RootComponent` (`|GetArrayItem` _spawnlocation (`KismetMathLibrary.RandomInteger` (`KismetArrayLibrary.Array_Length` _spawnlocation)))))
  (`|ExecutionSequence`
    (:`then_0`
      (set `/Game/Blueprint/Objets/BP_Balista.HasBolt?` true (`self.RefBalista`)))
    (:`then_1`
      (`ActorComponent.K2_DestroyComponent` (`self.StaticMesh`))
      (bind _returnvalue (`|CreateWidget` "/Game/Blueprint/UI/WBP_Survive.WBP_Survive_C"))
      (`UserWidget.AddToViewport` _returnvalue 0)
      (bind _returnvalue_2 (`|SpawnActorFromClass` "/Game/Blueprint/Objets/BP_Encirclement.BP_Encirclement_C" (`KismetMathLibrary.MakeTransform` (-4807.0 -915.0 999.0)) "Undefined" "OverrideRootScale" null null))
      (while (< (`self.NbrDejaSpawn`) (`self.NbrDeSpawn`))
        (`/Engine/EditorBlueprintResources/StandardMacros.IncrementInt` (`self.NbrDejaSpawn`)
          (:`  `
            (`AIBlueprintHelperLibrary.SpawnAIFromClass` (`self.MobASpawn`) null (`SceneComponent.K2_GetComponentLocation` _rootcomponent) (`SceneComponent.K2_GetComponentRotation` _rootcomponent) false null))))
      (`KismetSystemLibrary.Delay` 30.0)
      (`self.K2_DestroyActor` _returnvalue_2)
      (`Widget.RemoveFromParent` _returnvalue)
      (`self.K2_DestroyActor`))))

(fn `UserConstructionScript`)