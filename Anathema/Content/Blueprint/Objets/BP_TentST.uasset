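; BP_TentST is a destructible tent that stays effectively invulnerable until the referenced RefCanDestroy object has been activated.
; Tick checks that flag and, through DoOnce gates, sets the living-actor component's HP very high or low.
; On death, the destructible component simulates physics and shatters under applied damage, with fractures switching collision to physics-only.
; After a short delay, a timeline fades its dynamic material and destroys the actor.
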(event `self.ReceiveTick`
  (params (DeltaSeconds :type "Float (single-precision)"))
  (if (`/Game/Blueprint/UI/Subtitles/BP_CanDestroyGateST.HasBeenActivated` (`self.RefCanDestroy`))
    (`/Engine/EditorBlueprintResources/StandardMacros.DoOnce` false
      (:`Completed`
        (set `/Game/Blueprint/Component/Actor/BP_AC_LivingActor.CurrentHp` 5.0 (`self.BP_AC_LivingActor`))))
    (else
      (`/Engine/EditorBlueprintResources/StandardMacros.DoOnce` false
        (:`Completed`
          (set `/Game/Blueprint/Component/Actor/BP_AC_LivingActor.CurrentHp` 1000000.0 (`self.BP_AC_LivingActor`)))))))

(event `self.ReceiveBeginPlay`
  (`|ExecutionSequence`
    (:`then_0`
      (`KismetSystemLibrary.Delay` 0.01)
      (bind _asbp_player (cast `/Game/Blueprint/Player/BP_Player` (`GameplayStatics.GetPlayerPawn` 0)))
      (set `self.As BP Player` _asbp_player))
    (:`then_1`
      (bind _returnvalue (`PrimitiveComponent.CreateDynamicMaterialInstance` (`self.DestructibleComponent`) 0 null "None")))))

(event `self.BP_AC_LivingActor.OnDeath`
  (params (AttackOwner :type "Actor Object Reference"))
  (bind _destructiblecomponent (`self.DestructibleComponent`))
  (`PrimitiveComponent.SetSimulatePhysics` _destructiblecomponent true)
  (`DestructibleComponent.ApplyDamage` _destructiblecomponent 1000.0 (`SceneComponent.K2_GetComponentLocation` _destructiblecomponent) (* (`SceneComponent.GetForwardVector` _destructiblecomponent) 1000.0) 5000.0)
  (`KismetSystemLibrary.Delay` 2.0)
  (`/Engine/EditorBlueprintResources/StandardMacros.FlipFlop`
    (:`A`
      (bind (_direction _value) (`Timeline|fader` :!via `PlayFromStart` :!label _label)
        (:`Update`
          (`MaterialInstanceDynamic.SetScalarParameterValue` (stale `self.ReceiveBeginPlay` _returnvalue) "Fade" (`KismetMathLibrary.Lerp` 1.0 0.0 _value)))
        (:`Finished`
          (`self.K2_DestroyActor`))))
    (:`B`
      (goto _label :!via `ReverseFromEnd`))))

(event `self.DestructibleComponent.OnComponentFracture`
  (params (HitPoint :type "Vector Structure (by ref)") (HitDirection :type "Vector Structure (by ref)"))
  (`PrimitiveComponent.SetCollisionEnabled` (`self.DestructibleComponent`) "PhysicsOnly"))

(fn `UserConstructionScript`)