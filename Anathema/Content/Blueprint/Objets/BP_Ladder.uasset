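; BP_Ladder is a procedural ladder that acts as a one-time interactable.
; Its construction script stacks mesh segments at fixed spacing to match LadderHeight and fits the Box around them.
; The first interaction by BP_Player forwards to RefTp, apparently a teleport, then destroys the listed level 1 spawn actors.
; Climbing logic using a camera trace and Flying movement mode is disconnected, leaving the overlap events empty.
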(event `self.Box.OnComponentBeginOverlap`
  (params (OverlappedComponent :type "PrimitiveComponent Object Reference") (OtherActor :type "Actor Object Reference") (OtherComp :type "PrimitiveComponent Object Reference") (OtherBodyIndex :type Integer) (bFromSweep :type Boolean) (SweepResult :type "HitResult Structure (by ref)")))

(event `self.Box.OnComponentEndOverlap`
  (params (OverlappedComponent :type "PrimitiveComponent Object Reference") (OtherActor :type "Actor Object Reference") (OtherComp :type "PrimitiveComponent Object Reference") (OtherBodyIndex :type Integer)))

(event `/Game/Blueprint/Interface/BPI_Interact.Interact`
  (params (Player :type "Character Object Reference"))
  (`/Engine/EditorBlueprintResources/StandardMacros.DoOnce` false
    (:`Completed`
      (cast `/Game/Blueprint/Player/BP_Player` Player)
      (`/Game/Blueprint/Interface/BPI_Interact.Interact` (`self.refTp`) Player)
      (for _array_element (`self.ListeGrovSpawnLVl1ToDestroy`)
        (`/Game/Blueprint/Spawners/BP_PeriodicSpawner.Destroy` _array_element)))))

(fn `UserConstructionScript`
  (bind _returnvalue (`KismetMathLibrary.FTrunc` (/ (`self.LadderHeight`) 50.0)))
  (for _index (range 1 (+ _returnvalue 1))
    (`AddComponent|NODE_AddStaticMeshComponent-0` :`RelativeTransform` (`KismetMathLibrary.MakeTransform` (`KismetMathLibrary.MakeVector` 0.0 0.0 (* _index 50.0)))))
  (`AddComponent|NODE_AddStaticMeshComponent-1` :`RelativeTransform` (`KismetMathLibrary.MakeTransform` (`KismetMathLibrary.MakeVector` 0.0 0.0 (* (+ _returnvalue 1) 50.0))))
  (`SceneComponent.K2_SetRelativeLocation` (`self.Box`) (`KismetMathLibrary.MakeVector` 0.0 0.0 (+ (/ (`self.LadderHeight`) 2.0) 50.0)) false false)
  (`BoxComponent.SetBoxExtent` (`self.Box`) (`KismetMathLibrary.MakeVector` 64.0 32.0 (+ (/ (`self.LadderHeight`) 2.0) 50.0)) true))