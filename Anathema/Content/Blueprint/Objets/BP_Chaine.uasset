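; BP_Chaine is a destructible chain tied to the final room's multi-point spawner, which it casts from its owner at BeginPlay.
; Damage to its living-actor component prints a one-time taunt at each of two low-HP thresholds.
; On death it shatters the destructible mesh with physics and a forced impulse, then opens a grille after a brief delay.
; It also calls the spawner's NumberToAddEvent twice, before and after flagging itself destroyed.
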(event `self.ReceiveBeginPlay`
  (bind _asbp_spawner_multiple_spawn_point_salle_finale (cast `/Game/Blueprint/Objets/BP_SpawnerMultipleSpawnPointSalleFinale` (`self.GetOwner`)))
  (set `self.RefSpawner` _asbp_spawner_multiple_spawn_point_salle_finale))

(event `self.ReceiveTick`
  (params (DeltaSeconds :type "Float (single-precision)")))

(event `self.BP_AC_LivingActor.OnTakingDamage`
  (params (AttackOwner :type "Actor Object Reference") (DamageTaken :type "Float (single-precision)") (AttackType :type "/Game/Blueprint/Enum/E_AttackType Enum" :default "NewEnumerator0"))
  ;[1 1 1] Phase1
  (`|ExecutionSequence`
    (:`then_0`
      (if (<= (`/Game/Blueprint/Component/Actor/BP_AC_LivingActor.CurrentHp` (`self.BP_AC_LivingActor`)) 20.0)
        (if (`self.Phase1?`)
          (`KismetSystemLibrary.PrintString` "Je vais te goumer en sah")
          (set `self.Phase1?` false))))
    (:`then_1`
      ;[1 1 1] Phase2
      (if (<= (`/Game/Blueprint/Component/Actor/BP_AC_LivingActor.CurrentHp` (`self.BP_AC_LivingActor`)) 10.0)
        (if (`self.Phase2?`)
          (`KismetSystemLibrary.PrintString` "Arrête salaud")
          (set `self.Phase2?` false))))))

(event `self.BP_AC_LivingActor.OnDeath`
  (params (AttackOwner :type "Actor Object Reference"))
  (bind _refspawner (`self.RefSpawner`))
  (bind _destructiblecomponent (`self.DestructibleComponent`))
  ;[1 1 1] Phase 3 chaine explosion
  (`PrimitiveComponent.SetSimulatePhysics` _destructiblecomponent true)
  (`DestructibleComponent.ApplyDamage` _destructiblecomponent 10000.0 (`SceneComponent.K2_GetComponentLocation` _destructiblecomponent) (* (`SceneComponent.GetForwardVector` _destructiblecomponent) 500.0) 100.0)
  (`KismetSystemLibrary.Delay` 0.01)
  (`/Game/Blueprint/Objets/BP_Grille.OpenGrille` (`self.As BP Grille`))
  (`/Game/Blueprint/Objets/BP_SpawnerMultipleSpawnPointSalleFinale.NumberToAddEvent` _refspawner)
  (set `self.IsChainDestroyed?` true)
  (`/Game/Blueprint/Objets/BP_SpawnerMultipleSpawnPointSalleFinale.NumberToAddEvent` _refspawner))

(fn `UserConstructionScript`)