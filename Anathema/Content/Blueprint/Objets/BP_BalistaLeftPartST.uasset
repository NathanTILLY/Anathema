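; BP_BalistaLeftPartST is a pickup for a balista part, registering the first cog on the referenced balista.
; Interact or Destroyed sets HasCog1, checks for both cogs and the bolt, then Interact's sequence immediately destroys the actor.
; With all parts present, a delayed WBP_HaveAllParts popup is scheduled, though the immediate destruction likely prevents it from appearing.
; BeginPlay caches the player pawn after a short delay, but nothing here uses it.
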(event `self.ReceiveBeginPlay`
  (`KismetSystemLibrary.Delay` 0.1)
  (bind _asbp_player (cast `/Game/Blueprint/Player/BP_Player` (`GameplayStatics.GetPlayerPawn` 0)))
  (set `self.As BP Player` _asbp_player))

(event `/Game/Blueprint/Interface/BPI_Interact.Interact`
  (params (Player :type "Character Object Reference"))
  (bind _refbalista (`self.RefBalista`))
  (`|ExecutionSequence` :!label _label
    (:`then_0`
      (set `/Game/Blueprint/Objets/BP_Balista.HasCog1?` true (`self.RefBalista`)))
    (:`then_1`
      (if (`/Game/Blueprint/Objets/BP_Balista.HasCog1?` _refbalista)
        (if (`/Game/Blueprint/Objets/BP_Balista.HasCog2?` _refbalista)
          (if (`/Game/Blueprint/Objets/BP_Balista.HasBolt?` _refbalista)
            (`KismetSystemLibrary.Delay` 30.0)
            (bind _returnvalue (`|CreateWidget` "/Game/Blueprint/UI/Subtitles/WBP_HaveAllParts.WBP_HaveAllParts_C"))
            (`UserWidget.AddToViewport` _returnvalue 0)
            (`KismetSystemLibrary.Delay` 10.0)
            (`Widget.RemoveFromParent` _returnvalue)
            (`self.K2_DestroyActor`)))))
    (:`then_2`
      (`self.K2_DestroyActor`))))

(event `self.ReceiveDestroyed`
  (goto _label))

(fn `UserConstructionScript`
  (`parent.UserConstructionScript`))