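; Ballista bolt pickup that shows an interact widget on overlap and, when taken, flags the bolt on the ballista and starts a survival encounter.
; Interaction sets the Survive objective, spawns four encirclement actors and a wave of randomly picked, placed and scaled AI.
; Delayed steps would remove the encirclement and set the fix-ballista objective, but the sequence's last branch destroys the actor without waiting for them.
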(event `self.Box_0.OnComponentBeginOverlap`
  (params (OverlappedComponent :type "PrimitiveComponent Object Reference") (OtherActor :type "Actor Object Reference") (OtherComp :type "PrimitiveComponent Object Reference") (OtherBodyIndex :type Integer) (bFromSweep :type Boolean) (SweepResult :type "HitResult Structure (by ref)"))
  (bind _asbp_player (cast `/Game/Blueprint/Player/BP_Player` OtherActor))
  (set `self.PlayerRef` _asbp_player)
  (`/Engine/EditorBlueprintResources/StandardMacros.DoOnce` false :!label _label
    (:`Completed`
      (bind _returnvalue (`|CreateWidget` "/Game/Blueprint/UI/WBP_Interact.WBP_Interact_C"))
      (`KismetSystemLibrary.Delay` 0.002)
      (bind _output_get (set `self.RefInteract` _returnvalue))
      (`UserWidget.AddToViewport` _output_get 0))))

(event `self.Box_0.OnComponentEndOverlap`
  (params (OverlappedComponent :type "PrimitiveComponent Object Reference") (OtherActor :type "Actor Object Reference") (OtherComp :type "PrimitiveComponent Object Reference") (OtherBodyIndex :type Integer))
  (bind _refinteract (`self.RefInteract`))
  (`/Engine/EditorBlueprintResources/StandardMacros.IsValid` _refinteract
    (:`Is Valid`
      (`Widget.RemoveFromParent` _refinteract)
      (goto _label :!via `Reset`))))

(event `/Game/Blueprint/Interface/BPI_Interact.Interact`
  (params (Player :type "Character Object Reference"))
  (bind _refbalista (`self.RefBalista`))
  (bind _spawnlocation (`self.SpawnLocation`))
  (bind _mobaspawn (`self.MobASpawn`))
  (bind _rootcomponent (`Actor.RootComponent` (`|GetArrayItem` _spawnlocation (`KismetMathLibrary.RandomInteger` (`KismetArrayLibrary.Array_Length` _spawnlocation)))))
  ;[1 1 1] Player Interact with actor
  (`|ExecutionSequence`
    (:`then_0`
      (set `/Game/Blueprint/Objets/BP_Ballista.HasBolt?` true (`self.RefBalista`)))
    (:`then_1`
      (`ActorComponent.K2_DestroyComponent` (`self.Bolt`))
      (`ActorComponent.K2_DestroyComponent` (`self.Box_0`))
      (`/Game/Blueprint/Component/Actor/BP_AC_Objectives.SetPlayerObjectives` (`self.GetComponentByClass` (`self.PlayerRef`) "/Game/Blueprint/Component/Actor/BP_AC_Objectives.BP_AC_Objectives_C") "Survive")
      (bind _returnvalue (`|SpawnActorFromClass` "/Game/Blueprint/Objets/BP_Encirclement.BP_Encirclement_C" (`KismetMathLibrary.MakeTransform` (-3250.0 -1375.0 991.0) (struct :`Yaw` -90.0)) "Undefined" "OverrideRootScale" null null))
      (bind _returnvalue_2 (`|SpawnActorFromClass` "/Game/Blueprint/Objets/BP_Encirclement.BP_Encirclement_C" (`KismetMathLibrary.MakeTransform` (-5964.0 -2001.0 1114.0) (struct) (2.1875 2.1875 2.1875)) "Undefined" "OverrideRootScale" null null))
      (bind _returnvalue_3 (`|SpawnActorFromClass` "/Game/Blueprint/Objets/BP_Encirclement.BP_Encirclement_C" (`KismetMathLibrary.MakeTransform` (-5373.0 851.0 1062.0) (struct) (1.78125 1.78125 1.78125)) "Undefined" "OverrideRootScale" null null))
      (bind _returnvalue_4 (`|SpawnActorFromClass` "/Game/Blueprint/Objets/BP_Encirclement.BP_Encirclement_C" (`KismetMathLibrary.MakeTransform` (-3576.0 851.0 934.0) (struct) (1.03125 1.03125 1.03125)) "Undefined" "OverrideRootScale" null null))
      (while (< (`self.NbrDejaSpawn`) (`self.NbrDeSpawn`))
        (`/Engine/EditorBlueprintResources/StandardMacros.IncrementInt` (`self.NbrDejaSpawn`)
          (:`  `
            (bind _returnvalue_5 (`AIBlueprintHelperLibrary.SpawnAIFromClass` (`|GetArrayItem` _mobaspawn (`KismetMathLibrary.RandomIntegerInRange` 0 (`KismetArrayLibrary.Array_LastIndex` _mobaspawn))) null (`SceneComponent.K2_GetComponentLocation` _rootcomponent) (`SceneComponent.K2_GetComponentRotation` _rootcomponent) false null))
            (`/Engine/EditorBlueprintResources/StandardMacros.IsValid` _returnvalue_5
              (:`Is Valid`
                (bind _output_get (set `self.CurrentScale` (`KismetMathLibrary.RandomFloatInRange` 0.9 1.1)))
                (`self.SetActorScale3D` _returnvalue_5 (`KismetMathLibrary.MakeVector` _output_get _output_get _output_get)))))))
      (`KismetSystemLibrary.Delay` 30.0)
      (`self.K2_DestroyActor` _returnvalue_2)
      (`self.K2_DestroyActor` _returnvalue)
      (`self.K2_DestroyActor` _returnvalue_3)
      (`self.K2_DestroyActor` _returnvalue_4))
    (:`then_2`
      (if (and (`/Game/Blueprint/Objets/BP_Ballista.HasCog1?` _refbalista) (`/Game/Blueprint/Objets/BP_Ballista.HasCog2?` _refbalista) (`/Game/Blueprint/Objets/BP_Ballista.HasBolt?` _refbalista))
        (`KismetSystemLibrary.Delay` 30.0)
        (`/Game/Blueprint/Component/Actor/BP_AC_Objectives.SetPlayerObjectives` (`self.GetComponentByClass` (`self.PlayerRef`) "/Game/Blueprint/Component/Actor/BP_AC_Objectives.BP_AC_Objectives_C") "Fix the ballista")
        (`self.K2_DestroyActor`)))
    (:`then_3`
      (`self.K2_DestroyActor`))))

(event `self.ReceiveDestroyed`
  (set `/Game/Blueprint/Objets/BP_Ballista.HasBolt?` true (`self.RefBalista`))
  (`self.K2_DestroyActor`))

(fn `UserConstructionScript`)