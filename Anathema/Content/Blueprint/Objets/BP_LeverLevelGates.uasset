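; Interactable lever that opens the level gate paired with it.
; On Interact, Timeline_0 plays and lerps the pitch of the Niquettamère component from Close to Open.
; Every timeline update also searches all BP_LevelGate actors and calls OpenGate on the first whose DoorValue equals LeverValue, so that call repeats throughout the animation.
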(event `/Game/Blueprint/Interface/BPI_Interact.Interact`
  (params (Player :type "Character Object Reference"))
  (bind (_direction _trap) (`Timeline|Timeline_0`)
    (:`Update`
      (`SceneComponent.K2_SetRelativeRotation` (`self.niquettamère`) (`KismetMathLibrary.MakeRotator` 0.0 (`KismetMathLibrary.Lerp` (`self.Close`) (`self.Open`) _trap)) false false)
      (bind _outactors (`GameplayStatics.GetAllActorsOfClass` "/Game/Blueprint/Objets/BP_LevelGate.BP_LevelGate_C"))
      (for _array_element _outactors
        (if (== (`/Game/Blueprint/Objets/BP_LevelGate.DoorValue` _array_element) (`self.LeverValue`))
          (`/Game/Blueprint/Objets/BP_LevelGate.OpenGate` _array_element)
          (break))))))

(fn `UserConstructionScript`)