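; BP_BalistaRightPart is an interactable ballista piece that the player picks up to complete the ballista.
; On Interact it sets HasCog2 on the referenced ballista, then removes its interaction widget and destroys itself if that widget is valid.
; Its other events are unused stubs.
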(event `/Game/Blueprint/Interface/BPI_Interact.Interact`
  (params (Player :type "Character Object Reference"))
  (bind _refinteract (`self.RefInteract`))
  (`|ExecutionSequence`
    (:`then_0`
      (set `/Game/Blueprint/Objets/BP_Balista.HasCog2?` true (`self.RefBalista`)))
    (:`then_1`
      (`/Engine/EditorBlueprintResources/StandardMacros.IsValid` _refinteract
        (:`Is Valid`
          (`Widget.RemoveFromParent` _refinteract)
          (`self.K2_DestroyActor`))))))

(fn `UserConstructionScript`
  (`parent.UserConstructionScript`))