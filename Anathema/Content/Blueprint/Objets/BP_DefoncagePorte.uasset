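; Breakable door Blueprint that gets blown open when it takes damage.
; The first damage event from its LivingActor component, gated by a DoOnce, turns on physics for two static meshes and launches both with a large fixed force.
; It also spawns a scaled-up building destruction particle effect at its Scene component.
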(event `self.BP_AC_LivingActor.OnTakingDamage`
  (params (AttackOwner :type "Actor Object Reference") (DamageTaken :type "Float (single-precision)") (AttackType :type "/Game/Blueprint/Enum/E_AttackType Enum" :default "NewEnumerator0"))
  (`/Engine/EditorBlueprintResources/StandardMacros.DoOnce` false
    (:`Completed`
      (`|ExecutionSequence`
        (:`then_0`
          (`PrimitiveComponent.SetSimulatePhysics` (`self.StaticMesh1`) true)
          (`PrimitiveComponent.AddForce` (`self.StaticMesh1`) (0.0 19990000.0 1500000.0) "None" false))
        (:`then_1`
          (`PrimitiveComponent.SetSimulatePhysics` (`self.StaticMesh`) true)
          (`PrimitiveComponent.AddForce` (`self.StaticMesh`) (0.0 19990000.0 1500000.0) "None" false))
        (:`then_2`
          (`GameplayStatics.SpawnEmitterAtLocation` "/Game/VFX/Particles/Destruction/P_Destruction_Building_A.P_Destruction_Building_A" (`SceneComponent.K2_GetComponentLocation` (`self.Scene`)) (struct) (10.0 10.0 10.0)))))))

(fn `UserConstructionScript`)