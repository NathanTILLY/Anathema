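; BP_LastChance is a one-off scripted sequence in which a floating group of meshes bursts apart and its handle flies to the player's hand.
; It destroys itself if save "save1" exists; otherwise it bobs until a Tick-driven timer expires.
; The pieces then scatter with physics impulses and are removed later.
; A spawned BP_Handle replaces the original handle, interpolates via Timeline to SwordSocket, attaches briefly, then is destroyed.
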(event `GoToPlayerHand`
  (bind _handle (`self.Handle`))
  (bind _sk_mannequin_arms (`/Game/Blueprint/Player/BP_PlayerWithAnim.SK_Mannequin_Arms` (cast `/Game/Blueprint/Player/BP_PlayerWithAnim` (`GameplayStatics.GetPlayerPawn` 0) :!pure true)))
  (bind (_returnvalue_x _returnvalue_y _returnvalue_z) (`KismetMathLibrary.BreakVector` (`SceneComponent.GetSocketLocation` _sk_mannequin_arms "SwordSocket")))
  (`|ExecutionSequence`
    (:`then_0`
      (bind _returnvalue (`|SpawnActorFromClass` "/Game/Blueprint/Objets/BP_Handle.BP_Handle_C" (`SceneComponent.K2_GetComponentToWorld` _handle) "Undefined" "OverrideRootScale" null null))
      (bind (_direction _alpha) (`Timeline|Timeline_0`)
        (:`Update`
          (bind _defaultsceneroot (`/Game/Blueprint/Objets/BP_Handle.DefaultSceneRoot` _returnvalue))
          (bind (_returnvalue_location _returnvalue_rotation) (`KismetMathLibrary.BreakTransform` (`SceneComponent.K2_GetComponentToWorld` _defaultsceneroot)))
          (`SceneComponent.K2_SetWorldTransform` _defaultsceneroot (`KismetMathLibrary.MakeTransform` (`KismetMathLibrary.VInterpTo` _returnvalue_location (`KismetMathLibrary.MakeVector` (+ _returnvalue_x -2.0) (+ _returnvalue_y 0.0) (- _returnvalue_z 30.0)) _alpha 1.0) (`KismetMathLibrary.RInterpTo` _returnvalue_rotation (`SceneComponent.GetSocketRotation` _sk_mannequin_arms "SwordSocket") _alpha 1.0)) false false))
        (:`Finished`
          (`self.K2_AttachToComponent` _returnvalue _sk_mannequin_arms "SwordSocket" "SnapToTarget" "SnapToTarget" "SnapToTarget" true)
          (bind _rootcomponent (`Actor.RootComponent` _returnvalue))
          (bind (_relativelocation_x _relativelocation_y _relativelocation_z) (`KismetMathLibrary.BreakVector` (`SceneComponent.RelativeLocation` _rootcomponent)))
          (`SceneComponent.K2_SetRelativeLocation` _rootcomponent (`KismetMathLibrary.MakeVector` (+ _relativelocation_x -2.0) (+ _relativelocation_y 0.0) (- _relativelocation_z 30.0)) false true)
          (`KismetSystemLibrary.Delay` 4.0)
          (`self.K2_DestroyActor` _returnvalue))))
    (:`then_1`
      (`ActorComponent.K2_DestroyComponent` _handle))))

(event `DoIt`
  (bind _returnvalue (`KismetMathLibrary.RandomFloatInRange` 0.0 500.0))
  (`KismetArrayLibrary.Array_RemoveItem` (`self.Liste`) (`self.Handle`))
  (`ActorComponent.K2_DestroyComponent` (`self.S_CursedPlane`))
  (`ActorComponent.K2_DestroyComponent` (`self.Niagara`))
  (for _array_element (`self.Liste`)
    (`PrimitiveComponent.SetSimulatePhysics` _array_element true)
    (`PrimitiveComponent.AddImpulse` _array_element (`KismetMathLibrary.MakeVector` _returnvalue _returnvalue (`KismetMathLibrary.RandomFloatInRange` 500.0 800.0)) "None" false))
  (`PrimitiveComponent.SetSimulatePhysics` (`self.Handle`) true)
  (`KismetSystemLibrary.Delay` 2.0)
  (`self.GoToPlayerHand`)
  (`KismetSystemLibrary.Delay` 29.0)
  (for _array_element_2 (`self.Liste`)
    (`ActorComponent.K2_DestroyComponent` _array_element_2)))

(event `self.ReceiveBeginPlay`
  (bind _liste (`self.Liste`))
  (bind (_returnvalue_x _returnvalue_y _returnvalue_z) (`KismetMathLibrary.BreakVector` (`self.K2_GetActorLocation` (`GameplayStatics.GetPlayerPawn` 0))))
  (bind _returnvalue (`GameplayStatics.DoesSaveGameExist` "save1"))
  (if _returnvalue
    (`self.K2_DestroyActor`)
    (else
      (`|ExecutionSequence`
        (:`then_0`
          (`KismetArrayLibrary.Array_AddUnique` _liste (`self.StaticMesh1`))
          (`KismetArrayLibrary.Array_AddUnique` _liste (`self.StaticMesh2`))
          (`KismetArrayLibrary.Array_AddUnique` (`self.Liste`) (`self.StaticMesh3`))
          (`KismetArrayLibrary.Array_AddUnique` (`self.Liste`) (`self.StaticMesh4`))
          (`KismetArrayLibrary.Array_AddUnique` (`self.Liste`) (`self.StaticMesh5`))
          (`KismetArrayLibrary.Array_AddUnique` (`self.Liste`) (`self.StaticMesh6`))
          (`KismetArrayLibrary.Array_AddUnique` (`self.Liste`) (`self.StaticMesh7`))
          (`KismetArrayLibrary.Array_AddUnique` (`self.Liste`) (`self.StaticMesh8`))
          (`KismetArrayLibrary.Array_AddUnique` (`self.Liste`) (`self.StaticMesh9`))
          (`KismetArrayLibrary.Array_AddUnique` (`self.Liste`) (`self.StaticMesh10`))
          (`KismetArrayLibrary.Array_AddUnique` (`self.Liste`) (`self.StaticMesh11`))
          (`KismetArrayLibrary.Array_AddUnique` (`self.Liste`) (`self.S_Piece12`))
          (`KismetArrayLibrary.Array_AddUnique` (`self.Liste`) (`self.StaticMesh13`))
          (`KismetArrayLibrary.Array_AddUnique` (`self.Liste`) (`self.StaticMesh14`))
          (`KismetArrayLibrary.Array_AddUnique` (`self.Liste`) (`self.Handle`))
          (`KismetSystemLibrary.Delay` 0.2)
          (`self.Floating`))
        (:`then_1`
          (`SceneComponent.K2_SetWorldLocation` (`self.Niagara`) (`KismetMathLibrary.MakeVector` _returnvalue_x (+ _returnvalue_y -20.0) _returnvalue_z) false true))))))

(event `Floating`
  (bind _groupement (`self.Groupement`))
  (bind _groupement_2 (`self.Groupement`))
  (bind _returnvalue (`SceneComponent.GetRelativeTransform` _groupement))
  (bind _returnvalue_2 (`SceneComponent.GetRelativeTransform` _groupement_2))
  (if (< (`self.TimerBeforeExplosion`) 5.5) :!label _label
    (`KismetSystemLibrary.MoveComponentTo` _groupement (`KismetMathLibrary.MakeVector` (.x (.location _returnvalue)) (.y (.location _returnvalue)) (+ (.z (.location _returnvalue)) 30.0)) (.rotation _returnvalue) true true 2.5)
    (`KismetSystemLibrary.MoveComponentTo` _groupement_2 (`KismetMathLibrary.MakeVector` (.x (.location _returnvalue_2)) (.y (.location _returnvalue_2)) (+ (.z (.location _returnvalue_2)) -30.0)) (.rotation _returnvalue_2) true true 2.5)
    (`KismetSystemLibrary.Delay` 0.2)
    (goto _label)
    (else
      (`self.DoIt`))))

(event `self.ReceiveTick`
  (params (DeltaSeconds :type "Float (single-precision)"))
  (set `self.TimerBeforeExplosion` (+ (`GameplayStatics.GetWorldDeltaSeconds`) (`self.TimerBeforeExplosion`))))

(fn `NewFunction_0`
  (params (NewParam :type "StaticMeshComponent Object Reference"))
  (`SceneComponent.K2_SetWorldLocation` NewParam (0.0 0.0 0.0) false false))

(fn `UserConstructionScript`)