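; BP_BallistaRightPartST is an interactable pickup for one of the ballista's missing parts, its second cog.
; Interacting flags HasCog2 on the referenced ballista and destroys the actor.
; If both cogs and the bolt are then collected, it first sets the player's objective to "Fix the ballista" through BP_AC_Objectives.
; The Destroyed event also sets the HasCog2 flag, so any destruction of the part counts as collected.
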(event `/Game/Blueprint/Interface/BPI_Interact.Interact`
  (params (Player :type "Character Object Reference"))
  (bind _refbalista (`self.RefBalista`))
  (bind _asbp_player (cast `/Game/Blueprint/Player/BP_Player` Player))
  (set `self.PlayerRef` _asbp_player)
  (`|ExecutionSequence`
    (:`then_0`
      (set `/Game/Blueprint/Objets/BP_Ballista.HasCog2?` true (`self.RefBalista`)))
    (:`then_1`
      (if (and (`/Game/Blueprint/Objets/BP_Ballista.HasCog1?` _refbalista) (`/Game/Blueprint/Objets/BP_Ballista.HasCog2?` _refbalista) (`/Game/Blueprint/Objets/BP_Ballista.HasBolt?` _refbalista))
        (`/Game/Blueprint/Component/Actor/BP_AC_Objectives.SetPlayerObjectives` (`self.GetComponentByClass` (`self.PlayerRef`) "/Game/Blueprint/Component/Actor/BP_AC_Objectives.BP_AC_Objectives_C") "Fix the ballista")
        (`self.K2_DestroyActor`)))
    (:`then_2`
      (`self.K2_DestroyActor`))))

(event `self.ReceiveDestroyed`
  (set `/Game/Blueprint/Objets/BP_Ballista.HasCog2?` true (`self.RefBalista`))
  (`self.K2_DestroyActor`))

(fn `UserConstructionScript`
  (`parent.UserConstructionScript`))