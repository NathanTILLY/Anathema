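; Boss-area spawner that delivers a BP_SeptusCielus AI with a descending particle effect and impact burst.
; The Spawning event reveals two particle components and lowers them via a timeline, lerping from their current Z each update, so the drop accumulates.
; When it finishes, destruction, impact and "7emeciel" emitters play at the particle's location and the AI spawns there.
; All effect components are destroyed one second later.
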(event `self.ReceiveBeginPlay`)

(event `Spawning`
  (bind _particlesystem (`self.ParticleSystem`))
  (bind _returnvalue (`SceneComponent.K2_GetComponentLocation` (`self.ParticleSystem`)))
  (bind (_relativelocation_x _relativelocation_y _relativelocation_z) (`KismetMathLibrary.BreakVector` (`SceneComponent.RelativeLocation` _particlesystem)))
  (`SceneComponent.SetVisibility` (`self.ParticleSystem`) true false)
  (`SceneComponent.SetVisibility` (`self.ParticleSystem1`) true false)
  (bind (_direction _newtrack_0) (`Timeline|Timeline_0` :!via `PlayFromStart`)
    (:`Update`
      (`SceneComponent.K2_SetRelativeLocation` _particlesystem (`KismetMathLibrary.MakeVector` _relativelocation_x _relativelocation_y (`KismetMathLibrary.Lerp` _relativelocation_z (+ _relativelocation_z -5.0) _newtrack_0)) false false)
      (`SceneComponent.K2_SetRelativeLocation` (`self.ParticleSystem1`) (`KismetMathLibrary.MakeVector` _relativelocation_x _relativelocation_y (`KismetMathLibrary.Lerp` _relativelocation_z (+ _relativelocation_z -5.0) _newtrack_0)) false false))
    (:`Finished`
      (`|ExecutionSequence`
        (:`then_0`
          (bind _returnvalue_2 (`GameplayStatics.SpawnEmitterAtLocation` "/Game/VFX/Particles/Destruction/P_Destruction_Building_A.P_Destruction_Building_A" _returnvalue (struct) (3.0 3.0 3.0))))
        (:`then_1`
          (bind _returnvalue_3 (`GameplayStatics.SpawnEmitterAtLocation` "/Game/VFX/AuraEffect/PS_Impact.PS_Impact" _returnvalue (struct) (2.0 2.0 2.0))))
        (:`then_2`
          (bind _returnvalue_4 (`GameplayStatics.SpawnEmitterAtLocation` "/Game/VFX/AuraEffect/PS_7emeciel.PS_7emeciel" _returnvalue)))
        (:`then_3`
          (`AIBlueprintHelperLibrary.SpawnAIFromClass` "/Game/Blueprint/Enemies/SeptusCielus/BP_SeptusCielus.BP_SeptusCielus_C" null _returnvalue (struct) false null))
        (:`then_4`
          (`KismetSystemLibrary.Delay` 1.0)
          (`ActorComponent.K2_DestroyComponent` _returnvalue_3)
          (`ActorComponent.K2_DestroyComponent` (`self.ParticleSystem`))
          (`ActorComponent.K2_DestroyComponent` (`self.ParticleSystem1`))
          (`ActorComponent.K2_DestroyComponent` _returnvalue_4)
          (`ActorComponent.K2_DestroyComponent` _returnvalue_2))))))

(fn `UserConstructionScript`)