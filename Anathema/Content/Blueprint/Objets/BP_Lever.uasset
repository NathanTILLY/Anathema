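; BP_Lever is an interactable lever that opens a linked grille once the missing lever part is obtained.
; Without the part, interacting briefly shows a missing-parts widget.
; With it, the first interaction reveals the lever in place, and later ones play a timeline that rotates it down.
; The timeline's update calls OpenGrille on RefGrille through a short delay, and its completion sets Open.
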(event `/Game/Blueprint/Interface/BPI_Interact.Interact`
  (params (Player :type "Character Object Reference"))
  (if (`self.HasLever?`)
    (`|ExecutionSequence`
      (:`then_0`
        (if (`self.LeverInplace?`)
          (bind (_direction _newtrack_0) (`Timeline|LeverGoesDown`)
            (:`Update`
              (`SceneComponent.K2_SetRelativeRotation` (`self.Lever`) (`KismetMathLibrary.RLerp` (struct :`Pitch` -60.0 :`Yaw` -90.0) (`self.LeverRotationEnd`) _newtrack_0) false false)
              (`KismetSystemLibrary.Delay` 0.2)
              (`/Game/Blueprint/Objets/BP_Grille.OpenGrille` (`self.RefGrille`)))
            (:`Finished`
              (set `self.Open?` true)))))
      (:`then_1`
        (`SceneComponent.SetHiddenInGame` (`self.Lever`) false false)
        (set `self.LeverInplace?` true)))
    (else
      (bind _returnvalue (`|CreateWidget` "/Game/Blueprint/UI/WBP_MissingParts.WBP_MissingParts_C"))
      (`UserWidget.AddToViewport` _returnvalue 0)
      (`KismetSystemLibrary.Delay` 3.0)
      (`Widget.RemoveFromParent` _returnvalue))))

(fn `UserConstructionScript`
  (`parent.UserConstructionScript`))