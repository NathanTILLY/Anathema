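; BP_BallistaRightPart is a collectible ballista piece that counts as the second cog needed for the repair.
; Interact flags the cog on the referenced ballista, removes the interact widget and destroys the actor.
; Once both cogs and the bolt are held, it swaps the player's current HUD widget for WBP_FixTheBalista.
; The Destroyed event runs the same sequence, using a player reference cached shortly after BeginPlay.
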(event `self.ReceiveBeginPlay`
  (`KismetSystemLibrary.Delay` 0.1)
  (bind _asbp_player (cast `/Game/Blueprint/Player/BP_Player` (`GameplayStatics.GetPlayerPawn` 0)))
  (set `self.As BP Player` _asbp_player))

(event `/Game/Blueprint/Interface/BPI_Interact.Interact`
  (params (Player :type "Character Object Reference"))
  (bind _refbalista (`self.RefBalista`))
  (bind _refinteract (`self.RefInteract`))
  (`|ExecutionSequence` :!label _label
    (:`then_0`
      (set `/Game/Blueprint/Objets/BP_Ballista.HasCog2?` true (`self.RefBalista`)))
    (:`then_1`
      (`/Engine/EditorBlueprintResources/StandardMacros.IsValid` _refinteract
        (:`Is Valid`
          (`Widget.RemoveFromParent` _refinteract)
          (`self.K2_DestroyActor`))))
    (:`then_2`
      (if (`/Game/Blueprint/Objets/BP_Ballista.HasCog1?` _refbalista)
        (if (`/Game/Blueprint/Objets/BP_Ballista.HasCog2?` _refbalista)
          (if (`/Game/Blueprint/Objets/BP_Ballista.HasBolt?` _refbalista)
            (`Widget.RemoveFromParent` (`/Game/Blueprint/Player/BP_Player.RefFTMBP` (`self.As BP Player`)))
            (bind _returnvalue (`|CreateWidget` "/Game/Blueprint/UI/Objectives/WBP_FixTheBalista.WBP_FixTheBalista_C"))
            (bind _output_get (set `/Game/Blueprint/Player/BP_Player.RefFTB` _returnvalue (`self.As BP Player`)))
            (`UserWidget.AddToViewport` _output_get 0)
            (`self.K2_DestroyActor`)))))))

(event `self.ReceiveDestroyed`
  (goto _label))

(fn `UserConstructionScript`
  (`parent.UserConstructionScript`))