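; BP_CursedSwordStart is an actor that plays a timed shattering effect, apparently for the cursed sword's start.
; Five seconds after BeginPlay it destroys the SCursedPlane component, then shortly afterwards enables physics on Destructible1.
; It then hits that destructible with a huge impulse and massive damage directed along its forward vector.
; Tick applies an upward impulse to the destructible every frame and prints a debug "Hello".
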(event `self.ReceiveBeginPlay`
  (bind _destructible1 (`self.Destructible1`))
  (`KismetSystemLibrary.Delay` 5.0)
  (`ActorComponent.K2_DestroyComponent` (`self.S_CursedPlane`))
  (`KismetSystemLibrary.Delay` 0.2)
  (`PrimitiveComponent.SetSimulatePhysics` _destructible1 true)
  (`PrimitiveComponent.AddImpulse` (`self.Destructible1`) (1000000.0 1000000.0 1000000.0) "None" false)
  (`DestructibleComponent.ApplyDamage` _destructible1 5000000.0 (`SceneComponent.K2_GetComponentLocation` _destructible1) (* (`SceneComponent.GetForwardVector` _destructible1) 10000000.0) 1000000000.0))

(event `self.ReceiveTick`
  (params (DeltaSeconds :type "Float (single-precision)"))
  (`PrimitiveComponent.AddImpulse` (`self.Destructible1`) (0.0 0.0 10000.0) "None" false)
  (`KismetSystemLibrary.PrintString` "Hello"))

(fn `UserConstructionScript`)