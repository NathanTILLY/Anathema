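; BP_SaveLevel captures a snapshot of the player's state for saving.
; SavePlayerData gathers transform, current and max health, souls and weapon state through helper functions and packs them into PlayerStruct.
; The saved transform takes rotation from the controller's control rotation rather than the actor.
; Weapon state records the last weapon index, plus the consumable weapon's class and use count when its slot is valid.
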(fn `SavePlayerData`
  (params (Player :type "/Game/Blueprint/Player/BP_Player Object Reference"))
  (bind _returnvalue (`self.SetPlayerTransform` Player))
  (bind (_currenthp _maxhp) (`self.SetPlayerHealthValue` (`local.Player`)))
  (bind _currentsoul (`self.SetPlayerSoulValue` (`local.Player`)))
  (bind (_lastweaponindex _consumableweaponclass _numberofuses) (`self.SetPlayerWeapon` (`local.Player`)))
  (set `self.PlayerStruct` (make `/Game/Blueprint/Structure/SPlayerDataSave` _returnvalue (make `/Game/Blueprint/Structure/SHealthValue` _currenthp _maxhp) _currentsoul _lastweaponindex _consumableweaponclass _numberofuses)))

(fn `SetPlayerHealthValue`
  (params (Player :type "/Game/Blueprint/Player/BP_Player Object Reference"))
  (returns (CurrentHp :type "Float (double-precision)") (MaxHp :type "Float (double-precision)"))
  (bind _bp_ac_livingactor (`/Game/Blueprint/Player/BP_Player.BP_AC_LivingActor` Player))
  (return (`/Game/Blueprint/Component/Actor/BP_AC_LivingActor.CurrentHp` _bp_ac_livingactor) (`/Game/Blueprint/Component/Actor/BP_AC_LivingActor.MaxHp` _bp_ac_livingactor)))

(fn `SetPlayerSoulValue`
  (params (Player :type "/Game/Blueprint/Player/BP_Player Object Reference"))
  (returns (CurrentSoul :type "Float (double-precision)"))
  (return (`/Game/Blueprint/Component/Actor/BP_AC_SoulHandler.CurrentSoul` (`/Game/Blueprint/Player/BP_Player.BP_AC_SoulHandler` Player))))

(fn `SetPlayerTransform`
  (params (Player :type "/Game/Blueprint/Player/BP_Player Object Reference"))
  (returns (ReturnValue :type "Transform Structure"))
  (bind (_returnvalue_location _returnvalue_rotation _returnvalue_scale) (`KismetMathLibrary.BreakTransform` (`Actor.GetTransform` Player)))
  (return (`KismetMathLibrary.MakeTransform` _returnvalue_location (`Controller.GetControlRotation` (`/Game/Blueprint/Player/BP_Player.MyController` Player)) _returnvalue_scale)))

(fn `SetPlayerWeapon`
  (params (Player :type "/Game/Blueprint/Player/BP_Player Object Reference"))
  (returns (LastWeaponIndex :type Integer) (ConsumableWeaponClass :type "/Game/Blueprint/Weapons/Consumable/BP_ConsumableWeaponParent Class Reference") (NumberOfUses :type Integer))
  (bind _lastweaponindex (`/Game/Blueprint/Player/BP_Player.LastWeaponIndex` Player))
  (bind _weaponslot (`/Game/Blueprint/Component/Actor/BP_AC_ConsumableWeapon.WeaponSlot` (`/Game/Blueprint/Player/BP_Player.BP_AC_ConsumableWeapon` (`local.Player`))))
  (`/Engine/EditorBlueprintResources/StandardMacros.IsValid` _weaponslot
    (:`Is Valid`
      (return _lastweaponindex (`GameplayStatics.GetObjectClass` _weaponslot) (`/Game/Blueprint/Weapons/Consumable/BP_ConsumableWeaponParent.NumberOfUses` _weaponslot)))
    (:`Is Not Valid`
      (return _lastweaponindex null 0))))