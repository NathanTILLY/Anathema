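; BP_SetTable is a table-setting prop whose cutlery can be toggled per instance.
; Its construction script sets the visibility of two left and two right forks, two left and two right knives, and a spoon, each from its own boolean.
; Fork and knife toggles propagate to child components, while the spoon toggle does not.
; The event graph holds no active logic.
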(fn `UserConstructionScript`
  (`|ExecutionSequence`
    (:`then_0`
      (`|ExecutionSequence`
        (:`then_0`
          ;[1 1 1] Add/remove ForkLeft
          (`SceneComponent.SetVisibility` (`self.ForkLeft_02`) (`self.AddForkLeft`) true))
        (:`then_1`
          (`SceneComponent.SetVisibility` (`self.ForkLeft_01`) (`self.AddForkLeft2`) true))
        (:`then_2`
          ;[1 1 1] Add/remove ForkRight
          (`SceneComponent.SetVisibility` (`self.ForkRight_01`) (`self.AddForkRight`) true))
        (:`then_3`
          (`SceneComponent.SetVisibility` (`self.ForkRight_02`) (`self.AddForkRight2`) true))))
    (:`then_1`
      (`|ExecutionSequence`
        (:`then_0`
          ;[1 1 1] Add/Remove KnifeLeft
          (`SceneComponent.SetVisibility` (`self.KnifeLeft_01`) (`self.AddKinfeLeft`) true))
        (:`then_1`
          (`SceneComponent.SetVisibility` (`self.KnifeLeft_02`) (`self.AddKinfeLeft2`) true))
        (:`then_2`
          ;[1 1 1] Add/remove KnifeRight
          (`SceneComponent.SetVisibility` (`self.KnifeRight_01`) (`self.AddKinfeRight`) true))
        (:`then_3`
          (`SceneComponent.SetVisibility` (`self.KnifeRight_02`) (`self.AddKinfeRight2`) true))))
    (:`then_2`
      (`SceneComponent.SetVisibility` (`self.Spoon`) (`self.AddSpoon`) false))))