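; Configurable table-setting prop that bundles mugs, plates, forks, knives, spoons and vases into one placeable actor.
; The construction script sets each piece's visibility, propagated to children, from its own Add boolean, grouped by item type.
; Pieces are only shown or hidden, never spawned or removed, and the event graph has no active logic.
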(fn `UserConstructionScript`
  (`|ExecutionSequence`
    (:`then_0`
      (`|ExecutionSequence`
        (:`then_0`
          ;[1 1 1] Add/remove Choppe
          (`SceneComponent.SetVisibility` (`self.Choppe_01`) (`self.Add_Choppe`) true))
        (:`then_1`
          (`SceneComponent.SetVisibility` (`self.Choppe_02`) (`self.Add_Choppe_01`) true))
        (:`then_2`
          (`SceneComponent.SetVisibility` (`self.Choppe_03`) (`self.Add_Choppe_02`) true))
        (:`then_3`
          (`SceneComponent.SetVisibility` (`self.Choppe_04`) (`self.Add_Choppe_03`) true))))
    (:`then_1`
      (`|ExecutionSequence`
        (:`then_0`
          ;[1 1 1] Add/remove Assiette
          (`SceneComponent.SetVisibility` (`self.Assiette`) (`self.Add_Assiette`) true))
        (:`then_1`
          (`SceneComponent.SetVisibility` (`self.Assiette1`) (`self.Add_Assiette_01`) true))
        (:`then_2`
          (`SceneComponent.SetVisibility` (`self.Assiette2`) (`self.Add_Assiette_02`) true))
        (:`then_3`
          (`SceneComponent.SetVisibility` (`self.Assiette3`) (`self.Add_Assiette_03`) true))))
    (:`then_2`
      (`|ExecutionSequence`
        (:`then_0`
          ;[1 1 1] Add/remove Fork
          (`SceneComponent.SetVisibility` (`self.Fork`) (`self.Add_Fork`) true))
        (:`then_1`
          (`SceneComponent.SetVisibility` (`self.Fork1`) (`self.Add_Fork_01`) true))
        (:`then_2`
          (`SceneComponent.SetVisibility` (`self.Fork2`) (`self.Add_Fork_02`) true))
        (:`then_3`
          (`SceneComponent.SetVisibility` (`self.Fork3`) (`self.Add_Fork_03`) true))
        (:`then_4`
          (`SceneComponent.SetVisibility` (`self.Fork4`) (`self.Add_Fork_04`) true))))
    (:`then_3`
      (`|ExecutionSequence`
        (:`then_0`
          ;[1 1 1] Add/Remove Knife
          (`SceneComponent.SetVisibility` (`self.Knife`) (`self.Add_Knife`) true))
        (:`then_1`
          (`SceneComponent.SetVisibility` (`self.Knife1`) (`self.Add_Knife_01`) true))
        (:`then_2`
          (`SceneComponent.SetVisibility` (`self.Knife2`) (`self.Add_Knife_02`) true))
        (:`then_3`
          (`SceneComponent.SetVisibility` (`self.Knife3`) (`self.Add_Knife_03`) true))
        (:`then_4`
          (`SceneComponent.SetVisibility` (`self.Knife4`) (`self.Add_Knife_04`) true))))
    (:`then_4`
      (`|ExecutionSequence`
        (:`then_0`
          ;[1 1 1] Add/remove Spoon
          (`SceneComponent.SetVisibility` (`self.Spoon`) (`self.Add_Spoon`) true))
        (:`then_1`
          (`SceneComponent.SetVisibility` (`self.Spoon1`) (`self.Add_Spoon_01`) true))
        (:`then_2`
          (`SceneComponent.SetVisibility` (`self.Spoon2`) (`self.Add_Spoon_02`) true))
        (:`then_3`
          (`SceneComponent.SetVisibility` (`self.Spoon3`) (`self.Add_Spoon_03`) true))))
    (:`then_5`
      (`|ExecutionSequence`
        (:`then_0`
          ;[1 1 1] Add/Remove Vase
          (`SceneComponent.SetVisibility` (`self.Vase`) (`self.Add_Vase`) true))
        (:`then_1`
          (`SceneComponent.SetVisibility` (`self.Vase1`) (`self.Add_Vase_01`) true))))))