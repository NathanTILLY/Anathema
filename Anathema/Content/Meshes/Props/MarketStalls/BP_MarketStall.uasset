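; Market stall prop that displays weapons and armor, with each item toggled per instance.
; The construction script sets each swords, chestplate, armor part and shield component's visibility from its own boolean variable, propagating to child components.
; Toggles are grouped by item type with nested sequences.
; The event graph holds only disabled default events, so nothing runs at play time.
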(fn `UserConstructionScript`
  (`|ExecutionSequence`
    (:`then_0`
      (`|ExecutionSequence`
        (:`then_0`
          ;[1 1 1] Add/Remove Sword
          (`SceneComponent.SetVisibility` (`self.Sword`) (`self.AddSword_01`) true))
        (:`then_1`
          (`SceneComponent.SetVisibility` (`self.Sword1`) (`self.AddSword_02`) true))
        (:`then_2`
          (`SceneComponent.SetVisibility` (`self.Sword2`) (`self.AddSword_03`) true))
        (:`then_3`
          (`SceneComponent.SetVisibility` (`self.Sword3`) (`self.AddSword_04`) true))
        (:`then_4`
          (`SceneComponent.SetVisibility` (`self.Sword4`) (`self.AddSword_05`) true))
        (:`then_5`
          (`SceneComponent.SetVisibility` (`self.Sword5`) (`self.AddSword_06`) true))
        (:`then_6`
          (`SceneComponent.SetVisibility` (`self.Sword6`) (`self.AddSword_07`) true))
        (:`then_7`
          (`SceneComponent.SetVisibility` (`self.Sword7`) (`self.AddSword_08`) true))))
    (:`then_1`
      (`|ExecutionSequence`
        (:`then_0`
          ;[1 1 1] Add/Remove Chestplate
          (`SceneComponent.SetVisibility` (`self.ArmorChestplate`) (`self.AddChestplate`) true))
        (:`then_1`
          (`SceneComponent.SetVisibility` (`self.ArmorChestplate1`) (`self.AddChestplate_01`) true))
        (:`then_2`
          (`SceneComponent.SetVisibility` (`self.ArmorChestplate2`) (`self.AddChestplate_02`) true))
        (:`then_3`
          (`SceneComponent.SetVisibility` (`self.ArmorChestplate3`) (`self.AddChestplate_03`) true))))
    (:`then_2`
      (`|ExecutionSequence`
        (:`then_0`
          ;[1 1 1] Add/remove ArmorParts
          (`SceneComponent.SetVisibility` (`self.ArmorParts`) (`self.AddArmorParts`) true))
        (:`then_1`
          (`SceneComponent.SetVisibility` (`self.ArmorParts1`) (`self.AddArmorParts_01`) true))
        (:`then_2`
          (`SceneComponent.SetVisibility` (`self.ArmorParts2`) (`self.AddArmorParts_02`) true))
        (:`then_3`
          (`SceneComponent.SetVisibility` (`self.ArmorParts3`) (`self.AddArmorParts_03`) true))
        (:`then_4`
          (`SceneComponent.SetVisibility` (`self.ArmorParts4`) (`self.AddArmorParts_04`) true))
        (:`then_5`
          (`SceneComponent.SetVisibility` (`self.ArmorParts5`) (`self.AddArmorParts_05`) true))
        (:`then_6`
          (`SceneComponent.SetVisibility` (`self.ArmorParts6`) (`self.AddArmorParts_06`) true))
        (:`then_7`
          (`SceneComponent.SetVisibility` (`self.ArmorParts7`) (`self.AddArmorParts_07`) true))
        (:`then_8`
          (`SceneComponent.SetVisibility` (`self.ArmorParts8`) (`self.AddArmorParts_08`) true))
        (:`then_9`
          (`SceneComponent.SetVisibility` (`self.ArmorParts9`) (`self.AddArmorParts_09`) true))
        (:`then_10`
          (`SceneComponent.SetVisibility` (`self.ArmorParts10`) (`self.AddArmorParts_10`) true))))
    (:`then_3`
      (`|ExecutionSequence`
        (:`then_0`
          ;[1 1 1] Add/remove Shield
          (`SceneComponent.SetVisibility` (`self.Shield`) (`self.AddShield`) true))
        (:`then_1`
          (`SceneComponent.SetVisibility` (`self.Shield1`) (`self.AddShield_01`) true))
        (:`then_2`
          (`SceneComponent.SetVisibility` (`self.Shield2`) (`self.AddShield_02`) true))))))