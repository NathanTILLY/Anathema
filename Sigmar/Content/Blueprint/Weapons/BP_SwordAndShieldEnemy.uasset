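; BP_SwordAndShieldEnemy is an enemy weapon Blueprint that overrides hit validation on top of its parent's construction script.
; CanHit detects hits on BP_Shield and, through the BPI_UsingWeapon interface, tells the weapon's owner to deactivate the weapon, with debug prints along the way.
; Other hits count only if the actor is not the owner, the weapon, the owner's class, or either Griveton class.
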(fn `CanHit`
  (params (ActorHit :type "Object Object Reference"))
  (returns (`CanHit?` :type Boolean))
  (locals (LocActorHit :type "Object Object Reference"))
  (bind _returnvalue (`self.GetOwner`))
  (bind _output_get (set `local.LocActorHit` ActorHit))
  (if (== (`GameplayStatics.GetObjectClass` _output_get) "/Game/Blueprint/Weapons/BP_Shield.BP_Shield_C")
    (`KismetSystemLibrary.PrintString` "HitShield")
    (if (`KismetSystemLibrary.DoesImplementInterface` _returnvalue "/Game/Blueprint/Interface/BPI_UsingWeapon.BPI_UsingWeapon_C")
      (`KismetSystemLibrary.PrintString` "InactiveWeapon")
      (message `/Game/Blueprint/Interface/BPI_UsingWeapon.InactiveWeapon` _returnvalue)
      (else
        (`KismetSystemLibrary.PrintString` "error")))
    (elif (and (!= (`local.LocActorHit`) (`self.MyOwner`)) (!= (`local.LocActorHit`) self) (!= (`GameplayStatics.GetObjectClass` (`local.LocActorHit`)) (`GameplayStatics.GetObjectClass` (`self.MyOwner`))) (!= (`GameplayStatics.GetObjectClass` (`local.LocActorHit`)) "/Game/Blueprint/Enemies/GrivetonQuiAttend/BP_GrivetonAttend.BP_GrivetonAttend_C") (!= (`GameplayStatics.GetObjectClass` (`local.LocActorHit`)) "/Game/Blueprint/Enemies/Griveton/BP_Griveton.BP_Griveton_C"))
      (return true)
      (else
        (return false)))))

(fn `UserConstructionScript`
  (`parent.UserConstructionScript`))