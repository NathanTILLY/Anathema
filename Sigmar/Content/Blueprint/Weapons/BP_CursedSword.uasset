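; Cursed sword weapon Blueprint whose light and heavy attacks cost souls from the wielder.
; It overrides both attack functions, first calling the parent version, then asking the owner's BP_AC_SoulHandler component to consume that attack's cost.
; Each returns whether the soul was consumed, though the parent logic runs before that check.
; The event graph holds only disabled placeholder events.
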(fn `HeavyAttack`
  (returns (`CanAttack?` :type Boolean))
  (`parent.HeavyAttack`)
  (bind _canusesoul_ (`/Game/Blueprint/Component/Actor/BP_AC_SoulHandler.ConsumeSoul` (`self.GetComponentByClass` (`self.MyOwner`) "/Game/Blueprint/Component/Actor/BP_AC_SoulHandler.BP_AC_SoulHandler_C") (`self.HeavyAttackCost`)))
  (if _canusesoul_
    (return true)
    (else
      (return false))))

(fn `LightAttack`
  (returns (`CanAttack?` :type Boolean))
  (`parent.LightAttack`)
  (bind _canusesoul_ (`/Game/Blueprint/Component/Actor/BP_AC_SoulHandler.ConsumeSoul` (`self.GetComponentByClass` (`self.MyOwner`) "/Game/Blueprint/Component/Actor/BP_AC_SoulHandler.BP_AC_SoulHandler_C") (`self.LightAttackCost`)))
  (if _canusesoul_
    (return true)
    (else
      (return false))))

(fn `UserConstructionScript`
  (`parent.UserConstructionScript`))