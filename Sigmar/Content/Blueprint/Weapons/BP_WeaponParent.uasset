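; Parent melee weapon Blueprint that becomes visible on pickup, records its owner and damages living actors through a toggled hitbox.
; Light and heavy attacks set the damage; overlaps skip the owner's class and actors already hit until the hitbox deactivates.
; Each hit calls BP_AC_LivingActor's TakeDamage, cuts remaining damage to 66%, and spawns Niagara FX.
; A damage-scaled hit-stop duration is recalculated and broadcast through OnHit.
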(event `self.Hitbox.OnComponentBeginOverlap`
  (params (OverlappedComponent :type "PrimitiveComponent Object Reference") (OtherActor :type "Actor Object Reference") (OtherComp :type "PrimitiveComponent Object Reference") (OtherBodyIndex :type Integer) (bFromSweep :type Boolean) (SweepResult :type "HitResult Structure (by ref)"))
  (bind _canhit_ (`self.CanHit` OtherActor))
  (if _canhit_
    (bind _newactorhit (`self.ActorHit` OtherActor))
    (if _newactorhit
      (`AddComponent|NODE_AddNiagaraComponent-2` :`bManualAttachment` true :`RelativeTransform` (`SceneComponent.K2_GetComponentToWorld` (`self.Box`))))))

(event `/Game/Blueprint/Interface/BPI_WeaponAttack.PickUp`
  (params (Owner :type "Actor Object Reference"))
  (set `self.MyOwner` Owner)
  (`self.SetActorHiddenInGame` self false))

(fn `ActorHit`
  (params (ActorHit :type "Actor Object Reference"))
  (returns (NewActorHit :type Boolean))
  (locals (`LocAlreadyHit?` :type Boolean) (LocActorHit :type "Actor Object Reference") (LocLivingComponent :type "/Game/Blueprint/Component/Actor/BP_AC_LivingActor Object Reference"))
  ;[1 1 1] Check if the enemy hit has already been hit by the same attack
  (set `local.LocAlreadyHit?` false)
  (set `local.LocActorHit` ActorHit)
  (bind _output_get (set `local.LocLivingComponent` (`self.GetComponentByClass` ActorHit "/Game/Blueprint/Component/Actor/BP_AC_LivingActor.BP_AC_LivingActor_C")))
  (`/Engine/EditorBlueprintResources/StandardMacros.IsValid` _output_get
    (:`Is Valid`
      (for _array_element (`self.AlreadyHitActor`)
        (if (not (!= _array_element (`local.LocActorHit`)))
          (set `local.LocAlreadyHit?` true)))
      (if (`local.LocAlreadyHit?`)
        (return false)
        (else
          (`/Game/Blueprint/Component/Actor/BP_AC_LivingActor.TakeDamage` (`local.LocLivingComponent`) (`self.CurrentDamage`) (`self.MyOwner`))
          (bind _output_get_2 (set `self.CurrentDamage` (* (`self.CurrentDamage`) 0.66)))
          (`self.SetAnimationStopValue` _output_get_2)
          (`KismetArrayLibrary.Array_AddUnique` (`self.AlreadyHitActor`) (`local.LocActorHit`))
          (`self.OnHit` (`self.CurrentStopTimer`))
          (return true))))))

(fn `CanHit`
  (params (ActorHit :type "Object Object Reference"))
  (returns (`CanHit?` :type Boolean))
  (if (and (!= ActorHit (`self.MyOwner`)) (!= ActorHit self) (!= (`GameplayStatics.GetObjectClass` ActorHit) (`GameplayStatics.GetObjectClass` (`self.MyOwner`))))
    (return true)
    (else
      (return false))))

(fn `HeavyAttack`
  (returns (`CanAttack?` :type Boolean))
  (bind _output_get (set `self.CurrentDamage` (`self.HeavyAttackDamage`)))
  (`self.SetAnimationStopValue` _output_get)
  (return true))

(fn `LightAttack`
  (returns (`CanAttack?` :type Boolean))
  (bind _output_get (set `self.CurrentDamage` (`self.LightAttackDamage`)))
  (`self.SetAnimationStopValue` _output_get)
  (return true))

(fn `SetAnimationStopValue`
  (params (DamageValue :type "Float (double-precision)"))
  ;[1 1 1] Set the stop timer between 0.00...1s and 0.16s (0 (or 1, not sure) and 10 frame)
  (set `self.CurrentStopTimer` (* 0.16 (- 1.0 (/ 0.16 (`KismetMathLibrary.FClamp` (* DamageValue 0.25) 0.16 10000.0)))))
  (return))

(fn `SetHitboxState`
  (params (`Active?` :type Boolean))
  (if `Active?`
    (`PrimitiveComponent.SetCollisionEnabled` (`self.Hitbox`) "QueryOnly")
    (set `self.IsAttacking?` true)
    (else
      (`PrimitiveComponent.SetCollisionEnabled` (`self.Hitbox`) "NoCollision")
      (set `self.IsAttacking?` false)
      (`KismetArrayLibrary.Array_Clear` (`self.AlreadyHitActor`)))))

(fn `UserConstructionScript`)