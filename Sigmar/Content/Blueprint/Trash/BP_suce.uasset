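; Damageable living actor that breaks into physics-driven mesh pieces when it dies, using BP_AC_LivingActor for health events.
; On damage it prints remaining HP and stores a direction toward the attacker with fixed Z.
; On death it removes the capsule, hides Body, launches the static mesh pieces along the negated vector, then destroys itself after a delay.
; A MeleeAttack event briefly pulses an Attack flag.
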(event `self.BP_AC_LivingActor.OnTakingDamage`
  (params (AttackOwner :type "Actor Object Reference"))
  (bind _output_get (set `self.ExplosionVector` (`KismetMathLibrary.Normal` (- (`self.K2_GetActorLocation` AttackOwner) (`self.K2_GetActorLocation`)))))
  (set `self.ExplosionVector` (`KismetMathLibrary.MakeVector` (.x _output_get) (.y _output_get) 0.5))
  (`KismetSystemLibrary.PrintString` (`KismetStringLibrary.Concat_StrStr` (`KismetSystemLibrary.GetObjectName` self) " remaining hp : " (`KismetStringLibrary.Conv_DoubleToString` (`/Game/Blueprint/Component/Actor/BP_AC_LivingActor.CurrentHp` (`self.BP_AC_LivingActor`))))))

(event `self.BP_AC_LivingActor.OnDeath`
  (params (AttackOwner :type "Actor Object Reference"))
  (bind _body (`self.body`))
  (bind _capsule (`self.Capsule`))
  (bind _staticmesh1 (`self.StaticMesh1`))
  (bind _returnvalue (* (`self.ExplosionVector`) -500000.0))
  (`KismetSystemLibrary.PrintString` "So long")
  (`/Engine/EditorBlueprintResources/StandardMacros.IsValid` _capsule
    (:`Is Valid`
      (`ActorComponent.K2_DestroyComponent` _capsule)
      (`SceneComponent.SetHiddenInGame` _body true false)
      (`PrimitiveComponent.SetCollisionEnabled` _body "NoCollision")
      (`|ExecutionSequence`
        (:`then_0`
          (`PrimitiveComponent.SetCollisionProfileName` _staticmesh1 "IgnorePawn" true)
          (`PrimitiveComponent.SetSimulatePhysics` _staticmesh1 true)
          (`PrimitiveComponent.AddForce` _staticmesh1 _returnvalue "None" false)
          (`KismetSystemLibrary.Delay` 0.0 :!label _label)
          (`KismetSystemLibrary.Delay` 5.0)
          (`self.K2_DestroyActor`))
        (:`then_1`
          (for _array_element (`|MakeArray` null (`self.StaticMesh2`) (`self.StaticMesh3`) (`self.StaticMesh4`) (`self.StaticMesh5`) (`self.StaticMesh6`) (`self.StaticMesh7`) (`self.StaticMesh8`) (`self.StaticMesh9`) (`self.StaticMesh10`) (`self.StaticMesh11`) (`self.StaticMesh12`) (`self.StaticMesh13`) (`self.StaticMesh14`) (`self.StaticMesh15`) (`self.StaticMesh16`) (`self.StaticMesh17`) (`self.StaticMesh18`) (`self.StaticMesh19`) (`self.StaticMesh20`))
            (`/Engine/EditorBlueprintResources/StandardMacros.IsValid` _array_element
              (:`Is Valid`
                (`PrimitiveComponent.SetCollisionProfileName` _array_element "IgnorePawn" true)
                (`PrimitiveComponent.SetSimulatePhysics` _array_element true)
                (`PrimitiveComponent.AddForce` _array_element _returnvalue "None" false)
                (goto _label)))))))))

(event `/Game/Blueprint/Enemies/GeneralEnemy/BI_CombatInterface.MeleeAttack`
  (set `self.Attack?` true)
  (`KismetSystemLibrary.Delay` 0.2)
  (set `self.Attack?` false))

(fn `UserConstructionScript`)