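; BP_Enemy is a basic enemy actor whose health and death events come from its BP_AC_LivingActor component.
; Taking damage prints the actor's name and remaining HP as debug text.
; On death, it looks for a BP_AC_SoulHandler on the attack's owner, grants it SoulValue souls, prints a message and destroys itself.
; The destroy happens only when that soul handler exists.
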(event `self.BP_AC_LivingActor.OnTakingDamage`
  (params (AttackOwner :type "Actor Object Reference"))
  (`KismetSystemLibrary.PrintString` (`KismetStringLibrary.Concat_StrStr` (`KismetSystemLibrary.GetObjectName` self) " remaining hp : " (`KismetStringLibrary.Conv_DoubleToString` (`/Game/Blueprint/Component/Actor/BP_AC_LivingActor.CurrentHp` (`self.BP_AC_LivingActor`))))))

(event `self.BP_AC_LivingActor.OnDeath`
  (params (AttackOwner :type "Actor Object Reference"))
  (bind _returnvalue (`self.GetComponentByClass` AttackOwner "/Game/Blueprint/Component/Actor/BP_AC_SoulHandler.BP_AC_SoulHandler_C"))
  (`/Engine/EditorBlueprintResources/StandardMacros.IsValid` _returnvalue
    (:`Is Valid`
      (`/Game/Blueprint/Component/Actor/BP_AC_SoulHandler.GainSoul` _returnvalue (`self.SoulValue`))
      (`KismetSystemLibrary.PrintString` "So long")
      (`self.K2_DestroyActor`))))

(fn `UserConstructionScript`)