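; Anim notify named CreateCursedSwordProjectile that spawns a BP_CursedSwordProjectile when an animation reaches it, apparently a test version.
; The spawn point is the mesh component's world location plus a Test offset and a short horizontal push along its forward vector.
; The projectile takes the mesh's rotation and scale and is owned by the mesh's owner, and a debug "Hello" string prints afterwards.
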(fn `GetNotifyName`
  (returns (ReturnValue :type String))
  (return "CreateCursedSwordProjectile"))

(fn `Received_Notify`
  (params (MeshComp :type "SkeletalMeshComponent Object Reference") (Animation :type "AnimSequenceBase Object Reference"))
  (returns (ReturnValue :type Boolean))
  (bind (_returnvalue_location _returnvalue_rotation _returnvalue_scale) (`KismetMathLibrary.BreakTransform` (`SceneComponent.K2_GetComponentToWorld` MeshComp)))
  (bind (_returnvalue_x _returnvalue_y) (`KismetMathLibrary.BreakVector` (* (`SceneComponent.GetForwardVector` MeshComp) 10.0)))
  (`|SpawnActorFromClass` "/Game/Blueprint/Trash/BP_CursedSwordProjectile.BP_CursedSwordProjectile_C" (`KismetMathLibrary.MakeTransform` (+ (`self.Test?`) _returnvalue_location (`KismetMathLibrary.MakeVector` _returnvalue_x _returnvalue_y)) _returnvalue_rotation _returnvalue_scale) "Undefined" "OverrideRootScale" (`ActorComponent.GetOwner` MeshComp) null)
  (`KismetSystemLibrary.PrintString` "Hello")
  (return false))