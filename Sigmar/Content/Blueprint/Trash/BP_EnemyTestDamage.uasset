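; BP_EnemyTestDamage is a test enemy for damage and death handling.
; On BeginPlay it spawns a BP_SwordAndShield and snaps it to the skeletal mesh's sword socket.
; BP_AC_LivingActor events drive the rest: damage prints remaining HP and the offset toward the attacker.
; Death grants SoulValue through the attacker's BP_AC_SoulHandler, then destroys weapon and enemy, but only if that handler exists.
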(event `self.ReceiveBeginPlay`
  (bind _returnvalue (`|SpawnActorFromClass` "/Game/Blueprint/Weapons/BP_SwordAndShield.BP_SwordAndShield_C" (`self.GetTransform`) "Undefined" "OverrideRootScale" null null))
  (bind _output_get (set `self.CurrentWeapon` _returnvalue))
  (`self.K2_AttachToComponent` _output_get (`self.SkeletalMesh`) "Sword_joint" "SnapToTarget" "SnapToTarget" "SnapToTarget" true))

(event `self.BP_AC_LivingActor.OnTakingDamage`
  (params (AttackOwner :type "Actor Object Reference"))
  (`KismetSystemLibrary.PrintString` (`KismetStringLibrary.Concat_StrStr` (`KismetSystemLibrary.GetObjectName` self) " remaining hp : " (`KismetStringLibrary.Conv_DoubleToString` (`/Game/Blueprint/Component/Actor/BP_AC_LivingActor.CurrentHp` (`self.BP_AC_LivingActor`))) " \nExplosion Vector :" (`KismetStringLibrary.Conv_VectorToString` (- (`self.K2_GetActorLocation` AttackOwner) (`self.K2_GetActorLocation`))))))

(event `self.BP_AC_LivingActor.OnDeath`
  (params (AttackOwner :type "Actor Object Reference"))
  (bind _returnvalue (`self.GetComponentByClass` AttackOwner "/Game/Blueprint/Component/Actor/BP_AC_SoulHandler.BP_AC_SoulHandler_C"))
  (`/Engine/EditorBlueprintResources/StandardMacros.IsValid` _returnvalue
    (:`Is Valid`
      (`/Game/Blueprint/Component/Actor/BP_AC_SoulHandler.GainSoul` _returnvalue (`self.SoulValue`))
      (`KismetSystemLibrary.PrintString` "So long")
      (`self.K2_DestroyActor` (`self.CurrentWeapon`))
      (`self.K2_DestroyActor`))))

(fn `UserConstructionScript`)