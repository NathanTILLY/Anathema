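; Sword-and-shield Griveton enemy that fights in melee and bursts into physics-driven armor pieces when killed.
; On BeginPlay it spawns and attaches its weapon; melee events pulse an attack flag and toggle the weapon hitbox.
; Each hit stores a direction from the attacker, used on death to launch the armor parts.
; Death also grants souls to the killer, destroys the weapon, hides the mesh and destroys the actor after a delay.
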(event `self.ReceiveBeginPlay`
  (bind _returnvalue (`|SpawnActorFromClass` "/Game/Blueprint/Weapons/BP_SwordAndShieldEnemy.BP_SwordAndShieldEnemy_C" (`self.GetTransform`) "Undefined" "OverrideRootScale" null null))
  (bind _output_get (set `self.CurrentWeapon` _returnvalue))
  (`self.K2_AttachToComponent` _output_get (`self.Mesh`) "WeaponSocket" "SnapToTarget" "SnapToTarget" "SnapToTarget" true)
  (`/Game/Blueprint/Interface/BPI_WeaponAttack.PickUp` (`self.CurrentWeapon`) self))

(event `self.BP_AC_LivingActor.OnTakingDamage`
  (params (AttackOwner :type "Actor Object Reference"))
  (bind _output_get (set `self.ExplosionVector` (`KismetMathLibrary.Normal` (- (`self.K2_GetActorLocation` AttackOwner) (`self.K2_GetActorLocation`)))))
  (set `self.ExplosionVector` (`KismetMathLibrary.MakeVector` (.x _output_get) (.y _output_get) 0.5))
  (`KismetSystemLibrary.PrintString` (`KismetStringLibrary.Concat_StrStr` (`KismetSystemLibrary.GetObjectName` self) " remaining hp : " (`KismetStringLibrary.Conv_DoubleToString` (`/Game/Blueprint/Component/Actor/BP_AC_LivingActor.CurrentHp` (`self.BP_AC_LivingActor`))))))

(event `self.BP_AC_LivingActor.OnDeath`
  (params (AttackOwner :type "Actor Object Reference"))
  (bind _returnvalue (`self.GetComponentByClass` AttackOwner "/Game/Blueprint/Component/Actor/BP_AC_SoulHandler.BP_AC_SoulHandler_C"))
  (bind _currentweapon (`self.CurrentWeapon`))
  (bind _capsulecomponent (`self.CapsuleComponent`))
  (bind _chestplate (`self.Chestplate`))
  (bind _returnvalue_2 (* (`self.ExplosionVector`) -500000.0))
  (`/Engine/EditorBlueprintResources/StandardMacros.IsValid` _returnvalue
    (:`Is Valid`
      (`/Game/Blueprint/Component/Actor/BP_AC_SoulHandler.GainSoul` _returnvalue (`self.SoulValue`)))
    (:`Is Not Valid`
      _))
  (`/Engine/EditorBlueprintResources/StandardMacros.IsValid` _capsulecomponent
    (:`Is Valid`
      (`PrimitiveComponent.SetCollisionEnabled` _capsulecomponent "NoCollision")
      (`/Engine/EditorBlueprintResources/StandardMacros.IsValid` _currentweapon
        (:`Is Valid`
          (`self.K2_DestroyActor` _currentweapon)
          (`SceneComponent.SetHiddenInGame` (`self.Mesh`) true false)
          (`|ExecutionSequence`
            (:`then_0`
              (`PrimitiveComponent.SetCollisionProfileName` _chestplate "IgnorePawn" true)
              (`PrimitiveComponent.SetSimulatePhysics` _chestplate true)
              (`PrimitiveComponent.AddForce` _chestplate _returnvalue_2 "None" false)
              (`KismetSystemLibrary.Delay` 0.0 :!label _label)
              (`KismetSystemLibrary.Delay` 5.0)
              (`self.K2_DestroyActor`))
            (:`then_1`
              (for _array_element (`|MakeArray` null (`self.FootL`) (`self.FootR`) (`self.ForearmL`) (`self.ForearmPlateL`) (`self.ForearmPlateR`) (`self.ForearmR`) null null (`self.Head`) (`self.KneeL`) (`self.KneeR`) (`self.LegHL`) (`self.LegHR`) (`self.LegLL`) (`self.LegLR`) (`self.ShoulderPlateL`) (`self.ShoulderPlateR`) (`self.Tunic`) (`self.Visor`))
                (`/Engine/EditorBlueprintResources/StandardMacros.IsValid` _array_element
                  (:`Is Valid`
                    (`PrimitiveComponent.SetCollisionProfileName` _array_element "IgnorePawn" true)
                    (`PrimitiveComponent.SetSimulatePhysics` _array_element true)
                    (`PrimitiveComponent.AddForce` _array_element _returnvalue_2 "None" false)
                    (goto _label)))))))))))

(event `/Game/Blueprint/Enemies/GeneralEnemy/BI_CombatInterface.MeleeAttack`
  (set `self.Attack?` true)
  (`KismetSystemLibrary.Delay` 0.2)
  (set `self.Attack?` false))

(event `/Game/Blueprint/Interface/BPI_UsingWeapon.ActiveWeapon`
  (bind _currentweapon (`self.CurrentWeapon`))
  (`/Engine/EditorBlueprintResources/StandardMacros.IsValid` _currentweapon
    (:`Is Valid`
      (`/Game/Blueprint/Weapons/BP_WeaponParent.SetHitboxState` _currentweapon true))))

(event `/Game/Blueprint/Interface/BPI_UsingWeapon.InactiveWeapon`
  (bind _currentweapon (`self.CurrentWeapon`))
  (`/Engine/EditorBlueprintResources/StandardMacros.IsValid` _currentweapon
    (:`Is Valid`
      (`/Game/Blueprint/Weapons/BP_WeaponParent.SetHitboxState` _currentweapon false)
      (set `/Game/Blueprint/Weapons/BP_WeaponParent.CurrentDamage` (`/Game/Blueprint/Weapons/BP_WeaponParent.LightAttackDamage` _currentweapon) _currentweapon))))

(fn `UserConstructionScript`)