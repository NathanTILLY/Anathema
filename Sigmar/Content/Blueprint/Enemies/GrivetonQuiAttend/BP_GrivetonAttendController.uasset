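; AI controller for the waiting Griveton enemy, driving it through the BT_GrivetonAttend behavior tree.
; On BeginPlay it starts the tree, stores the controlled Character and applies Speed as its max walk speed.
; Perception updates set the CanSeePlayer blackboard key when BP_Player is sensed, and nothing here clears it on loss.
; Patrol-path blackboard setup is present but unconnected, so it never runs.
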(event `self.ReceiveBeginPlay`
  (`|ExecutionSequence`
    (:`then_0`
      (`self.RunBehaviorTree` "/Game/Blueprint/Enemies/GrivetonQuiAttend/BT_GrivetonAttend.BT_GrivetonAttend")
      (bind _ascharacter (cast `Character` (`self.K2_GetPawn`)))
      (set `self.PawnTest` _ascharacter))
    (:`then_1`
      (set `CharacterMovementComponent.MaxWalkSpeed` (`self.Speed`) (`Character.CharacterMovement` (`self.PawnTest`))))))

(event `self.AIPerception.OnTargetPerceptionUpdated`
  (params (Actor :type "Actor Object Reference") (Stimulus :type "AIStimulus Structure"))
  (cast `/Game/Blueprint/Player/BP_Player` Actor)
  (bind _output_get (set `self.EntreDeux` (`.bSuccessfullySensed` (break `AIStimulus` Stimulus))))
  (if _output_get
    (`BlackboardComponent.SetValueAsBool` (`AIBlueprintHelperLibrary.GetBlackboard` null) "CanSeePlayer" true)))

(fn `UserConstructionScript`)