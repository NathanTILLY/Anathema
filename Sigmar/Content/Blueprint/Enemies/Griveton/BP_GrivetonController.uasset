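; AI controller for the Griveton enemy that runs its behavior tree and feeds it player sightings.
; On BeginPlay it starts BT_Griveton, caches the controlled Character and applies the Speed variable as its max walk speed.
; Perception updates for BP_Player write the sensing result to the CanSeePlayer blackboard key.
; Disconnected nodes for writing patrol path settings to the blackboard never run.
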(event `self.ReceiveBeginPlay`
  (`|ExecutionSequence`
    (:`then_0`
      (`self.RunBehaviorTree` "/Game/Blueprint/Enemies/Griveton/BT_Griveton.BT_Griveton")
      (bind _ascharacter (cast `Character` (`self.K2_GetPawn`)))
      (set `self.PawnTest` _ascharacter))
    (:`then_1`
      (set `CharacterMovementComponent.MaxWalkSpeed` (`self.Speed`) (`Character.CharacterMovement` (`self.PawnTest`))))))

(event `self.AIPerception.OnTargetPerceptionUpdated`
  (params (Actor :type "Actor Object Reference") (Stimulus :type "AIStimulus Structure"))
  (cast `/Game/Blueprint/Player/BP_Player` Actor)
  (`BlackboardComponent.SetValueAsBool` (`AIBlueprintHelperLibrary.GetBlackboard` null) "CanSeePlayer" (`.bSuccessfullySensed` (break `AIStimulus` Stimulus))))

(fn `UserConstructionScript`)