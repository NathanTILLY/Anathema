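; AI controller for enemy pawns that runs the BT_EnemyAI behavior tree to drive patrolling and player detection.
; On BeginPlay it casts the controlled pawn to BP_EnemyAI and seeds the Blackboard with its patrol path's looping flag and wait time, plus an initial direction.
; AI perception updates set CanSeePlayer whenever the player is sensed or lost.
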(event `self.ReceiveBeginPlay`
  (bind _returnvalue (`AIBlueprintHelperLibrary.GetBlackboard` null))
  (`self.RunBehaviorTree` "/Game/Blueprint/Enemies/GeneralEnemy/BT_EnemyAI.BT_EnemyAI")
  (bind _asbp_ennemy_ai (cast `/Game/Blueprint/Enemies/GeneralEnemy/BP_EnemyAI` (`self.K2_GetPawn`)))
  (bind _output_get (set `self.MyPawn` _asbp_ennemy_ai))
  (`BlackboardComponent.SetValueAsBool` (`AIBlueprintHelperLibrary.GetBlackboard` null) "PathLooping" (`/Game/Blueprint/Enemies/BP_PatrolPath.IsLooping` (`/Game/Blueprint/Enemies/GeneralEnemy/BP_EnemyAI.PatrolPath` _output_get)))
  (`BlackboardComponent.SetValueAsInt` _returnvalue "Direction" 1)
  (`BlackboardComponent.SetValueAsFloat` _returnvalue "WaitTime" (`/Game/Blueprint/Enemies/BP_PatrolPath.WaitTime` (`/Game/Blueprint/Enemies/GeneralEnemy/BP_EnemyAI.PatrolPath` (`self.MyPawn`)))))

(event `self.AIPerception.OnTargetPerceptionUpdated`
  (params (Actor :type "Actor Object Reference") (Stimulus :type "AIStimulus Structure"))
  (cast `/Game/Blueprint/Player/BP_Player` Actor)
  (`BlackboardComponent.SetValueAsBool` (`AIBlueprintHelperLibrary.GetBlackboard` null) "CanSeePlayer" (`.bSuccessfullySensed` (break `AIStimulus` Stimulus))))

(fn `UserConstructionScript`)