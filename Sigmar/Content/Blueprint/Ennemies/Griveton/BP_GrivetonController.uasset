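; BP_GrivetonController is the AI controller for the Griveton enemy.
; On BeginPlay it runs BT_Griveton, caches the controlled pawn and sets its walk speed from a Speed variable.
; AI Perception updates for the player write the sensed state to the CanSeePlayer blackboard key that the tree can read.
; Blackboard setup for patrol looping, direction and wait time is present but disconnected, so it never runs.
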(event `self.ReceiveBeginPlay`
  (`|ExecutionSequence`
    (:`then_0`
      (`self.RunBehaviorTree` "/Game/Blueprint/Ennemies/Griveton/BT_Griveton.BT_Griveton")
      (bind _asbp_griveton (cast `/Game/Blueprint/Ennemies/Griveton/BP_Griveton` (`self.K2_GetPawn`)))
      (bind _output_get (set `self.MyPawn` _asbp_griveton)))
    (:`then_1`
      (set `CharacterMovementComponent.MaxWalkSpeed` (`self.Speed`) (`Character.CharacterMovement` (`self.MyPawn`))))))

(event `self.AIPerception.OnTargetPerceptionUpdated`
  (params (Actor :type "Actor Object Reference") (Stimulus :type "AIStimulus Structure"))
  (cast `/Game/Blueprint/Player/BP_Player` Actor)
  (`BlackboardComponent.SetValueAsBool` (`AIBlueprintHelperLibrary.GetBlackboard` null) "CanSeePlayer" (`.bSuccessfullySensed` (break `AIStimulus` Stimulus))))

(fn `UserConstructionScript`)