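; BP_Spawner is a trigger-box enemy spawner that spawns AI enemies when BP_Player enters its Box.
; The overlap runs a loop that spawns BP_EnnemyAI pawns with BT_EnnemyAI at the SpawnLocation reference's transform until NbrDejaSpawn reaches NbrDeSpawn, printing each count.
; All spawns happen in one burst, and the counter is never reset here, so later overlaps add none once the quota is met.
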(event `self.Box.OnComponentBeginOverlap`
  (params (OverlappedComponent :type "PrimitiveComponent Object Reference") (OtherActor :type "Actor Object Reference") (OtherComp :type "PrimitiveComponent Object Reference") (OtherBodyIndex :type Integer) (bFromSweep :type Boolean) (SweepResult :type "HitResult Structure (by ref)"))
  (bind _nbrdejaspawn (`self.NbrDejaSpawn`))
  (bind _rootcomponent (`Actor.RootComponent` (`self.SpawnLocation`)))
  (cast `/Game/Blueprint/Player/BP_Player` OtherActor)
  (while (< (`self.NbrDejaSpawn`) (`self.NbrDeSpawn`))
    (`/Engine/EditorBlueprintResources/StandardMacros.IncrementFloat` _nbrdejaspawn
      (:`  `
        (`KismetSystemLibrary.PrintString` (`KismetStringLibrary.Conv_DoubleToString` _nbrdejaspawn))
        (`AIBlueprintHelperLibrary.SpawnAIFromClass` "/Game/Blueprint/Ennemies/GeneralEnnemy/BP_EnnemyAI.BP_EnnemyAI_C" "/Game/Blueprint/Ennemies/GeneralEnnemy/BT_EnnemyAI.BT_EnnemyAI" (`SceneComponent.K2_GetComponentLocation` _rootcomponent) (`SceneComponent.K2_GetComponentRotation` _rootcomponent) false null)))))

(fn `UserConstructionScript`)