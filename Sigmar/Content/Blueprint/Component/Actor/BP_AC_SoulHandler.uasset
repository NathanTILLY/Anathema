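; Actor component that manages a soul resource, gained from enemy kills and spent through a cost.
; GainSoul adds souls up to a maximum unless the current weapon is the Cursed Sword.
; ConsumeSoul succeeds whenever any soul remains, clamping at zero even if the cost exceeds it, and does not check the weapon despite its comment.
; An attempt with no soul left fires OnLastSoulUsed and returns false.
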(fn `ConsumeSoul`
  (params (SoulCost :type "Float (double-precision)"))
  (returns (`CanUseSoul?` :type Boolean))
  ;[1 1 1] Can't use soul if equal to zero or weapon is CursedSword
  (if (> (`self.CurrentSoul`) 0.0)
    (set `self.CurrentSoul` (`KismetMathLibrary.FClamp` (- (`self.CurrentSoul`) SoulCost) 0.0 (`self.MaxSoul`)))
    (return true)
    (else
      (`self.OnLastSoulUsed`)
      (return false))))

(fn `GainSoul`
  (params (AddedSoul :type "Float (double-precision)"))
  ;[1 1 1] Gain soul when enemy dies with weapon other than the Cursed Sword
  (if (not (== (`self.CurrentWeaponClass`) "/Game/Blueprint/Weapons/BP_CursedSword.BP_CursedSword_C"))
    (set `self.CurrentSoul` (`KismetMathLibrary.FClamp` (+ AddedSoul (`self.CurrentSoul`)) 0.0 (`self.MaxSoul`)))))